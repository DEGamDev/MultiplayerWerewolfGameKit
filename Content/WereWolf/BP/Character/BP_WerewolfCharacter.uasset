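; Player character for a Werewolf social-deduction game, handling camera-relative movement, body color, death state, visibility and return to spawn.
; On the server, capsule overlaps track the current task or emergency button, and ReportSphere overlaps let living players target dead characters for reporting.
; WW-prefixed interface messages expose this state and exchange data with controller, game mode and settings, which supply color and walk speed; most other interface getters are empty defaults.
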(event `UpdateCapsuleOverlap`
  ;[1 0.1039 0.1238] カプセルの重なりを更新
  (`PrimitiveComponent.SetCollisionEnabled` (`self.CapsuleComponent`) "NoCollision")
  (`PrimitiveComponent.SetCollisionEnabled` (`self.CapsuleComponent`) "QueryOnly"))

(event `CreateMeshMI`
  ;[0.2104 0.2948 1] メッシュのマテリアルインスタンスを作成
  (bind _returnvalue (`PrimitiveComponent.CreateDynamicMaterialInstance` (`self.GetMeshComp`) 0 null "None"))
  (`self.SetMIMesh` _returnvalue))

(event `self.ReceiveBeginPlay`
  ;[1 0.301 0.01818] BegimPlay
  (`|ExecutionSequence`
    (:`then_0`
      (`self.CreateMeshMI`)
      (`SceneComponent.SetVisibility` (`self.TextRender`) (`self.IsDebug`) false))
    (:`then_1`
      (`/Engine/EditorBlueprintResources/ActorMacros.Switch Has Authority`
        (:`Authority`
          (`|ExecutionSequence`
            (:`then_0`
              ;;[1 1 1] 初期の位置と回転を保存
              (`self.SetStartLocation` (`self.K2_GetActorLocation`))
              (`self.SetStartRotation` (`self.K2_GetActorRotation`)))
            (:`then_1`
              (`KismetSystemLibrary.Delay` 0.0)
              (`self.UpdateCapsuleOverlap`))))))))

(event `SetMIMesh`
  (params (MI_Mesh :type "MaterialInstanceDynamic Object Reference"))
  ;[0.1598 0.398 1] メッシュのマテリアルインスタンスをセット
  (set `self.MI_Mesh` MI_Mesh))

(event `/Game/WereWolf/BP/BP_WerewolfInterface.WW_SetCharacterColor`
  (params (Color :type "LinearColor Structure"))
  ;[0.633 0.1864 1] キャラクターの色をセット
  (`self.SetCharacterColor` Color))

(event `SetCharacterColor`
  (params (Color :type "LinearColor Structure"))
  (bind _mi_mesh (`self.GetMI_Mesh`))
  ;[0.633 0.1864 1] キャラクターの色をセット
  (`/Engine/EditorBlueprintResources/StandardMacros.IsValid` _mi_mesh
    (:`Is Valid`
      (`MaterialInstanceDynamic.SetVectorParameterValue` _mi_mesh "BodyColor" Color))))

(event `/Game/WereWolf/BP/BP_WerewolfInterface.WW_MoveForward`
  (params (Value :type "Float (single-precision)"))
  ;[1 1 1] 前後に移動
  (`self.AddMovementInput` (`KismetMathLibrary.GetForwardVector` (`self.GetMovementBaseRotation`)) Value))

(event `SetIsDead`
  (params (IsDead :type Boolean))
  ;[1 0.3018 0.3217] 死亡したかをセット
  (set `self.IsDead` IsDead)
  (message `/Game/WereWolf/BP/BP_WerewolfInterface.WW_SetIsDead` (`self.GetController`) true 0))

(event `/Game/WereWolf/BP/BP_WerewolfInterface.WW_MoveRight`
  (params (Value :type "Float (single-precision)"))
  ;[1 1 1] 左右に移動
  (`self.AddMovementInput` (`KismetMathLibrary.GetRightVector` (`self.GetMovementBaseRotation`)) Value))

(event `InitializeCharacterColor`
  ;[1 0.2187 0.2286] キャラクターの色を初期化
  (bind _gamesettings (message `/Game/WereWolf/BP/BP_WerewolfInterface.WW_GetGameSettings` (`GameplayStatics.GetGameMode`)))
  (bind _index (message `/Game/WereWolf/BP/BP_WerewolfInterface.WW_GetPlayerIndex` (`self.GetController`)))
  (bind _color (message `/Game/WereWolf/BP/BP_WerewolfInterface.WW_GetPlayerColorByIndex` _gamesettings _index))
  (`self.SetCharacterColor` _color))

(event `/Game/WereWolf/BP/BP_WerewolfInterface.WW_SetActiveCharacterMovement`
  (params (IsActive :type Boolean))
  ;[1 0.2604 0.2604] キャラクタームーブメントのアクティブをセット
  (`self.SetActiveCharacterMovement` IsActive))

(event `SetActiveCharacterMovement`
  (params (bNewActive :type Boolean))
  ;[1 0.2604 0.2604] キャラクタームーブメントのアクティブをセット
  (`CharacterMovementComponent.SetMovementMode` (`self.GetCharacterMovement`) (select `bool` bNewActive :`false` "MOVE_None" :`true` "MOVE_Walking" :!type "EMovementMode Enum") 0))

(event `/Game/WereWolf/BP/BP_WerewolfInterface.WW_InitializeCharacterColor`
  ;[1 0.2187 0.2286] キャラクターの色を初期化
  (`self.InitializeCharacterColor`))

(event `/Game/WereWolf/BP/BP_WerewolfInterface.WW_Turn`
  (params (Value :type "Float (single-precision)"))
  ;[1 1 1] カメラを左右に移動
  (`self.AddControllerYawInput` Value))

(event `/Game/WereWolf/BP/BP_WerewolfInterface.WW_LookUp`
  (params (Value :type "Float (single-precision)"))
  ;[1 1 1] カメラを上下に移動
  (`self.AddControllerPitchInput` Value))

(event `CapsuleBeginOverlap`
  (params (OtherActor :type "Actor Object Reference"))
  ;[1 1 1] カプセルが重なり始めたとき
  (`/Engine/EditorBlueprintResources/ActorMacros.Switch Has Authority`
    (:`Authority`
      ;;[1 1 1] タスク
      (bind _newparam (message `/Game/WereWolf/BP/BP_WerewolfInterface.WW_IsTask` OtherActor))
      (if _newparam
        (set `self.OverlapTask` OtherActor)
        (else
          ;;[1 1 1] 緊急ボタン
          (bind _newparam_2 (message `/Game/WereWolf/BP/BP_WerewolfInterface.WW_IsEmergencyButton` OtherActor))
          (if _newparam_2
            (set `self.OverlapEmergencyButton` OtherActor)))))))

(event `self.CapsuleComponent.OnComponentBeginOverlap`
  (params (OverlappedComponent :type "PrimitiveComponent Object Reference") (OtherActor :type "Actor Object Reference") (OtherComp :type "PrimitiveComponent Object Reference") (OtherBodyIndex :type Integer) (bFromSweep :type Boolean) (SweepResult :type "HitResult Structure (by ref)"))
  ;[1 1 1] カプセルが重なり始めたとき
  (`self.CapsuleBeginOverlap` OtherActor))

(event `CapsuleEndOverlap`
  (params (OtherActor :type "Actor Object Reference"))
  ;[1 1 1] カプセルが重なり終えたとき
  (`/Engine/EditorBlueprintResources/ActorMacros.Switch Has Authority`
    (:`Authority`
      ;;[1 1 1] 重なっているタスクと重なり終えたとき、重なっているタスクの参照を削除
      (bind _newparam (message `/Game/WereWolf/BP/BP_WerewolfInterface.WW_IsTask` OtherActor))
      (if _newparam
        (if (== OtherActor (`self.OverlapTask`))
          (set `self.OverlapTask` null))
        (else
          ;;[1 1 1] 重なっている緊急ボタンと重なり終えたとき、重なっている緊急ボタンの参照を削除
          (bind _newparam_2 (message `/Game/WereWolf/BP/BP_WerewolfInterface.WW_IsEmergencyButton` OtherActor))
          (if _newparam_2
            (if (== OtherActor (`self.GetOverlapEmergencyButton`))
              (`self.SetOverlapEmergencyButton` null) ; 重なっている緊急ボタンの参照を削除
            )))))))

(event `SetOverlapEmergencyButton`
  (params (OverlapEmergencyButton :type "Actor Object Reference"))
  ;[1 0.2708 0.2807] 重なっている緊急ボタンをセット
  (set `self.OverlapEmergencyButton` OverlapEmergencyButton))

(event `SetStartLocation`
  (params (StartLocation :type "Vector Structure"))
  ;[1 0.2708 0.2807] 初期位置をセット
  (set `self.StartLocation` StartLocation))

(event `self.CapsuleComponent.OnComponentEndOverlap`
  (params (OverlappedComponent :type "PrimitiveComponent Object Reference") (OtherActor :type "Actor Object Reference") (OtherComp :type "PrimitiveComponent Object Reference") (OtherBodyIndex :type Integer))
  ;[1 1 1] カプセルが重なり終えたとき
  (`self.CapsuleEndOverlap` OtherActor))

(event `SetStartRotation`
  (params (StartRotation :type "Rotator Structure"))
  ;[1 0.2708 0.2807] 初期回転をセット
  (set `self.StartRotation` StartRotation))

(event `/Game/WereWolf/BP/BP_WerewolfInterface.WW_ReturnToInitialLocation`
  ;[1 0.2708 0.2807] 初期位置へ戻る
  (`self.REturnToInitialLocatin`))

(event `ReturnToInitialLocatin`
  ;[1 0.2708 0.2807] 初期位置へ戻る
  (`self.K2_SetActorLocation` (`self.GetStartLocation`))
  (`self.K2_SetActorRotation` (`self.GetStartRotation`)))

(event `self.ReportSphere.OnComponentBeginOverlap`
  (params (OverlappedComponent :type "PrimitiveComponent Object Reference") (OtherActor :type "Actor Object Reference") (OtherComp :type "PrimitiveComponent Object Reference") (OtherBodyIndex :type Integer) (bFromSweep :type Boolean) (SweepResult :type "HitResult Structure (by ref)"))
  ;[1 1 1] 通報するSphereが重なった時
  (`/Engine/EditorBlueprintResources/ActorMacros.Switch Has Authority`
    (:`Authority`
      (if (not (`self.GetIsDead`))
        ;;[1 0.2071 0.1872] 通報する球がほかのキャラクターのカプセルと重なった時、そのキャラクターを通報可能にする
        (bind _newparam (message `/Game/WereWolf/BP/BP_WerewolfInterface.WW_GetIsCharacterCapsule` OtherActor OtherComp)) ; 相手のキャラクターのカプセルか？
        (bind _isdead (message `/Game/WereWolf/BP/BP_WerewolfInterface.WW_GetIsDead` OtherActor))
        (if (and _newparam _isdead)
          (`self.SetReportTarget` OtherActor) ; 通報するターゲットをセット
        )))))

(event `SetReportTarget`
  (params (ReportTarget :type "Actor Object Reference"))
  ;[1 0.1771 0.1771] 通報するターゲットをセット
  (set `self.ReportTarget` ReportTarget))

(event `self.ReportSphere.OnComponentEndOverlap`
  (params (OverlappedComponent :type "PrimitiveComponent Object Reference") (OtherActor :type "Actor Object Reference") (OtherComp :type "PrimitiveComponent Object Reference") (OtherBodyIndex :type Integer))
  ;[1 1 1] 通報するSphereが重なり終えた時
  (`/Engine/EditorBlueprintResources/ActorMacros.Switch Has Authority`
    (:`Authority`
      (if (not (`self.GetIsDead`))
        ;;[1 0.2071 0.1872] 通報する球がほかのキャラクターのカプセルと重なった時、そのキャラクターを通報可能にする
        (bind _newparam (message `/Game/WereWolf/BP/BP_WerewolfInterface.WW_GetIsCharacterCapsule` OtherActor OtherComp)) ; 相手のキャラクターのカプセルか？
        (bind _isdead (message `/Game/WereWolf/BP/BP_WerewolfInterface.WW_GetIsDead` OtherActor))
        (if (and _newparam _isdead)
          (if (== OtherActor (`self.GetReportTarget`))
            (`self.SetReportTarget` null) ; 通報するターゲットを削除
          ))))))

(event `/Game/WereWolf/BP/BP_WerewolfInterface.WW_SetWalkingSpeed`
  (params (Speed :type "Float (single-precision)"))
  ;[1 1 1] 移動速度をセットする
  (`self.SetMaxWalkSpeed` Speed))

(event `SetMaxWalkSpeed`
  (params (`Max Walk Speed` :type "Float (double-precision)"))
  ;[0.5838 0.1874 1] 最大歩行速度をセット
  (set `CharacterMovementComponent.MaxWalkSpeed` `Max Walk Speed` (`self.GetCharacterMovement`)))

(event `/Game/WereWolf/BP/BP_WerewolfInterface.WW_ApplyGameSettings`
  (params (GameSettings :type "Actor Object Reference"))
  ;[1 0.187 0.177] ゲーム設定を適用する
  (`self.ApplyGameSettings` GameSettings))

(event `ApplyGameSettings`
  (params (GameSettings :type "Actor Object Reference"))
  ;[1 0.187 0.177] ゲーム設定を適用する
  (`/Engine/EditorBlueprintResources/StandardMacros.IsValid` GameSettings
    (:`Is Valid`
      (bind _speed (message `/Game/WereWolf/BP/BP_WerewolfInterface.WW_GetMovingSpeed` GameSettings))
      (`self.SetMaxWalkSpeed` _speed))))

(event `/Game/WereWolf/BP/BP_WerewolfInterface.WW_SetCharacterVisible`
  (params (Visible :type Boolean))
  ;[1 0.1146 0.1146] キャラクターの可視性をセット
  (`self.SetCharacterVisible` Visible))

(event `SetCharacterVisible`
  (params (Visible :type Boolean))
  ;[1 0.1146 0.1146] キャラクターの可視性をセット
  (`self.SetActorHiddenInGame` (not Visible)))

(fn `Get Capsule Comp`
  (returns (Comp :type "CapsuleComponent Object Reference"))
  (return (`self.CapsuleComponent`)))

(fn `GetCameraRotation`
  (returns (Rotation :type "Rotator Structure"))
  (return (`SceneComponent.K2_GetComponentRotation` (`self.Camera`))))

(fn `GetCharacterMovement`
  (returns (`Character Movement` :type "CharacterMovementComponent Object Reference"))
  (return (`self.CharacterMovement`)))

(fn `GetIsDead`
  (returns (IsDead :type Boolean))
  (return (`self.IsDead`)))

(fn `GetMeshComp`
  (returns (Mesh :type "SkeletalMeshComponent Object Reference"))
  (return (`self.Mesh`)))

(fn `GetMI_Mesh`
  (returns (MI_Mesh :type "MaterialInstanceDynamic Object Reference"))
  (return (`self.MI_Mesh`)))

(fn `GetMovementBaseRotation`
  (returns (Rotation :type "Rotator Structure"))
  (return (`KismetMathLibrary.MakeRotator` 0.0 0.0 (.yaw (`self.GetCameraRotation`)))))

(fn `GetOverlapEmergencyButton`
  (returns (OverlapEmergencyButton :type "Actor Object Reference"))
  (return (`self.OverlapEmergencyButton`)))

(fn `GetReportTarget`
  (returns (ReportTarget :type "Actor Object Reference"))
  (return (`self.ReportTarget`)))

(fn `GetStartLocation`
  (returns (StartLocation :type "Vector Structure"))
  (return (`self.StartLocation`)))

(fn `GetStartRotation`
  (returns (StartRotation :type "Rotator Structure"))
  (return (`self.StartRotation`)))

(fn `UserConstructionScript`)

(fn `WW_GetAllCharacters`
  (returns (Characters :type "Array of Actor Object Reference"))
  (return))

(fn `WW_GetAllPC`
  (returns (PC :type "Array of Actor Object Reference"))
  (return))

(fn `WW_GetAllPlayersCount`
  (returns (Count :type Integer))
  (return 0))

(fn `WW_GetAllWolfs`
  (returns (Wolfs :type "Array of Actor Object Reference"))
  (return))

(fn `WW_GetCanMovingHatches`
  (returns (Hatches :type "Array of Actor Object Reference"))
  (return))

(fn `WW_GetCanUseEmergencyButton`
  (params (UsedCount :type Integer))
  (returns (Can :type Boolean))
  (return false))

(fn `WW_GetCharacterType`
  (returns (CharacterType :type "/Game/WereWolf/e_CharacterType Enum"))
  (return "NewEnumerator0"))

(fn `WW_GetCompletedTaskCount`
  (returns (Count :type Integer))
  (return 0))

(fn `WW_GetEmergencyButton`
  (returns (EmergencyButton :type "Actor Object Reference"))
  (return (`self.GetOverlapEmergencyButton`)))

(fn `WW_GetEmergencyMeetingCoolTime`
  (returns (Time :type Integer))
  (return 0))

(fn `WW_GetEmergencyTasks`
  (returns (Tasks :type "Array of Actor Object Reference"))
  (return))

(fn `WW_GetGameSettings`
  (returns (GameSettings :type "Actor Object Reference"))
  (return null))

(fn `WW_GetIsCharacterCapsule`
  (params (Comp :type "SceneComponent Object Reference"))
  (returns (NewParam :type Boolean))
  (return (== Comp (`self.CapsuleComponent`))))

(fn `WW_GetIsDead`
  (returns (IsDead :type Boolean))
  (return (`self.GetIsDead`)))

(fn `WW_GetIsEmergencyTaskCoolDown`
  (returns (IsCoolDown :type Boolean))
  (return false))

(fn `WW_GetIsEnableTask`
  (returns (IsEnable :type Boolean))
  (return false))

(fn `WW_GetIsGameFinished`
  (returns (IsGameFinished :type Boolean))
  (return false))

(fn `WW_GetIsInGame`
  (returns (IsInGame :type Boolean))
  (return false))

(fn `WW_GetIsInHatch`
  (returns (IsIn :type Boolean))
  (return false))

(fn `WW_GetIsInMeeting`
  (returns (In :type Boolean))
  (return false))

(fn `WW_GetIsInVotingTime`
  (returns (In :type Boolean))
  (return false))

(fn `WW_GetIsKillCoolDown`
  (returns (CoolDown :type Boolean))
  (return false))

(fn `WW_GetIsPlayerStart`
  (returns (NewParam :type Boolean))
  (return false))

(fn `WW_GetIsPutHand`
  (returns (IsPut :type Boolean))
  (return false))

(fn `WW_GetIsSabotageCoolDown`
  (returns (IsCoolDown :type Boolean))
  (return false))

(fn `WW_GetIsTaskManager`
  (returns (NewParam :type Boolean))
  (return false))

(fn `WW_GetIsUseCamera`
  (returns (Use :type Boolean))
  (return false))

(fn `WW_GetIsValidEmergencyTimer`
  (returns (IsValid :type Boolean))
  (return false))

(fn `WW_GetIsVotedToPlayer`
  (returns (NewParam :type Boolean))
  (return false))

(fn `WW_GetKillCoolDownTime`
  (returns (Time :type Integer))
  (return 0))

(fn `WW_GetMovingSpeed`
  (returns (Speed :type "Float (double-precision)"))
  (return 0.0))

(fn `WW_GetOverlapHatch`
  (returns (Hatch :type "Actor Object Reference"))
  (return null))

(fn `WW_GetPCByIndex`
  (params (Index :type Integer))
  (returns (PC :type "Actor Object Reference"))
  (return null))

(fn `WW_GetPlayerColorByIndex`
  (params (Index :type Integer))
  (returns (Color :type "LinearColor Structure"))
  (return))

(fn `WW_GetPlayerIndex`
  (returns (Index :type Integer))
  (return 0))

(fn `WW_GetPlayerName`
  (returns (Name :type String))
  (return ""))

(fn `WW_GetPlayerStarts`
  (returns (PlayerStarts :type "Array of Actor Object Reference"))
  (return))

(fn `WW_GetReportTarget`
  (returns (ReportTarget :type "Actor Object Reference"))
  (return (`self.GetReportTarget`)))

(fn `WW_GetSabotageCooldownPercent`
  (returns (Percent :type "Float (double-precision)"))
  (return 0.0))

(fn `WW_GetTask`
  (returns (Task :type "Actor Object Reference"))
  (return (`self.OverlapTask`)))

(fn `WW_GetTaskManagers`
  (returns (TaskManagers :type "Array of Actor Object Reference"))
  (return))

(fn `WW_GetTaskUIClass`
  (returns (TaskUIClass :type "UserWidget Class Reference"))
  (return null))

(fn `WW_GetVotedFromPlayerCount`
  (returns (Count :type Integer))
  (return 0))

(fn `WW_GetVotedFromPlayerIndex`
  (returns (Index :type "Array of Integer"))
  (return))

(fn `WW_GetVoteTime`
  (returns (Time :type Integer))
  (return 0))

(fn `WW_IsCompleted`
  (returns (NewParam :type Boolean))
  (return false))

(fn `WW_IsCompletedAllTask`
  (returns (IsCompleted :type Boolean))
  (return false))

(fn `WW_IsControlledCharacter`
  (returns (ReturnValue :type Boolean))
  (return (`self.IsControlled`)))

(fn `WW_IsEmergencyButton`
  (returns (NewParam :type Boolean))
  (return false))

(fn `WW_IsEmergencyTask`
  (returns (NewParam :type Boolean))
  (return false))

(fn `WW_IsGameSettings`
  (returns (ReturnValue :type Boolean))
  (return false))

(fn `WW_IsHatch`
  (returns (IsHatch :type Boolean))
  (return false))

(fn `WW_IsReportSphere`
  (params (Comp :type "PrimitiveComponent Object Reference"))
  (returns (NewParam :type Boolean))
  (return false))

(fn `WW_IsTask`
  (returns (NewParam :type Boolean))
  (return false))

(fn `WW_IsVillager`
  (returns (IsVillager :type Boolean))
  (return false))

(fn `WW_IsWolf`
  (returns (IsWolf :type Boolean))
  (return false))

(fn `WW_SetHatchButtonAngle`
  (params (Angle :type "Float (double-precision)"))
  (return))

(fn `WW_SpawnPlayers`
  (returns (Vilagers :type "Array of Actor Object Reference") (Wolfs :type "Array of Actor Object Reference"))
  (return))