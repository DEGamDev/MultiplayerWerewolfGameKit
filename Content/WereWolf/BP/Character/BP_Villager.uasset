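; BP_Villager is the villager character in the WereWolf game, handling its death when killed by a wolf.
; The kill event marks it dead, ragdolls the mesh, deactivates movement, and has the controller show the death screen, switch to UI input and remove task UI.
; It refreshes capsule overlaps by toggling collision, then tells the GameMode to decrement living villagers and check for game end.
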(event `SimulateBody`
  (bind _mesh (`self.Mesh`))
  ;[0.5587 0.217 1] メッシュを物理シミュレーション
  (`PrimitiveComponent.SetCollisionResponseToAllChannels` _mesh "ECR_Ignore")
  (`PrimitiveComponent.SetCollisionResponseToChannel` _mesh "ECC_WorldStatic" "ECR_Block")
  (`PrimitiveComponent.SetCollisionResponseToChannel` _mesh "ECC_WorldDynamic" "ECR_Block")
  (`PrimitiveComponent.SetCollisionEnabled` _mesh "PhysicsOnly")
  (`PrimitiveComponent.SetSimulatePhysics` _mesh true))

(event `/Game/WereWolf/BP/BP_WerewolfInterface.WW_KilledFromWolf`
  ;[1 0.2495 0.2395] 狼によって殺害されたとき
  (`self.KilledByWolf`))

(event `KilledByWolf`
  (bind _returnvalue (`self.GetController`))
  ;[1 0.2495 0.2395] 狼によって殺害されたとき
  (`|ExecutionSequence`
    (:`then_0`
      (`self.SetIsDead` true)
      (`self.SimulateBody`)
      (`ActorComponent.Deactivate` (`self.CharacterMovement`))
      (message `/Game/WereWolf/BP/BP_WerewolfInterface.WW_ShowDeadScreen` _returnvalue)
      (message `/Game/WereWolf/BP/BP_WerewolfInterface.WW_DisableGameInput` _returnvalue)
      (message `/Game/WereWolf/BP/BP_WerewolfInterface.WW_EnableUIInput` _returnvalue)
      (message `/Game/WereWolf/BP/BP_WerewolfInterface.WW_RemoveTaskUI` _returnvalue)
      (`self.UpdateCapsuleOverlap`))
    (:`then_1`
      (message `/Game/WereWolf/BP/BP_WerewolfInterface.WW_DecrementAliveVillagersCount` (`GameplayStatics.GetGameMode`)) ; 生存している村人の数を減らす
      (message `/Game/WereWolf/BP/BP_WerewolfInterface.WW_GameFinishCheck` (`GameplayStatics.GetGameMode`)))))

(event `UpdateCapsuleOverlap`
  ;[1 0.1039 0.1238] カプセルの重なりを更新
  (`PrimitiveComponent.SetCollisionEnabled` (`self.CapsuleComponent`) "NoCollision")
  (`PrimitiveComponent.SetCollisionEnabled` (`self.CapsuleComponent`) "QueryOnly"))

(fn `UserConstructionScript`
  (`parent.UserConstructionScript`))

(fn `WW_GetCharacterType`
  (returns (CharacterType :type "/Game/WereWolf/e_CharacterType Enum"))
  (return "NewEnumerator2"))