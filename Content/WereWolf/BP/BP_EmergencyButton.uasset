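; BP_EmergencyButton is the emergency button actor for the WereWolf game mode, identified to other systems through a shared set of WW_ query functions.
; WW_IsEmergencyButton returns true, while every other WW_ function returns an empty or default value.
; The event graph and construction script are empty, so the graphs shown act only as a type tag and contain no press or meeting logic.
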(fn `UserConstructionScript`)

(fn `WW_GetAllCharacters`
  (returns (Characters :type "Array of Actor Object Reference"))
  (return))

(fn `WW_GetAllPC`
  (returns (PC :type "Array of Actor Object Reference"))
  (return))

(fn `WW_GetAllPlayersCount`
  (returns (Count :type Integer))
  (return 0))

(fn `WW_GetAllWolfs`
  (returns (Wolfs :type "Array of Actor Object Reference"))
  (return))

(fn `WW_GetCanMovingHatches`
  (returns (Hatches :type "Array of Actor Object Reference"))
  (return))

(fn `WW_GetCanUseEmergencyButton`
  (params (UsedCount :type Integer))
  (returns (Can :type Boolean))
  (return false))

(fn `WW_GetCharacterType`
  (returns (CharacterType :type "/Game/WereWolf/e_CharacterType Enum"))
  (return "NewEnumerator0"))

(fn `WW_GetCompletedTaskCount`
  (returns (Count :type Integer))
  (return 0))

(fn `WW_GetEmergencyButton`
  (returns (EmergencyButton :type "Actor Object Reference"))
  (return null))

(fn `WW_GetEmergencyMeetingCoolTime`
  (returns (Time :type Integer))
  (return 0))

(fn `WW_GetEmergencyTasks`
  (returns (Tasks :type "Array of Actor Object Reference"))
  (return))

(fn `WW_GetGameSettings`
  (returns (GameSettings :type "Actor Object Reference"))
  (return null))

(fn `WW_GetIsCharacterCapsule`
  (params (Comp :type "SceneComponent Object Reference"))
  (returns (NewParam :type Boolean))
  (return false))

(fn `WW_GetIsDead`
  (returns (IsDead :type Boolean))
  (return false))

(fn `WW_GetIsEmergencyTaskCoolDown`
  (returns (IsCoolDown :type Boolean))
  (return false))

(fn `WW_GetIsEnableTask`
  (returns (IsEnable :type Boolean))
  (return false))

(fn `WW_GetIsGameFinished`
  (returns (IsGameFinished :type Boolean))
  (return false))

(fn `WW_GetIsInGame`
  (returns (IsInGame :type Boolean))
  (return false))

(fn `WW_GetIsInHatch`
  (returns (IsIn :type Boolean))
  (return false))

(fn `WW_GetIsInMeeting`
  (returns (In :type Boolean))
  (return false))

(fn `WW_GetIsInVotingTime`
  (returns (In :type Boolean))
  (return false))

(fn `WW_GetIsKillCoolDown`
  (returns (CoolDown :type Boolean))
  (return false))

(fn `WW_GetIsPlayerStart`
  (returns (NewParam :type Boolean))
  (return false))

(fn `WW_GetIsPutHand`
  (returns (IsPut :type Boolean))
  (return false))

(fn `WW_GetIsSabotageCoolDown`
  (returns (IsCoolDown :type Boolean))
  (return false))

(fn `WW_GetIsTaskManager`
  (returns (NewParam :type Boolean))
  (return false))

(fn `WW_GetIsUseCamera`
  (returns (Use :type Boolean))
  (return false))

(fn `WW_GetIsValidEmergencyTimer`
  (returns (IsValid :type Boolean))
  (return false))

(fn `WW_GetIsVotedToPlayer`
  (returns (NewParam :type Boolean))
  (return false))

(fn `WW_GetKillCoolDownTime`
  (returns (Time :type Integer))
  (return 0))

(fn `WW_GetMovingSpeed`
  (returns (Speed :type "Float (double-precision)"))
  (return 0.0))

(fn `WW_GetOverlapHatch`
  (returns (Hatch :type "Actor Object Reference"))
  (return null))

(fn `WW_GetPCByIndex`
  (params (Index :type Integer))
  (returns (PC :type "Actor Object Reference"))
  (return null))

(fn `WW_GetPlayerColorByIndex`
  (params (Index :type Integer))
  (returns (Color :type "LinearColor Structure"))
  (return))

(fn `WW_GetPlayerIndex`
  (returns (Index :type Integer))
  (return 0))

(fn `WW_GetPlayerName`
  (returns (Name :type String))
  (return ""))

(fn `WW_GetPlayerStarts`
  (returns (PlayerStarts :type "Array of Actor Object Reference"))
  (return))

(fn `WW_GetReportTarget`
  (returns (ReportTarget :type "Actor Object Reference"))
  (return null))

(fn `WW_GetSabotageCooldownPercent`
  (returns (Percent :type "Float (double-precision)"))
  (return 0.0))

(fn `WW_GetTask`
  (returns (Task :type "Actor Object Reference"))
  (return null))

(fn `WW_GetTaskManagers`
  (returns (TaskManagers :type "Array of Actor Object Reference"))
  (return))

(fn `WW_GetTaskUIClass`
  (returns (TaskUIClass :type "UserWidget Class Reference"))
  (return null))

(fn `WW_GetVotedFromPlayerCount`
  (returns (Count :type Integer))
  (return 0))

(fn `WW_GetVotedFromPlayerIndex`
  (returns (Index :type "Array of Integer"))
  (return))

(fn `WW_GetVoteTime`
  (returns (Time :type Integer))
  (return 0))

(fn `WW_IsCompleted`
  (returns (NewParam :type Boolean))
  (return false))

(fn `WW_IsCompletedAllTask`
  (returns (IsCompleted :type Boolean))
  (return false))

(fn `WW_IsControlledCharacter`
  (returns (ReturnValue :type Boolean))
  (return false))

(fn `WW_IsEmergencyButton`
  (returns (NewParam :type Boolean))
  (return true))

(fn `WW_IsEmergencyTask`
  (returns (NewParam :type Boolean))
  (return false))

(fn `WW_IsGameSettings`
  (returns (ReturnValue :type Boolean))
  (return false))

(fn `WW_IsHatch`
  (returns (IsHatch :type Boolean))
  (return false))

(fn `WW_IsReportSphere`
  (params (Comp :type "PrimitiveComponent Object Reference"))
  (returns (NewParam :type Boolean))
  (return false))

(fn `WW_IsTask`
  (returns (NewParam :type Boolean))
  (return false))

(fn `WW_IsVillager`
  (returns (IsVillager :type Boolean))
  (return false))

(fn `WW_IsWolf`
  (returns (IsWolf :type Boolean))
  (return false))

(fn `WW_SpawnPlayers`
  (returns (Vilagers :type "Array of Actor Object Reference") (Wolfs :type "Array of Actor Object Reference"))
  (return))