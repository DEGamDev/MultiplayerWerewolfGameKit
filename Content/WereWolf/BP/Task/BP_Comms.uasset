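; Communications task for a werewolf game: a touch-turned dial must be matched to a random target value set at BeginPlay.
; Dragging converts the touch direction around the dial into a normalized angle that rotates the dial and varies the left waveform's width by distance from the target.
; Within tolerance the red lamp goes dark, and releasing then sends task completion to the PlayerController.
; Construction creates dynamic materials for both lamps and waveforms.
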(event `self.ReceiveBeginPlay`
  (`parent.ReceiveBeginPlay`)
  (set `self.successValue` (`KismetMathLibrary.RandomFloat`))
  (`self.UpdateAngle` (`self.angle`)))

(event `self.Move`
  (params (Location :type "Vector Structure"))
  ;[1 1 1] タッチを動かしたとき
  (`parent.Move` Location)
  (`self.SetAngle` Location))

(event `self.Release`
  (params (PlayerController :type "PlayerController Object Reference"))
  ;[1 1 1] タッチを離したとき
  (`parent.Release` PlayerController)
  ;[1 1 1] 成功しているとき、プレイヤーコントローラーにタスク完了イベントを呼ぶ
  (if (`self.isSuccess`)
    (message `/Game/WereWolf/BP/BP_WerewolfInterface.WW_TaskComplete` PlayerController)))

(fn `GetValue`
  (returns (ReturnValue :type "Float (double-precision)"))
  (return (- 1.0 (`KismetMathLibrary.Abs` (mod (+ (/ (+ (.roll (`SceneComponent.RelativeRotation` (`self.DialMeshRoot`))) 180.0) 360.0) 0.5) 1.0)))))

(fn `SetAngle`
  (params (location :type "Vector Structure"))
  (locals (value_l :type "Float (double-precision)" :default 0.0))
  (`|ExecutionSequence`
    (:`then_0`
      (bind _output_get (set `local.value_l` (- 1.0 (`KismetMathLibrary.Abs` (mod (+ (/ (+ (.roll (`KismetMathLibrary.MakeRotFromXY` (`self.GetActorForwardVector`) (`KismetMathLibrary.GetForwardVector` (`KismetMathLibrary.FindLookAtRotation` (`SceneComponent.K2_GetComponentLocation` (`self.DialMeshRoot`)) location)))) 180.0) 360.0) 0.5) 1.0)))))
      (set `self.angle` _output_get)
      (bind _output_get_2 (set `self.isSuccess` (`KismetMathLibrary.NearlyEqual_FloatFloat` (`local.value_l`) (`self.successValue`) (`self.successTolerance`))))
      (if _output_get_2
        (`self.SetRampBrightness` (`self.M_RedRamp`))
        (else
          (`self.SetRampBrightness` (`self.M_RedRamp`) 2.0))))
    (:`then_1`
      (`self.UpdateAngle` (`self.angle`)))))

(fn `SetRampBrightness`
  (params (M_Ramp :type "MaterialInstanceDynamic Object Reference") (Value :type "Float (double-precision)"))
  (`MaterialInstanceDynamic.SetScalarParameterValue` M_Ramp "Brightness" Value))

(fn `SetRampColor`
  (params (M_Ramp :type "MaterialInstanceDynamic Object Reference") (Color :type "LinearColor Structure"))
  (`MaterialInstanceDynamic.SetVectorParameterValue` M_Ramp "Color" Color))

(fn `UpdateAngle`
  (params (Value :type "Float (double-precision)"))
  (`|ExecutionSequence`
    (:`then_0`
      (`SceneComponent.K2_SetRelativeRotation` (`self.DialMeshRoot`) (`KismetMathLibrary.MakeRotator` (`KismetMathLibrary.Lerp` 0.0 -360.0 Value)) false false))
    (:`then_1`
      (bind _m_wave_l (`self.M_Wave_L`)
        (:`then`
          (`MaterialInstanceDynamic.SetScalarParameterValue` _m_wave_l "Width" (`KismetMathLibrary.Lerp` 1.0 (`self.WaveWidth`) (/ (`KismetMathLibrary.Abs` (mod (- Value (`self.successValue`)) 1.0)) 0.5))))
        (:`else`)))))

(fn `UserConstructionScript`
  (bind _m_wave_r (`self.M_Wave_R`))
  (bind _m_wave_l (`self.M_Wave_L`))
  (`parent.UserConstructionScript`)
  (`|ExecutionSequence`
    (:`then_0`
      ;[1 1 1] ランプ
      (`|ExecutionSequence`
        (:`then_0`
          ;[1 1 1] 緑色のランプのマテリアルをセット
          (bind _returnvalue (`PrimitiveComponent.CreateDynamicMaterialInstance` (`self.GreenRampMesh`) 0 null "None"))
          (bind _output_get (set `self.M_GreenRamp` _returnvalue))
          (`self.SetRampColor` _output_get (struct :`G` 0.057292 :`B` 0.002391 :`A` 1.0))
          (`self.SetRampBrightness` _output_get 1.0))
        (:`then_1`
          ;[1 1 1] 赤色のランプのマテリアルをセット
          (bind _returnvalue_2 (`PrimitiveComponent.CreateDynamicMaterialInstance` (`self.RedRampMesh`) 0 null "None"))
          (bind _output_get_2 (set `self.M_RedRamp` _returnvalue_2))
          (`self.SetRampColor` _output_get_2 (struct :`R` 0.145833 :`G` 0.001255 :`A` 1.0))
          (`self.SetRampBrightness` _output_get_2 2.0))))
    (:`then_1`
      ;[1 1 1] 音声波形
      (`|ExecutionSequence`
        (:`then_0`
          ;[1 1 1] 右側の音声波形のマテリアルをセット
          (bind _returnvalue_3 (`KismetMaterialLibrary.CreateDynamicMaterialInstance` "/Game/Material/M_Wave.M_Wave"))
          (set `self.M_Wave_R` _returnvalue_3)
          (`PrimitiveComponent.SetMaterial` (`self.WaveMesh_R`) 0 _m_wave_r)
          (`MaterialInstanceDynamic.SetVectorParameterValue` _m_wave_r "BackColor" (`self.backColor`))
          (`MaterialInstanceDynamic.SetVectorParameterValue` _m_wave_r "WaveColor" (`self.waveColor`))
          (`MaterialInstanceDynamic.SetScalarParameterValue` _m_wave_r "Noise" 0.0))
        (:`then_1`
          ;[1 1 1] 左側の音声波形のマテリアルをセット
          (bind _returnvalue_4 (`KismetMaterialLibrary.CreateDynamicMaterialInstance` "/Game/Material/M_Wave.M_Wave"))
          (set `self.M_Wave_L` _returnvalue_4)
          (`PrimitiveComponent.SetMaterial` (`self.WaveMesh_L`) 0 _m_wave_l)
          (`MaterialInstanceDynamic.SetVectorParameterValue` _m_wave_l "BackColor" (`self.backColor`))
          (`MaterialInstanceDynamic.SetVectorParameterValue` _m_wave_l "WaveColor" (`self.waveColor`)))))
    (:`then_2`
      (`self.UpdateAngle` (`self.angle`)))))