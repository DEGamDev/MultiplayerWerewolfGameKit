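; Task manager actor for the WereWolf game that groups tasks into a set, apparently used as an emergency task.
; On BeginPlay the server binds to each BP_Task's completion event.
; An enable message activates every task; once all report completed, it disables itself and tells the GameMode to clear the emergency task.
; It identifies itself through the shared WW interface, leaving that interface's other getters as default stubs.
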(event `BindEvent`
  ;[1 1 1] タスクを完了したときにイベントをバインド
  (for _array_element (`self.GetTasks`)
    (bind _asbp_task (cast `/Game/WereWolf/BP/Task/BP_Task` _array_element))
    (add `/Game/WereWolf/BP/Task/BP_Task.OnCompleted` _asbp_task (delegate `OnTaskCompleted`))))

(event `self.ReceiveBeginPlay`
  (`/Engine/EditorBlueprintResources/ActorMacros.Switch Has Authority`
    (:`Authority`
      (`self.BindEvent`))))

(event `OnTaskCompleted`
  (params (Task :type "Actor Object Reference"))
  ;[1 1 1] タスクを完了したとき
  (bind _completed (`self.Get Is Tasks Complete`))
  (if _completed
    (`self.SetTaskComplete`)))

(event `/Game/WereWolf/BP/BP_WerewolfInterface.WW_EnableSetTask`
  ;[1 1 1] セットタスクを有効にする
  (set `self.IsEnable` true)
  (for _array_element (`self.Tasks`)
    (message `/Game/WereWolf/BP/BP_WerewolfInterface.WW_TaskEnable` _array_element)))

(event `SetTaskComplete`
  ;[1 0.1869 0.2167] セットタスクを完了する
  (set `self.IsEnable` false)
  (message `/Game/WereWolf/BP/BP_WerewolfInterface.WW_ClearEmergencyTask` (`GameplayStatics.GetGameMode`))
  (`KismetSystemLibrary.PrintString` "SetTaskCompleted" true true (struct :`R` 1.0 :`G` 0.351839 :`A` 1.0)))

(fn `Get Is Tasks Complete`
  (returns (Completed :type Boolean))
  (for _array_element (`self.Tasks`)
    (bind _newparam (message `/Game/WereWolf/BP/BP_WerewolfInterface.WW_IsCompleted` _array_element))
    (if (not _newparam)
      (return false)))
  (return true))

(fn `GetTasks`
  (returns (Tasks :type "Array of Actor Object Reference"))
  (return (`self.Tasks`)))

(fn `UserConstructionScript`)

(fn `WW_GetAllCharacters`
  (returns (Characters :type "Array of Actor Object Reference"))
  (return))

(fn `WW_GetAllPC`
  (returns (PC :type "Array of Actor Object Reference"))
  (return))

(fn `WW_GetAllPlayersCount`
  (returns (Count :type Integer))
  (return 0))

(fn `WW_GetCanMovingHatches`
  (returns (Hatches :type "Array of Actor Object Reference"))
  (return))

(fn `WW_GetCanUseEmergencyButton`
  (params (UsedCount :type Integer))
  (returns (Can :type Boolean))
  (return false))

(fn `WW_GetCharacterType`
  (returns (CharacterType :type "/Game/WereWolf/e_CharacterType Enum"))
  (return "NewEnumerator0"))

(fn `WW_GetCompletedTaskCount`
  (returns (Count :type Integer))
  (return 0))

(fn `WW_GetEmergencyButton`
  (returns (EmergencyButton :type "Actor Object Reference"))
  (return null))

(fn `WW_GetEmergencyMeetingCoolTime`
  (returns (Time :type Integer))
  (return 0))

(fn `WW_GetEmergencyTasks`
  (returns (Tasks :type "Array of Actor Object Reference"))
  (return))

(fn `WW_GetGameSettings`
  (returns (GameSettings :type "Actor Object Reference"))
  (return null))

(fn `WW_GetIsCharacterCapsule`
  (params (Comp :type "SceneComponent Object Reference"))
  (returns (NewParam :type Boolean))
  (return false))

(fn `WW_GetIsDead`
  (returns (IsDead :type Boolean))
  (return false))

(fn `WW_GetIsEmergencyTaskCoolDown`
  (returns (IsCoolDown :type Boolean))
  (return false))

(fn `WW_GetIsGameFinished`
  (returns (IsGameFinished :type Boolean))
  (return false))

(fn `WW_GetIsInGame`
  (returns (IsInGame :type Boolean))
  (return false))

(fn `WW_GetIsInHatch`
  (returns (IsIn :type Boolean))
  (return false))

(fn `WW_GetIsInMeeting`
  (returns (In :type Boolean))
  (return false))

(fn `WW_GetIsInVotingTime`
  (returns (In :type Boolean))
  (return false))

(fn `WW_GetIsKillCoolDown`
  (returns (CoolDown :type Boolean))
  (return false))

(fn `WW_GetIsPlayerStart`
  (returns (NewParam :type Boolean))
  (return false))

(fn `WW_GetIsPutHand`
  (returns (IsPut :type Boolean))
  (return false))

(fn `WW_GetIsTaskManager`
  (returns (NewParam :type Boolean))
  (return true) ; 自分はタスクマネージャー
)

(fn `WW_GetIsUseCamera`
  (returns (Use :type Boolean))
  (return false))

(fn `WW_GetIsValidEmergencyTimer`
  (returns (IsValid :type Boolean))
  (return false))

(fn `WW_GetIsVotedToPlayer`
  (returns (NewParam :type Boolean))
  (return false))

(fn `WW_GetKillCoolDownTime`
  (returns (Time :type Integer))
  (return 0))

(fn `WW_GetMovingSpeed`
  (returns (Speed :type "Float (double-precision)"))
  (return 0.0))

(fn `WW_GetOverlapHatch`
  (returns (Hatch :type "Actor Object Reference"))
  (return null))

(fn `WW_GetPCByIndex`
  (params (Index :type Integer))
  (returns (PC :type "Actor Object Reference"))
  (return null))

(fn `WW_GetPlayerColorByIndex`
  (params (Index :type Integer))
  (returns (Color :type "LinearColor Structure"))
  (return))

(fn `WW_GetPlayerIndex`
  (returns (Index :type Integer))
  (return 0))

(fn `WW_GetPlayerName`
  (returns (Name :type String))
  (return ""))

(fn `WW_GetPlayerStarts`
  (returns (PlayerStarts :type "Array of Actor Object Reference"))
  (return))

(fn `WW_GetReportTarget`
  (returns (ReportTarget :type "Actor Object Reference"))
  (return null))

(fn `WW_GetTask`
  (returns (Task :type "Actor Object Reference"))
  (return null))

(fn `WW_GetTaskManagers`
  (returns (TaskManagers :type "Array of Actor Object Reference"))
  (return))

(fn `WW_GetTaskUIClass`
  (returns (TaskUIClass :type "UserWidget Class Reference"))
  (return null))

(fn `WW_GetVotedFromPlayerCount`
  (returns (Count :type Integer))
  (return 0))

(fn `WW_GetVotedFromPlayerIndex`
  (returns (Index :type "Array of Integer"))
  (return))

(fn `WW_GetVoteTime`
  (returns (Time :type Integer))
  (return 0))

(fn `WW_IsCompleted`
  (returns (NewParam :type Boolean))
  (return false))

(fn `WW_IsCompletedAllTask`
  (returns (IsCompleted :type Boolean))
  (return false))

(fn `WW_IsControlledCharacter`
  (returns (ReturnValue :type Boolean))
  (return false))

(fn `WW_IsEmergencyButton`
  (returns (NewParam :type Boolean))
  (return false))

(fn `WW_IsEmergencyTask`
  (returns (NewParam :type Boolean))
  (return false))

(fn `WW_IsGameSettings`
  (returns (ReturnValue :type Boolean))
  (return false))

(fn `WW_IsHatch`
  (returns (IsHatch :type Boolean))
  (return false))

(fn `WW_IsReportSphere`
  (params (Comp :type "PrimitiveComponent Object Reference"))
  (returns (NewParam :type Boolean))
  (return false))

(fn `WW_IsTask`
  (returns (NewParam :type Boolean))
  (return false))

(fn `WW_IsVillager`
  (returns (IsVillager :type Boolean))
  (return false))

(fn `WW_IsWolf`
  (returns (IsWolf :type Boolean))
  (return false))

(fn `WW_SpawnPlayers`
  (returns (Vilagers :type "Array of Actor Object Reference") (Wolfs :type "Array of Actor Object Reference"))
  (return))