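; Game instance for the Werewolf game that carries match results and the gameplay level name across level loads.
; Setter events store the winners' info, the winning character type and the level name, with a getter for the level name.
; Network and travel failures are printed, and on a server network failure it destroys the session and prints the result.
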(event `SetWinnersInfo`
  (params (WinnersInfo :type "Array of /Game/Werewolf/BP/Result/s_WinnerInfo Structure"))
  ;[1 1 1] 勝者の情報をセット
  (set `self.WinnersInfo` WinnersInfo))

(event `SetWinnerCharacterType`
  (params (CharacterType :type "/Game/Werewolf/Enum/e_CharacterType Enum" :default "NewEnumerator1"))
  ;[1 1 1] 勝者のキャラクタータイプをセット
  (set `self.WinnerCharacterType` CharacterType))

(event `SetGameplayLevelName`
  (params (Name :type String))
  ;[1 1 1] ゲームのレベル名をセット
  (set `self.GameplayLevelName` Name))

(event `self.HandleNetworkError`
  (params (FailureType :type "ENetworkFailure Enum" :default "NetDriverAlreadyExists") (bIsServer :type Boolean))
  (`KismetSystemLibrary.PrintString` (`|GetEnumeratorNameAsString` FailureType))
  (if bIsServer
    (`DestroySessionCallbackProxy.DestroySession` (`GameplayStatics.GetPlayerController` 0)
      (:`OnSuccess`
        (`KismetSystemLibrary.PrintString` "Destroy Session Success"))
      (:`OnFailure`
        (`KismetSystemLibrary.PrintString` "Destroy Session Fail")))))

(event `self.HandleTravelError`
  (params (FailureType :type "ETravelFailure Enum" :default "NoLevel"))
  (`KismetSystemLibrary.PrintString` (`|GetEnumeratorNameAsString` FailureType)))

(fn `GetGameplayLevelName`
  (returns (Name :type String))
  (return (`self.GameplayLevelName`)))