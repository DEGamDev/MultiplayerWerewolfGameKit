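; Werewolf task minigame in which a player stops rotating discs one after another to complete the task.
; The construction script gathers three BP_RotateButton child actors and gives them colors and numbers.
; Each success starts the next disc until the count reaches ButtonCount and completes the task for that PlayerController.
; Opening the task or failing a stop resets all discs with a shared randomized start position and restarts from the first.
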(event `self.ReceiveBeginPlay`
  (`parent.ReceiveBeginPlay`)
  ;[1 1 1] 円盤を止めるのに成功したときと失敗したときのイベントをバインド
  (for _array_element (`self.rotateButtons`)
    (`/Engine/EditorBlueprintResources/StandardMacros.IsValid` _array_element
      (:`Is Valid`
        (add `/Game/Werewolf/BP/Task/BP_RotateButton.OnSuccess` _array_element (delegate `RotateButtonOnSuccess`))
        (add `/Game/Werewolf/BP/Task/BP_RotateButton.OnFail` _array_element (delegate `RotateButtonOnFail`))))))

(event `RotateButtonOnFail`
  ;[1 1 1] 回転を止めるのに失敗したとき、タスクを失敗する
  (`self.TaskFailPerPlayer`))

(event `RotateButtonOnSuccess`
  (params (PC :type "/Game/Werewolf/BP/Gameplay/BP_GameplayPlayerController Object Reference"))
  (bind _rotatebuttons (`self.rotateButtons`))
  ;[1 1 1] 回転を止めるのに成功したとき、全ての回転を止めていればタスクを完了する
  (`|ExecutionSequence`
    (:`then_0`
      (bind _output_get (set `self.successCount` (+ (`self.successCount`) 1)))
      (if (`KismetArrayLibrary.Array_IsValidIndex` _rotatebuttons _output_get)
        (bind _output (`|GetArrayItem` _rotatebuttons _output_get))
        (set `/Game/Werewolf/BP/Task/BP_RotateButton.isEnable` true _output)
        (`/Game/Werewolf/BP/Task/BP_RotateButton.StartRotate` _output)))
    (:`then_1`
      (if (`self.GetIsComplete`)
        (`/Engine/EditorBlueprintResources/StandardMacros.IsValid` PC
          (:`Is Valid`
            (`/Game/Werewolf/BP/Gameplay/BP_GameplayPlayerController.TaskComplete` PC)))))))

(event `self.OnOpenPerPlayerTask`
  (params (PC :type "/Game/Werewolf/BP/Gameplay/BP_GameplayPlayerController Object Reference"))
  ;[1 1 1] タスクを開いたとき、初期化する
  (`parent.OnOpenPerPlayerTask` PC)
  (`self.InitializePerPlayerTask`))

(event `self.TaskFailPerPlayer`
  ;[1 1 1] タスクを失敗したとき、初期化する
  (`parent.TaskFailPerPlayer`)
  (`self.InitializePerPlayerTask`))

(event `self.InitializePerPlayerTask`
  (bind _startalpharandom (`self.startAlphaRandom`))
  (bind _rotatebuttons (`self.rotateButtons`))
  (bind _output (`|GetArrayItem` _rotatebuttons))
  ;[1 1 1] 初期化
  (`parent.InitializePerPlayerTask`)
  (`|ExecutionSequence`
    (:`then_0`
      (for _array_element (`self.rotateButtons`)
        (`/Game/Werewolf/BP/Task/BP_RotateButton.Reset` _array_element)))
    (:`then_1`
      (`|ExecutionSequence`
        (:`then_0`
          (`|ExecutionSequence`
            (:`then_0`
              (set `self.randomValue` (`KismetMathLibrary.RandomFloatInRange` (* (/ _startalpharandom 2.0) -1.0) _startalpharandom)))
            (:`then_1`
              (for _array_element_2 (`self.rotateButtons`)
                (set `/Game/Werewolf/BP/Task/BP_RotateButton.startAlpha` (`KismetMathLibrary.Abs` (mod (+ (`self.startAlpha`) (`self.randomValue`)) 1.0)) _array_element_2)
                (set `/Game/Werewolf/BP/Task/BP_RotateButton.alpha` 0.0 _array_element_2)
                (`/Game/Werewolf/BP/Task/BP_RotateButton.SetAlpha` _array_element_2 (`/Game/Werewolf/BP/Task/BP_RotateButton.currentAlpha` _array_element_2))))))
        (:`then_1`
          (set `self.successCount` 0)
          (if (`KismetArrayLibrary.Array_IsValidIndex` _rotatebuttons)
            (set `/Game/Werewolf/BP/Task/BP_RotateButton.isEnable` true _output)
            (`/Game/Werewolf/BP/Task/BP_RotateButton.StartRotate` _output)))))))

(fn `GetIsComplete`
  (returns (complete :type Boolean))
  (return (== (`self.successCount`) (`self.buttonCount`))))

(fn `UserConstructionScript`
  (bind _colors (`self.colors`))
  (`parent.UserConstructionScript`)
  (`|ExecutionSequence`
    (:`then_0`
      (for _array_element (`|MakeArray` (`self.ChildActor`) (`self.ChildActor1`) (`self.ChildActor2`))
        (bind _asbp_rotate_button (cast `/Game/Werewolf/BP/Task/BP_RotateButton` (`ChildActorComponent.ChildActor` _array_element)))
        (`KismetArrayLibrary.Array_Add` (`self.rotateButtons`) _asbp_rotate_button)))
    (:`then_1`
      (for (_array_element_2 _array_index) (`self.rotateButtons`)
        (if (`KismetArrayLibrary.Array_IsValidIndex` _colors _array_index)
          (`/Game/Werewolf/BP/Task/BP_RotateButton.SetColor` _array_element_2 (`|GetArrayItem` _colors _array_index))
          (`/Game/Werewolf/BP/Task/BP_RotateButton.SetNumber` _array_element_2 (+ _array_index 1)))))))