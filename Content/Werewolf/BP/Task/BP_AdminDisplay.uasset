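; Admin display task for the Werewolf game that shows how many living players are in each room, excluding those in hatches.
; On the server it takes its UI class from game settings and binds to comms toggles and every character's floor enter/leave events.
; Opening it sends all room counts to that player, while floor changes update only players using this task.
; Comms state enables or disables the display.
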(event `self.Initialize`
  ;[1 1 1] 初期化
  (`parent.Initialize`)
  (`/Engine/EditorBlueprintResources/ActorMacros.Switch Has Authority`
    (:`Authority`
      (bind _asbp_gameplay_game_mode (cast `/Game/Werewolf/BP/Gameplay/BP_GameplayGameMode` (`GameplayStatics.GetGameMode`)))
      (`|ExecutionSequence`
        (:`then_0`
          ;;[1 1 1] 通信の有効性が切り替わったときのイベントをバインド
          (add `/Game/Werewolf/BP/Gameplay/BP_GameplayGameMode.OnCommsEnabled` _asbp_gameplay_game_mode (`|CreateDelegate` :!event `OnCommsEnable`)) ; 通信が有効になったとき
          (add `/Game/Werewolf/BP/Gameplay/BP_GameplayGameMode.OnCommsDisabled` _asbp_gameplay_game_mode (`|CreateDelegate` :!event `OnCommsDisable`)) ; 通信が無効になったとき
          (bind _gamesettings (`/Game/Werewolf/BP/Gameplay/BP_GameplayGameMode.GetGameSettings` _asbp_gameplay_game_mode))
          (`/Engine/EditorBlueprintResources/StandardMacros.IsValid` _gamesettings
            (:`Is Valid`
              (set `self.TaskUIClass` (`/Game/Werewolf/BP/Gameplay/BP_GameSettings.UI_AdminDisplayClass` _gamesettings)) ; ゲームモードの管理画面UIに上書き
            )))
        (:`then_1`
          ;;[1 1 1] 全てのキャラクターが部屋から出入りしたときのイベントをバインド
          (for _array_element (`/Game/Werewolf/BP/Gameplay/BP_GameplayGameMode.Get All Characters` _asbp_gameplay_game_mode)
            (`/Engine/EditorBlueprintResources/StandardMacros.IsValid` _array_element
              (:`Is Valid`
                (add `/Game/Werewolf/BP/Character/BP_WerewolfCharacter.OnEnterFloor` _array_element (`|CreateDelegate` :!event `CharacterOnEnterFloor`)) ; 部屋に入ったとき
                (add `/Game/Werewolf/BP/Character/BP_WerewolfCharacter.OnLeaveFloor` _array_element (`|CreateDelegate` :!event `CharacterOnLeaveFloor`)) ; 部屋から出たとき
              ))))))))

(event `OnCommsEnable`
  ;[1 1 1] 通信が有効になったとき、管理画面を有効にする
  (bind _asbp_gameplay_game_mode (cast `/Game/Werewolf/BP/Gameplay/BP_GameplayGameMode` (`GameplayStatics.GetGameMode`)))
  (for _array_element (`/Game/Werewolf/BP/Gameplay/BP_GameplayGameMode.GetAllPC` _asbp_gameplay_game_mode)
    (`/Engine/EditorBlueprintResources/StandardMacros.IsValid` _array_element
      (:`Is Valid`
        (`/Game/Werewolf/BP/Gameplay/BP_GameplayPlayerController.SetAdminDisplayEnabled` _array_element true)))))

(event `OnCommsDisable`
  ;[1 1 1] 通信が無効になったとき、管理画面を無効にする
  (bind _asbp_gameplay_game_mode (cast `/Game/Werewolf/BP/Gameplay/BP_GameplayGameMode` (`GameplayStatics.GetGameMode`)))
  (for _array_element (`/Game/Werewolf/BP/Gameplay/BP_GameplayGameMode.GetAllPC` _asbp_gameplay_game_mode)
    (`/Engine/EditorBlueprintResources/StandardMacros.IsValid` _array_element
      (:`Is Valid`
        (`/Game/Werewolf/BP/Gameplay/BP_GameplayPlayerController.SetAdminDisplayEnabled` _array_element false)))))

(event `self.OnOpen`
  (params (PC :type "/Game/Werewolf/BP/Gameplay/BP_GameplayPlayerController Object Reference"))
  ;[1 1 1] 管理画面を開いたとき、プレイヤーに対して管理画面を初期化する
  (`parent.OnOpen` PC)
  (`self.InitializeDisplayToPlayer` PC))

(event `CharacterOnEnterFloor`
  (params (Character :type "/Game/Werewolf/BP/Character/BP_WerewolfCharacter Object Reference"))
  (bind _pc (`/Game/Werewolf/BP/Character/BP_WerewolfCharacter.GetPC` Character))
  (bind _floor (`/Game/Werewolf/BP/Gameplay/BP_GameplayPlayerController.GetInFloor` _pc))
  ;[1 1 1] 部屋に入ったとき、その部屋の人数を管理画面を開いている全てのプレイヤーへ更新
  (`/Engine/EditorBlueprintResources/StandardMacros.IsValid` Character
    (:`Is Valid`
      (`/Engine/EditorBlueprintResources/StandardMacros.IsValid` _pc
        (:`Is Valid`
          (`/Engine/EditorBlueprintResources/StandardMacros.IsValid` _floor
            (:`Is Valid`
              (`self.UpdateFloorToAllPlayers` (`/Game/Werewolf/BP/Floor/BP_FloorVolume.floorName` _floor)))
            (:`Is Not Valid`
              (`KismetSystemLibrary.PrintString` "UpdateFloorToAllPlayers Failed" true true (struct :`R` 1.0 :`A` 1.0) :!label _label))))
        (:`Is Not Valid`
          (goto _label))))
    (:`Is Not Valid`
      (goto _label))))

(event `InitializeDisplayToPlayer`
  (params (PC :type "/Game/Werewolf/BP/Gameplay/BP_GameplayPlayerController Object Reference"))
  ;[1 1 1] プレイヤーに対して管理画面を初期化
  (`/Engine/EditorBlueprintResources/StandardMacros.IsValid` PC
    (:`Is Valid`
      (bind _gm (`/Game/Werewolf/BP/Gameplay/BP_GameplayPlayerController.GM` PC)
        (:`then`
          (for _array_element (`/Game/Werewolf/BP/Gameplay/BP_GameplayGameMode.AllFloors` _gm)
            (`/Engine/EditorBlueprintResources/StandardMacros.IsValid` _array_element
              (:`Is Valid`
                (bind _floorname (`/Game/Werewolf/BP/Floor/BP_FloorVolume.floorName` _array_element))
                (bind _number (`self.GetNumberOfFloors` _floorname))
                (`/Game/Werewolf/BP/Gameplay/BP_GameplayPlayerController.UpdateAdminDisplay` PC _floorname _number))))
          (`/Game/Werewolf/BP/Gameplay/BP_GameplayPlayerController.SetAdminDisplayEnabled` PC (`/Game/Werewolf/BP/Gameplay/BP_GameplayGameMode.Get Comms Enabled` _gm)) ; 通信の有効性をセット
        )
        (:`else`)))))

(event `CharacterOnLeaveFloor`
  (params (Character :type "/Game/Werewolf/BP/Character/BP_WerewolfCharacter Object Reference") (Floor :type "/Game/Werewolf/BP/Floor/BP_FloorVolume Object Reference"))
  ;[1 1 1] 部屋から出たとき、その部屋の人数を管理画面を開いている全てのプレイヤーへ更新
  (`/Engine/EditorBlueprintResources/StandardMacros.IsValid` Character
    (:`Is Valid`
      (`/Engine/EditorBlueprintResources/StandardMacros.IsValid` (`/Game/Werewolf/BP/Character/BP_WerewolfCharacter.GetPC` Character)
        (:`Is Valid`
          (`/Engine/EditorBlueprintResources/StandardMacros.IsValid` Floor
            (:`Is Valid`
              (`self.UpdateFloorToAllPlayers` (`/Game/Werewolf/BP/Floor/BP_FloorVolume.floorName` Floor)))
            (:`Is Not Valid`
              (`KismetSystemLibrary.PrintString` "UpdateFloorToAllPlayers Failed" true true (struct :`R` 1.0 :`A` 1.0) :!label _label_2))))
        (:`Is Not Valid`
          (goto _label_2))))
    (:`Is Not Valid`
      (goto _label_2))))

(fn `GetNumberOfFloors`
  (params (Name :type String))
  (returns (Number :type Integer))
  (locals (Num_l :type Integer))
  ;[1 1 1] 部屋にいる生存しているプレイヤー数を取得
  (bind _asbp_gameplay_game_mode (cast `/Game/Werewolf/BP/Gameplay/BP_GameplayGameMode` (`GameplayStatics.GetGameMode`))
    (:`then`
      (for _array_element (`/Game/Werewolf/BP/Gameplay/BP_GameplayGameMode.GetAllPC` _asbp_gameplay_game_mode)
        (`/Engine/EditorBlueprintResources/StandardMacros.IsValid` _array_element
          (:`Is Valid`
            (bind _floor (`/Game/Werewolf/BP/Gameplay/BP_GameplayPlayerController.GetInFloor` _array_element))
            (`/Engine/EditorBlueprintResources/StandardMacros.IsValid` _floor
              (:`Is Valid`
                (if (not (`/Game/Werewolf/BP/Gameplay/BP_GameplayPlayerController.GetIsDead` _array_element))
                  (bind _isin (`/Game/Werewolf/BP/BP_WerewolfInterface.WW_GetIsInHatch` (`/Game/Werewolf/BP/Gameplay/BP_GameplayPlayerController.GetCharacter` _array_element)))
                  (if (and (`KismetStringLibrary.EqualEqual_StrStr` (`/Game/Werewolf/BP/Floor/BP_FloorVolume.floorName` _floor) Name) (not _isin))
                    (set `local.Num_l` (+ (`local.Num_l`) 1)))))))))
      (return (`local.Num_l`)))
    (:`CastFailed`
      (return 0))))

(fn `UpdateFloorToAllPlayers`
  (params (floorName :type String))
  (locals (colors_l :type "Array of LinearColor Structure") (Num_l :type Integer :default 0))
  ;[1 1 1] 全てのプレイヤーに対して部屋の人数を更新する
  (bind _asbp_gameplay_game_mode (cast `/Game/Werewolf/BP/Gameplay/BP_GameplayGameMode` (`GameplayStatics.GetGameMode`)))
  (bind _number (`self.GetNumberOfFloors` floorName))
  (set `local.Num_l` _number)
  (for _array_element (`/Game/Werewolf/BP/Gameplay/BP_GameplayGameMode.GetAllPC` _asbp_gameplay_game_mode)
    (`/Engine/EditorBlueprintResources/StandardMacros.IsValid` _array_element
      (:`Is Valid`
        (if (== (`/Game/Werewolf/BP/Gameplay/BP_GameplayPlayerController.GetTask` _array_element) self)
          (`/Game/Werewolf/BP/Gameplay/BP_GameplayPlayerController.UpdateAdminDisplay` _array_element floorName (`local.Num_l`))
          (`/Game/Werewolf/BP/Gameplay/BP_GameplayPlayerController.SetAdminDisplayEnabled` _array_element (`/Game/Werewolf/BP/Gameplay/BP_GameplayGameMode.Get Comms Enabled` _asbp_gameplay_game_mode)))))))

(fn `UpdateFloorToPlayer`
  (params (floorName :type String) (PC :type "/Game/Werewolf/BP/Gameplay/BP_GameplayPlayerController Object Reference"))
  ;[1 1 1] 部屋の中にいる生存しているプレイヤー数を更新
  (bind _number (`self.GetNumberOfFloors` floorName))
  (`/Engine/EditorBlueprintResources/StandardMacros.IsValid` PC
    (:`Is Valid`
      (`/Game/Werewolf/BP/Gameplay/BP_GameplayPlayerController.UpdateAdminDisplay` PC floorName _number))))

(fn `UserConstructionScript`
  (`parent.UserConstructionScript`))