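; Base Blueprint for a Werewolf game task that tracks whether a player has a hand placed on it.
; Enabling the task clears the state; putting a hand sets it, plays a sound and fires CallOnPutHand.
; Closing releases the hand, which only clears the state and notifies while the game master's emergency timer is valid.
; A debug hold-pressed setting keeps the hand down in that case.
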(event `self.TaskEnable`
  (params (TargetPC :type "/Game/Werewolf/BP/Gameplay/BP_GameplayPlayerController Object Reference"))
  ;[1 1 1] 有効になったとき、手を置いている状態を初期化
  (`parent.TaskEnable` TargetPC)
  (`self.SetIsPutHand` false))

(event `SetIsPutHand`
  (params (IsPut :type Boolean))
  ;[1 1 1] タスクに手を置いているかをセット
  (set `self.IsPutHand` IsPut))

(event `self.OnClose`
  (params (PC :type "/Game/Werewolf/BP/Gameplay/BP_GameplayPlayerController Object Reference"))
  ;[1 1 1] タスクを閉じたとき、手を離す
  (`parent.OnClose` PC)
  (`/Game/Werewolf/BP/BP_WerewolfInterface.WW_ReleaseHand` PC))

(event `/Game/Werewolf/BP/BP_WerewolfInterface.WW_PutHand`
  (params (PC :type "/Game/Werewolf/BP/Gameplay/BP_GameplayPlayerController Object Reference"))
  ;[1 1 1] 手を置く
  (`self.SetIsPutHand` true) ; デバッグ中でなければ手を離す
  (`/Game/Werewolf/BP/Gameplay/BP_GameplayPlayerController.PlayPutHandSound` PC (`self.PutHandSound`))
  (`self.OnPutHand` (`self.GetIsPutHand`)))

(event `/Game/Werewolf/BP/BP_WerewolfInterface.WW_ReleaseHand`
  (params (PC :type "/Game/Werewolf/BP/Gameplay/BP_GameplayPlayerController Object Reference"))
  ;[1 1 1] 手を離す
  (bind _gm (`/Game/Werewolf/BP/Gameplay/BP_GameplayPlayerController.GM` PC)
    (:`then`
      (if (`/Game/Werewolf/BP/Gameplay/BP_GameplayGameMode.GetIsValidEmergencyTimer` _gm)
        (if (not (`/Game/Werewolf/BP/Gameplay/BP_GameSettings.IsDebugTaskHoldPressed` (`/Game/Werewolf/BP/Gameplay/BP_GameplayGameMode.GetGameSettings` _gm)))
          (`self.SetIsPutHand` false) ; デバッグ中でなければ手を離す
          (`/Game/Werewolf/BP/Gameplay/BP_GameplayPlayerController.StopPutHandSound` PC)
          (`self.OnPutHand` (`self.GetIsPutHand`)))
        (else
          (`/Game/Werewolf/BP/Gameplay/BP_GameplayPlayerController.StopPutHandSound` PC))))
    (:`else`)))

(fn `GetIsPutHand`
  (returns (IsPut :type Boolean))
  (return (`self.IsPutHand`)))

(fn `UserConstructionScript`
  (`parent.UserConstructionScript`))

(fn `WW_GetIsPutHand`
  (returns (IsPut :type Boolean))
  (return (`self.GetIsPutHand`)))