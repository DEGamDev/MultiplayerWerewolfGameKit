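; BP_RotateButton is a touchable task button with a rotating ring, where the player must stop it at a target angle.
; A looping timeline, rate-scaled by Speed, spins it; a press stops it and compares the current alpha to SuccessAlpha within a tolerance.
; Success snaps the angle, fills the gauge, lights the lamp and notifies listeners, while failure returns to StartAlpha.
; UpdatePercent adds random jitter to the gauge while enabled.
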(event `self.ReceiveBeginPlay`
  ;[1 0.3051 0] BeginPlay
  (`parent.ReceiveBeginPlay`)
  (`|ExecutionSequence`
    (:`then_0`
      ;;[1 1 1] ゲージを初期化
      (bind _asui_gage (cast `/Game/Werewolf/UI/Gameplay/UI_Gage` (`WidgetComponent.GetUserWidgetObject` (`self.Widget`))))
      (bind _output_get (set `self.UI_Bar` _asui_gage))
      (`/Game/Werewolf/UI/Gameplay/UI_Gage.SetBarColor` _output_get (`self.ringColor`))
      (`/Game/Werewolf/UI/Gameplay/UI_Gage.SetPercent` _output_get 0.0))
    (:`then_1`
      ;;[1 1 1] ゲージを更新するタイマーをセット
      (`KismetSystemLibrary.K2_SetTimerDelegate` (`|CreateDelegate` :!event `UpdatePercent`) (`KismetMathLibrary.RandomFloatInRange` 0.08 0.1) true))))

(event `StartRotate`
  (bind _tl_rotate (`self.TL_Rotate`))
  ;[1 1 1] ボタンの回転を開始
  (`TimelineComponent.SetPlayRate` _tl_rotate (/ 1.0 (`self.speed`)))
  (`TimelineComponent.PlayFromStart` _tl_rotate)
  (`TimelineComponent.SetLooping` _tl_rotate true))

(event `Reset`
  ;[1 1 1] リセット
  (`|ExecutionSequence`
    (:`then_0`
      (bind _ui_bar (`self.UI_Bar`)
        (:`then`
          (`/Game/Werewolf/UI/Gameplay/UI_Gage.SetPercent` _ui_bar 0.0))
        (:`else`)))
    (:`then_1`
      (set `self.isSuccess` false))
    (:`then_2`
      (set `self.isEnable` false))
    (:`then_3`
      (`self.lightOff`))
    (:`then_4`
      (`self.StopRotate`))))

(event `StopRotate`
  ;[1 1 1] ボタンを止める
  (`TimelineComponent.Stop` (`self.TL_Rotate`)))

(event `/Game/Werewolf/BP/BP_TouchInterface.TCH_PresseByPlayer`
  (params (PC :type "/Game/Werewolf/BP/Gameplay/BP_GameplayPlayerController Object Reference") (Comp :type "SceneComponent Object Reference"))
  ;[1 1 1] ボタンが押されたとき、回転を止める
  (if (not (`self.isSuccess`))
    (`|ExecutionSequence`
      (:`then_0`
        (set `self.isEnable` false)
        (`self.StopRotate`))
      (:`then_1`
        (if (`KismetMathLibrary.NearlyEqual_FloatFloat` (`self.currentAlpha`) (`self.successAlpha`) (`self.successTolerance`))
          (set `self.isSuccess` true)
          (`|ExecutionSequence`
            (:`then_0`
              (`|ExecutionSequence`
                (:`then_0`
                  (`self.SetAlpha` (`self.successAlpha`)))
                (:`then_1`
                  (bind _ui_bar (`self.UI_Bar`)
                    (:`then`
                      (`/Game/Werewolf/UI/Gameplay/UI_Gage.SetPercent` _ui_bar 1.0))
                    (:`else`)))
                (:`then_2`
                  (`self.lightOn`))))
            (:`then_1`
              (`self.OnSuccess` PC)
              (`GameplayStatics.PlaySound2D` "/Engine/VREditor/Sounds/UI/Flashlight_Switch.Flashlight_Switch" 1.0 1.0 0.0 null null)))
          (else
            (set `self.isSuccess` false)
            (`self.OnFail`)
            (`GameplayStatics.PlaySound2D` "/Engine/EditorSounds/Notifications/CompileFailed.CompileFailed" 1.0 1.0 0.0 null null)
            (`self.SetAlpha` (`self.startAlpha`))))))))

(fn `BPI_CanTouch`
  (returns (can :type Boolean))
  (return (`self.isEnable`)))

(fn `currentAlpha`
  (returns (ReturnValue :type "Float (double-precision)"))
  (return (`KismetMathLibrary.Abs` (mod (+ (`self.startAlpha`) (`self.alpha`)) 1.0))))

(fn `lightOff`
  (`PrimitiveComponent.SetMaterial` (`self.LightMesh1`) 0 "/Game/Werewolf/Materials/M_CableLight_Off.M_CableLight_Off"))

(fn `lightOn`
  (`PrimitiveComponent.SetMaterial` (`self.LightMesh1`) 0 "/Game/Werewolf/Materials/M_CableLight_On.M_CableLight_On"))

(fn `SetAlpha`
  (params (Alpha :type "Float (double-precision)"))
  (`SceneComponent.K2_SetRelativeRotation` (`self.RotateRoot`) (`KismetMathLibrary.MakeRotator` (`KismetMathLibrary.Lerp` 0.0 360.0 Alpha)) false false))

(fn `SetColor`
  (params (ringColor :type "LinearColor Structure"))
  (set `self.ringColor` ringColor)
  (bind _m_ring (`self.M_Ring`)
    (:`then`
      (`MaterialInstanceDynamic.SetVectorParameterValue` _m_ring "Color" (`self.ringColor`)))
    (:`else`)))

(fn `SetNumber`
  (params (number :type Integer))
  (set `self.number` number)
  (`TextRenderComponent.K2_SetText` (`self.TextRender`) (`KismetTextLibrary.Conv_IntToText` (`self.number`))))

(fn `UpdatePercent`
  (bind _returnvalue (/ (`self.randomRange`) 2.0))
  (if (`self.isEnable`)
    (bind _ui_bar (`self.UI_Bar`)
      (:`then`
        (`/Game/Werewolf/UI/Gameplay/UI_Gage.SetPercent` _ui_bar (`KismetMathLibrary.FClamp` (+ (`KismetMathLibrary.SelectFloat` 1.0 0.0 (`self.isSuccess`)) (`KismetMathLibrary.RandomFloatInRange` (* _returnvalue -1.0) _returnvalue)))))
      (:`else`))))

(fn `UserConstructionScript`
  (`|ExecutionSequence`
    (:`then_0`
      (bind _returnvalue (`PrimitiveComponent.CreateDynamicMaterialInstance` (`self.StaticMesh`) 0 null "None"))
      (set `self.M_Ring` _returnvalue))
    (:`then_1`
      (`self.SetColor` (`self.ringColor`)))
    (:`then_2`
      (`self.SetNumber` 0))))