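; Character actor for the Werewolf result scene, showing a configurable mesh with a player color and name label.
; The construction script applies the mesh and animation class from CharacterSettings.
; SetColor creates a dynamic instance of each material and tints it through the parameter name listed at the same index in CharacterSettings.
; SetName stores the name and forwards it to the UI_Name widget cached from the widget component on BeginPlay.
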(event `self.ReceiveBeginPlay`
  (bind _asui_name (cast `/Game/Werewolf/UI/Character/UI_Name` (`WidgetComponent.GetUserWidgetObject` (`self.Widget`))))
  (set `self.UI_Name` _asui_name))

(event `SetColor`
  (params (color :type "LinearColor Structure"))
  (bind _mesh (`self.Mesh`))
  (bind _materialparams (`/Game/Werewolf/DA/PDA_CharacterSettings.MaterialParams` (`self.CharacterSettings`)))
  (set `self.color` color)
  (for (_array_element _array_index) (`MeshComponent.GetMaterials` _mesh)
    (bind _returnvalue (`PrimitiveComponent.CreateDynamicMaterialInstance` _mesh _array_index _array_element "None"))
    (if (`KismetArrayLibrary.Array_IsValidIndex` _materialparams _array_index)
      (`MaterialInstanceDynamic.SetVectorParameterValue` _returnvalue (`KismetStringLibrary.Conv_StringToName` (`|GetArrayItem` _materialparams _array_index)) (`self.color`)))))

(event `SetName`
  (params (name :type String))
  (set `self.name` name)
  (bind _ui_name (`self.UI_Name`)
    (:`then`
      (`/Game/Werewolf/UI/Character/UI_Name.SetName` _ui_name (`self.name`)))
    (:`else`)))

(fn `UserConstructionScript`
  (bind _mesh (`self.Mesh`))
  (bind _charactersettings (`self.CharacterSettings`))
  (`SkinnedMeshComponent.SetSkinnedAssetAndUpdate` _mesh (`/Game/Werewolf/DA/PDA_CharacterSettings.Mesh` _charactersettings) true)
  (`SkeletalMeshComponent.SetAnimInstanceClass` _mesh (`/Game/Werewolf/DA/PDA_CharacterSettings.ABPClass` _charactersettings)))