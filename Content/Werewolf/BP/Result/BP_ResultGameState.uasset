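; Game state for the Werewolf result screen, exposing a ShowResult event that presents the game's outcome.
; It has player 0's result HUD display win or loss, then switches that player's view to the supplied camera.
; It also pairs placed result characters with winner info by array index, setting each name and color and hiding any surplus characters.
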(event `ShowResult`
  (params (WinnerrInfo :type "Array of /Game/Werewolf/BP/Result/s_WinnerInfo Structure") (IsWin :type Boolean) (Camera :type "Actor Object Reference"))
  (bind _returnvalue (`GameplayStatics.GetPlayerController` 0))
  ;[1 1 1] ゲームの結果を表示する
  (`|ExecutionSequence`
    (:`then_0`
      (bind _asbp_result_hud (cast `/Game/Werewolf/BP/Result/BP_ResultHUD` (`PlayerController.GetHUD` _returnvalue))
        (:`then`
          (`/Game/Werewolf/BP/Result/BP_ResultHUD.DisplayResultScreen` _asbp_result_hud IsWin)
          (`PlayerController.SetViewTargetWithBlend` _returnvalue Camera 0.0 "VTBlend_Linear" 0.0 false))
        (:`CastFailed`
          (`KismetSystemLibrary.PrintString` "DisplayResultScreen Failed" true true (struct :`R` 1.0 :`A` 1.0)))))
    (:`then_1`
      (bind _outactors (`GameplayStatics.GetAllActorsOfClass` "/Game/Werewolf/BP/Result/BP_ResultCharacter.BP_ResultCharacter_C"))
      (for (_array_element _array_index) _outactors
        (if (`KismetArrayLibrary.Array_IsValidIndex` WinnerrInfo _array_index)
          (bind (_name _color) (break `/Game/Werewolf/BP/Result/s_WinnerInfo` (`|GetArrayItem` WinnerrInfo _array_index)))
          (`/Game/Werewolf/BP/Result/BP_ResultCharacter.SetName` _array_element _name)
          (`/Game/Werewolf/BP/Result/BP_ResultCharacter.SetColor` _array_element _color)
          (else
            (`self.SetActorHiddenInGame` _array_element true)))))))

(fn `UserConstructionScript`)