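; Game mode for the Werewolf game's result level, showing each player the winners and whether they won, then restarting the match.
; ShowResult passes winner info from the game instance and a "Camera"-tagged actor to the player controller, retrying Initialize if the instance is missing.
; Player controller swaps copy character type, which decides victory against the winning type.
; RestartGame clears result screens, shows loading screens and runs ServerTravel to the gameplay level.
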(event `Initialize`
  ;[1 1 1] 初期化
  (`|ExecutionSequence`
    (:`then_0`
      (bind _asbp_werewolf_game_instance (cast `/Game/Werewolf/BP/BP_WerewolfGameInstance` (`GameplayStatics.GetGameInstance`))
        (:`then`
          (set `self.GI` _asbp_werewolf_game_instance))
        (:`CastFailed`
          (`KismetSystemLibrary.PrintString` "Initialize Failed" true true (struct :`R` 1.0 :`A` 1.0)))))
    (:`then_1`
      (bind _outactors (`GameplayStatics.GetAllActorsWithTag` "Camera"))
      (if (`KismetArrayLibrary.Array_IsValidIndex` _outactors)
        (set `self.Camera` (`|GetArrayItem` _outactors))
        (else
          (`KismetSystemLibrary.PrintString` "Initialize Camera Failed" true true (struct :`R` 1.0 :`A` 1.0)))))))

(event `ShowResult`
  (params (PC :type "/Game/Werewolf/BP/Result/BP_ResultPlayerController Object Reference"))
  ;[1 1 1] ログインしたプレイヤーにゲーム結果を表示する
  (`/Engine/EditorBlueprintResources/StandardMacros.IsValid` PC
    (:`Is Valid`
      (bind _gi (`self.GI`)
        (:`then`
          (`/Game/Werewolf/BP/Result/BP_ResultPlayerController.ShowResultToPlayer` PC (`/Game/Werewolf/BP/BP_WerewolfGameInstance.WinnersInfo` _gi) (`self.GetIsWinPlayer` PC) (`self.Camera`)))
        (:`else`
          (`self.Initialize`)
          (bind _gi_2 (`self.GI`)
            (:`then`
              (`/Game/Werewolf/BP/Result/BP_ResultPlayerController.ShowResultToPlayer` PC (`/Game/Werewolf/BP/BP_WerewolfGameInstance.WinnersInfo` _gi_2) (`self.GetIsWinPlayer` PC) (`self.Camera`)))
            (:`else`
              (`KismetSystemLibrary.PrintString` "ShowGameResult Failed" true true (struct :`R` 1.0 :`A` 1.0)))))))
    (:`Is Not Valid`
      (`KismetSystemLibrary.PrintString` "ShowGameResult Failed" true true (struct :`R` 1.0 :`A` 1.0)))))

(event `self.K2_OnSwapPlayerControllers`
  (params (OldPC :type "PlayerController Object Reference") (NewPC :type "PlayerController Object Reference"))
  ;[1 1 1] プレイヤーのキャラクタータイプを復元
  (`parent.K2_OnSwapPlayerControllers` OldPC NewPC)
  (bind _charactertype (message `/Game/Werewolf/BP/BP_WerewolfInterface.WW_GetCharacterType` OldPC))
  (message `/Game/Werewolf/BP/BP_WerewolfInterface.WW_SetCharacterType` NewPC _charactertype))

(event `RestartGame`
  ;[1 1 1] ゲームを再開する
  (bind _gi (`self.GI`)
    (:`then`
      (for _array_element (`GameStateBase.PlayerArray` (`GameplayStatics.GetGameState`))
        (bind _asbp_result_player_controller (cast `/Game/Werewolf/BP/Result/BP_ResultPlayerController` (`self.GetOwner` _array_element)))
        (`/Game/Werewolf/BP/Result/BP_ResultPlayerController.RemoveResult` _asbp_result_player_controller) ; 全てのプレイヤーの結果画面を削除
        (`/Game/Werewolf/BP/Result/BP_ResultPlayerController.DisplayRoadingScreen` _asbp_result_player_controller))
      (`KismetSystemLibrary.ExecuteConsoleCommand` (`KismetStringLibrary.Concat_StrStr` "ServerTravel " (`/Game/Werewolf/BP/BP_WerewolfGameInstance.GetGameplayLevelName` _gi)) (`GameplayStatics.GetPlayerController` 0)))
    (:`else`
      (`KismetSystemLibrary.PrintString` "RestartGame Failed" true true (struct :`R` 1.0 :`A` 1.0)))))

(fn `GetIsWinPlayer`
  (params (PC :type "/Game/Werewolf/BP/Result/BP_ResultPlayerController Object Reference"))
  (returns (Win :type Boolean))
  (`/Engine/EditorBlueprintResources/StandardMacros.IsValid` PC
    (:`Is Valid`
      (bind _gi (`self.GI`)
        (:`then`
          (return (`|EnumEquality` (`/Game/Werewolf/BP/Result/BP_ResultPlayerController.Character Type` PC) (`/Game/Werewolf/BP/BP_WerewolfGameInstance.WinnerCharacterType` _gi))))
        (:`else`
          (return false))))
    (:`Is Not Valid`
      (return false))))

(fn `UserConstructionScript`)