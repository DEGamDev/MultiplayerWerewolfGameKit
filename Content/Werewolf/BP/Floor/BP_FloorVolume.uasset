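; Room volume actor for the Werewolf game that seals a room by closing its assigned Doors and reopens it later.
; CloseDoors starts a timer for the closed period, and OpenFloor reopens the doors and starts a cooldown timer, whose end is broadcast via OnEndCooldown.
; Getters expose whether it can close, the remaining cooldown fraction and door update state.
; The construction script sets the volume mesh, with an optional preview material.
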(event `CloseDoors`
  (params (CoolTime :type Integer) (CloseTime :type Integer))
  ;[1 1 1] 部屋を封鎖する
  (set `self.IsOpen` false)
  (set `self.Cooldown` CoolTime)
  (for _array_element (`self.doors`)
    (`/Engine/EditorBlueprintResources/StandardMacros.IsValid` _array_element
      (:`Is Valid`
        (`/Game/Werewolf/BP/Door/BP_Door.Close` _array_element))))
  (bind _returnvalue (`KismetSystemLibrary.K2_SetTimerDelegate` (`|CreateDelegate` :!event `OpenFloor`) (`KismetMathLibrary.Conv_IntToDouble` CloseTime)))
  (set `self.openFloorTimer` _returnvalue))

(event `EndCoolDown`
  ;[1 1 1] クールダウンを終える
  (set `self.IsCooldown` false)
  (`self.OnEndCooldown` self))

(event `Initialize`
  ;[1 1 1] 部屋を初期化
  (set `self.Cooldown` 0)
  (set `self.IsCooldown` false) ; クールダウン中ではない
  (set `self.IsOpen` true) ; 部屋を開放している
  (`KismetSystemLibrary.K2_ClearAndInvalidateTimerHandle` (`self.openFloorTimer`)) ; 部屋を開放するタイマーを削除
  (`KismetSystemLibrary.K2_ClearAndInvalidateTimerHandle` (`self.coolDownTimer`)) ; 部屋を封鎖するクールダウンを削除
)

(event `OpenAllFloors`
  ;[1 0.1543 0.1244] 全てのドアを開ける
  (for _array_element (`self.doors`)
    (`/Engine/EditorBlueprintResources/StandardMacros.IsValid` _array_element
      (:`Is Valid`
        (`/Game/Werewolf/BP/Door/BP_Door.InitializeDoor` _array_element)))))

(event `OpenFloor`
  ;[1 1 1] 部屋を解放する
  (set `self.IsOpen` true)
  (for _array_element (`self.doors`)
    (`/Engine/EditorBlueprintResources/StandardMacros.IsValid` _array_element
      (:`Is Valid`
        (`/Game/Werewolf/BP/Door/BP_Door.Open` _array_element))))
  (bind _returnvalue (`KismetSystemLibrary.K2_SetTimerDelegate` (`|CreateDelegate` :!event `EndCoolDown`) (`KismetMathLibrary.Conv_IntToDouble` (`self.Cooldown`)))) ; クールダウンを開始
  (set `self.coolDownTimer` _returnvalue)
  (set `self.IsCooldown` true))

(fn `CanClose`
  (returns (Can :type Boolean))
  (return (and (`self.GetIsOpen`) (not (`self.GetisCoolDown`)))))

(fn `Get Floor Is Update Opening`
  (returns (Update :type Boolean))
  (for _array_element (`self.doors`)
    (`/Engine/EditorBlueprintResources/StandardMacros.IsValid` _array_element
      (:`Is Valid`
        (if (`/Game/Werewolf/BP/Door/BP_Door.GetIs Update Opening` _array_element)
          (return true)))))
  (return false))

(fn `GetCooldown`
  (returns (Cooldown :type "Float (double-precision)"))
  (bind _cooldowntimer (`self.coolDownTimer`))
  (if (`KismetSystemLibrary.K2_TimerExistsHandle` _cooldowntimer)
    (return (/ (`KismetSystemLibrary.K2_GetTimerRemainingTimeHandle` _cooldowntimer) (`self.Cooldown`)))
    (else
      (return 0.0))))

(fn `GetisCoolDown`
  (returns (Cooldown :type Boolean))
  (return (`self.IsCooldown`)))

(fn `GetIsOpen`
  (returns (Open :type Boolean))
  (return (`self.IsOpen`)))

(fn `UserConstructionScript`
  (bind _floormesh (`self.FloorMesh`))
  (`StaticMeshComponent.SetStaticMesh` _floormesh (`self.FloorVolume`))
  (if (`self.IsPreview`)
    (`PrimitiveComponent.SetMaterial` _floormesh 0 "/Engine/EditorResources/FieldNodes/_Resources/M_FieldRadiusPreview.M_FieldRadiusPreview")
    (`SceneComponent.SetVisibility` _floormesh true false)))