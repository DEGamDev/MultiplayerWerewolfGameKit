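; Hatch actor for the Werewolf game, which opens and closes on request and exposes the list of hatches that can be moved to from it.
; WW interface events drive a timeline that swings HatchRoot up to 90 degrees in pitch, at a rate set on authority from OpenSpeed, and trigger sounds via the passed PlayerController.
; The construction script applies the mesh; other shared interface functions are mostly default stubs, with IsHatch returning true.
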(event `self.ReceiveBeginPlay`
  ;[1 0.2766 0] BeginPlay
  (`/Engine/EditorBlueprintResources/ActorMacros.Switch Has Authority`
    (:`Authority`
      (`TimelineComponent.SetPlayRate` (`self.TL_Open`) (/ 1.0 (`self.OpenSpeed`))) ; 開く速度をセット
    )))

(event `/Game/Werewolf/BP/BP_WerewolfInterface.WW_OpenHatch`
  (params (PC :type "/Game/Werewolf/BP/Gameplay/BP_GameplayPlayerController Object Reference"))
  ;[1 0.1976 0.2175] 開く
  (`self.Open` PC))

(event `Open`
  (params (PC :type "/Game/Werewolf/BP/Gameplay/BP_GameplayPlayerController Object Reference"))
  ;[1 0.1976 0.2175] 開く
  (`TimelineComponent.PlayFromStart` (`self.TL_Open`))
  (`/Engine/EditorBlueprintResources/StandardMacros.IsValid` PC
    (:`Is Valid`
      (`/Game/Werewolf/BP/Gameplay/BP_GameplayPlayerController.PlayHatchOpenSound` PC))))

(event `/Game/Werewolf/BP/BP_WerewolfInterface.WW_CloseHatch`
  (params (PC :type "/Game/Werewolf/BP/Gameplay/BP_GameplayPlayerController Object Reference"))
  ;[1 0.1557 0.1458] 閉じる
  (`self.Close` PC))

(event `Close`
  (params (PC :type "/Game/Werewolf/BP/Gameplay/BP_GameplayPlayerController Object Reference"))
  ;[1 0.1557 0.1458] 閉じる
  (`TimelineComponent.ReverseFromEnd` (`self.TL_Open`))
  (`/Engine/EditorBlueprintResources/StandardMacros.IsValid` PC
    (:`Is Valid`
      (`/Game/Werewolf/BP/Gameplay/BP_GameplayPlayerController.PlayHatchCloseSound` PC))))

(event `PlayOpenSound`
  ;[0.217 0.3564 1] 開ける音を再生
  (`GameplayStatics.PlaySound2D` (`self.OpenSound`) 1.0 1.0 0.0 null null))

(event `PlayCloseSound`
  ;[0.217 0.3564 1] 閉じる音を再生
  (`GameplayStatics.PlaySound2D` (`self.CloseSound`) 1.0 1.0 0.0 null null))

(fn `GetCanMovingHatches`
  (returns (CanMovingHatches :type "Array of Actor Object Reference"))
  (return (`self.CanMovingHatches`)))

(fn `UserConstructionScript`
  (`StaticMeshComponent.SetStaticMesh` (`self.HatchMesh`) (`self.Mesh`)))

(fn `WW_GetAllCharacters`
  (returns (Characters :type "Array of Actor Object Reference"))
  (return))

(fn `WW_GetAllPC`
  (returns (PC :type "Array of Actor Object Reference"))
  (return))

(fn `WW_GetAllPlayersCount`
  (returns (Count :type Integer))
  (return 0))

(fn `WW_GetAllWolfs`
  (returns (Wolfs :type "Array of Actor Object Reference"))
  (return))

(fn `WW_GetCanMovingHatches`
  (returns (Hatches :type "Array of Actor Object Reference"))
  (return (`self.GetCanMovingHatches`)))

(fn `WW_GetCanUseEmergencyButton`
  (params (UsedCount :type Integer))
  (returns (Can :type Boolean))
  (return false))

(fn `WW_GetCharacterType`
  (returns (CharacterType :type "/Game/Werewolf/Enum/e_CharacterType Enum"))
  (return "NewEnumerator1"))

(fn `WW_GetCompletedTaskCount`
  (returns (Count :type Integer))
  (return 0))

(fn `WW_GetEmergencyButton`
  (returns (EmergencyButton :type "Actor Object Reference"))
  (return null))

(fn `WW_GetEmergencyMeetingCoolTime`
  (returns (Time :type Integer))
  (return 0))

(fn `WW_GetEmergencyTasks`
  (returns (Tasks :type "Array of Actor Object Reference"))
  (return))

(fn `WW_GetGameSettings`
  (returns (GameSettings :type "Actor Object Reference"))
  (return null))

(fn `WW_GetIsCharacterCapsule`
  (params (Comp :type "SceneComponent Object Reference"))
  (returns (NewParam :type Boolean))
  (return false))

(fn `WW_GetIsDead`
  (returns (IsDead :type Boolean))
  (return false))

(fn `WW_GetIsEmergencyTaskCoolDown`
  (returns (IsCoolDown :type Boolean))
  (return false))

(fn `WW_GetIsEnableTask`
  (returns (IsEnable :type Boolean))
  (return false))

(fn `WW_GetIsGameFinished`
  (returns (IsGameFinished :type Boolean))
  (return false))

(fn `WW_GetIsInGame`
  (returns (IsInGame :type Boolean))
  (return false))

(fn `WW_GetIsInHatch`
  (returns (IsIn :type Boolean))
  (return false))

(fn `WW_GetIsInMeeting`
  (returns (In :type Boolean))
  (return false))

(fn `WW_GetIsInVotingTime`
  (returns (In :type Boolean))
  (return false))

(fn `WW_GetIsKillCoolDown`
  (returns (CoolDown :type Boolean))
  (return false))

(fn `WW_GetIsKilling`
  (returns (Killing :type Boolean))
  (return false))

(fn `WW_GetIsPlayerStart`
  (returns (NewParam :type Boolean))
  (return false))

(fn `WW_GetIsPutHand`
  (returns (IsPut :type Boolean))
  (return false))

(fn `WW_GetIsSabotageCoolDown`
  (returns (IsCoolDown :type Boolean))
  (return false))

(fn `WW_GetIsTaskManager`
  (returns (NewParam :type Boolean))
  (return false))

(fn `WW_GetIsUseCamera`
  (returns (Use :type Boolean))
  (return false))

(fn `WW_GetIsValidEmergencyTimer`
  (returns (IsValid :type Boolean))
  (return false))

(fn `WW_GetIsVotedToPlayer`
  (returns (NewParam :type Boolean))
  (return false))

(fn `WW_GetKillCoolDownTime`
  (returns (Time :type Integer))
  (return 0))

(fn `WW_GetMovingSpeed`
  (returns (Speed :type "Float (double-precision)"))
  (return 0.0))

(fn `WW_GetOverlapHatch`
  (returns (Hatch :type "/Game/Werewolf/BP/Hatch/BP_Hatch Object Reference"))
  (return null))

(fn `WW_GetPCByIndex`
  (params (Index :type Integer))
  (returns (PC :type "Actor Object Reference"))
  (return null))

(fn `WW_GetPlayerColorByIndex`
  (params (Index :type Integer))
  (returns (Color :type "LinearColor Structure"))
  (return))

(fn `WW_GetPlayerIndex`
  (returns (Index :type Integer))
  (return 0))

(fn `WW_GetPlayerName`
  (returns (Name :type String))
  (return ""))

(fn `WW_GetPlayerStarts`
  (returns (PlayerStarts :type "Array of Actor Object Reference"))
  (return))

(fn `WW_GetReportTarget`
  (returns (ReportTarget :type "Actor Object Reference"))
  (return null))

(fn `WW_GetSabotageCooldownPercent`
  (returns (Percent :type "Float (double-precision)"))
  (return 0.0))

(fn `WW_GetTask`
  (returns (Task :type "Actor Object Reference"))
  (return null))

(fn `WW_GetTaskManagers`
  (returns (TaskManagers :type "Array of Actor Object Reference"))
  (return))

(fn `WW_GetTaskUIClass`
  (returns (TaskUIClass :type "UserWidget Class Reference"))
  (return null))

(fn `WW_GetVotedFromPlayerCount`
  (returns (Count :type Integer))
  (return 0))

(fn `WW_GetVotedFromPlayerIndex`
  (returns (Index :type "Array of Integer"))
  (return))

(fn `WW_GetVoteTime`
  (returns (Time :type Integer))
  (return 0))

(fn `WW_IsCompleted`
  (returns (Completed :type Boolean))
  (return false))

(fn `WW_IsCompletedAllTask`
  (returns (IsCompleted :type Boolean))
  (return false))

(fn `WW_IsControlledCharacter`
  (returns (ReturnValue :type Boolean))
  (return false))

(fn `WW_IsEmergencyButton`
  (returns (NewParam :type Boolean))
  (return false))

(fn `WW_IsEmergencyTask`
  (returns (NewParam :type Boolean))
  (return false))

(fn `WW_IsGameSettings`
  (returns (ReturnValue :type Boolean))
  (return false))

(fn `WW_IsHatch`
  (returns (IsHatch :type Boolean))
  (return true))

(fn `WW_IsReportSphere`
  (params (Comp :type "PrimitiveComponent Object Reference"))
  (returns (NewParam :type Boolean))
  (return false))

(fn `WW_IsTask`
  (returns (NewParam :type Boolean))
  (return false))

(fn `WW_IsValidDeadBody`
  (returns (Valid :type Boolean))
  (return false))

(fn `WW_IsVillager`
  (returns (IsVillager :type Boolean))
  (return false))

(fn `WW_IsWolf`
  (returns (Wolf :type Boolean))
  (return false))

(fn `WW_SetHatchButtonAngle`
  (params (Angle :type "Float (double-precision)"))
  (return))

(fn `WW_SpawnPlayers`
  (returns (Vilagers :type "Array of /Game/Werewolf/BP/Character/BP_Villager Object Reference") (Wolfs :type "Array of /Game/Werewolf/BP/Character/BP_Wolf Object Reference"))
  (return))