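; BP_Door is a double sliding door that opens and closes with a sound at its location.
; Guarded Open and Close events play or reverse a timeline, whose alpha feeds UpdateDoorOpen to slide both door roots apart along local Y by Length.
; The construction script assigns one mesh to both leaves and applies the IsOpen pose, which SetOpen also snaps to without animation.
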(event `self.ReceiveBeginPlay`
  (`/Engine/EditorBlueprintResources/ActorMacros.Switch Has Authority`))

(event `InitializeDoor`
  (bind _tl_open (`self.TL_Open`))
  ;[1 0.1543 0.1244] ドアを初期化
  (`TimelineComponent.Stop` _tl_open)
  (`TimelineComponent.SetPlaybackPosition` _tl_open 1.0 false true) ; ドアを開閉している途中の状態で止まってしまうのを防ぐ
)

(event `Open`
  ;[1 0.1543 0.1244] ドアを開く
  (if (not (`self.isOpen`))
    (set `self.isOpen` true)
    (`TimelineComponent.PlayFromStart` (`self.TL_Open`))
    (`self.PlayOpenSound`)))

(event `PlayOpenSound`
  ;[0.4557 0.2946 1] ドアを開く音を再生
  (`GameplayStatics.PlaySoundAtLocation` (`self.OpenSound`) (`self.K2_GetActorLocation`) (struct) 0.5 1.0 0.0 null null null null))

(event `Close`
  ;[1 0.1543 0.1244] ドアを閉じる
  (if (`self.isOpen`)
    (set `self.isOpen` false)
    (`TimelineComponent.ReverseFromEnd` (`self.TL_Open`))
    (`self.PlayCloseSound`)))

(event `PlayCloseSound`
  ;[0.4557 0.2946 1] ドアを閉じる音を再生
  (`GameplayStatics.PlaySoundAtLocation` "/Game/Werewolf_01/Sound/Door_Open.Door_Open" (`self.K2_GetActorLocation`) (struct) 0.5 1.0 0.0 null null null null))

(event `InitializeOpen`
  ;[1 0.1543 0.1244] ドアの開閉を初期化
  (if (`self.isOpen`)
    (`self.UpdateDoorOpen` 1.0)
    (else
      (`self.UpdateDoorOpen` 0.0))))

(event `SetOpen`
  (params (Open :type Boolean))
  ;[1 0.1543 0.1244] ドアの開閉をセット
  (set `self.isOpen` Open)
  (`self.InitializeOpen`))

(fn `GetIs Update Opening`
  (returns (Update :type Boolean))
  (return (`TimelineComponent.IsPlaying` (`self.TL_Open`))))

(fn `GetIsOpen`
  (returns (Open :type Boolean))
  (return (`self.isOpen`)))

(fn `UpdateDoorOpen`
  (params (Alpha :type "Float (double-precision)"))
  (bind _returnvalue (`KismetMathLibrary.Lerp` 0.0 (`self.length`) Alpha))
  (`|ExecutionSequence`
    (:`then_0`
      (`SceneComponent.K2_SetRelativeLocation` (`self.RightDoorRoot`) (`KismetMathLibrary.MakeVector` 0.0 _returnvalue) false false))
    (:`then_1`
      (`SceneComponent.K2_SetRelativeLocation` (`self.LeftDoorRoot`) (`KismetMathLibrary.MakeVector` 0.0 (* _returnvalue -1.0)) false false))))

(fn `UserConstructionScript`
  (bind _doormesh (`self.DoorMesh`))
  ;[1 1 1] ドアのメッシュをセット
  (`StaticMeshComponent.SetStaticMesh` (`self.LeftDoorMesh`) _doormesh)
  (`StaticMeshComponent.SetStaticMesh` (`self.RightDoorMesh`) _doormesh)
  (`self.InitializeOpen`))