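; Game settings actor for the werewolf game, holding match tunables such as role counts, timings, speed and player colors, served through interface getters.
; On BeginPlay, the authority seeds the GameMode's alive villager and wolf counts.
; SpawnPlayers shuffles GameMode player starts, spawns wolves then villagers, and passes itself to each pawn.
; Sabotage cooldown and in-game events are empty stubs, with the cooldown timer and wolf-screen logic left unwired.
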(event `self.ReceiveBeginPlay`
  (bind _returnvalue (`GameplayStatics.GetGameMode`))
  (`/Engine/EditorBlueprintResources/ActorMacros.Switch Has Authority`
    (:`Authority`
      (message `/Game/Werewolf_01/BP/BP_WerewolfInterface.WW_SetAliveVillagersCount` _returnvalue (`self.GetVillagerCount`)) ; 生存している村人の数を初期化
      (message `/Game/Werewolf_01/BP/BP_WerewolfInterface.WW_SetAliveWolfCount` _returnvalue (`self.GetWolfCount`)) ; 生存している狼の数を初期化
    )))

(event `/Game/Werewolf_01/BP/BP_WerewolfInterface.WW_SetIsInGame`
  (params (IsInGame :type Boolean))
  ;[1 0.2272 0.1973] ゲーム中かをセット
  (`self.SetIsInGame` IsInGame))

(event `SetIsInGame`
  (params (IsInGame :type Boolean))
  ;[1 0.2272 0.1973] ゲーム中かをセット
)

(event `/Game/Werewolf_01/BP/BP_WerewolfInterface.WW_StartSabotageCooldown`
  ;[1 0.2384 0.2185] 妨害のクールダウンを開始する
  (`self.StartSabotageCooldown`))

(event `StartSabotageCooldown`
  ;[1 0.2384 0.2185] 妨害のクールダウンを開始する
)

(event `EndSabotageCooldown`
  ;[1 0.2384 0.2185] 妨害のクールダウンを終了する
)

(event `/Game/Werewolf_01/BP/BP_WerewolfInterface.WW_ClearSabotageCooldown`
  ;[1 0.2384 0.2185] 妨害のクールダウンを削除する
  (`self.ClearSabotageCooldown`))

(event `ClearSabotageCooldown`
  ;[1 0.2384 0.2185] 妨害のクールダウンを削除する
)

(event `RemoveAllWolfSabotageCooldownScreen`
  ;[1 0.2395 0.2495] 全ての狼のサボタージュのクールダウンを非表示
  (bind _pc (message `/Game/Werewolf_01/BP/BP_WerewolfInterface.WW_GetAllPC` (`GameplayStatics.GetGameMode`)))
  (for _array_element _pc
    (bind _wolf (message `/Game/Werewolf_01/BP/BP_WerewolfInterface.WW_IsWolf` _array_element))
    (if _wolf
      (message `/Game/Werewolf_01/BP/BP_WerewolfInterface.WW_RemoveSabotageCooldown` _array_element))))

(fn `GetCanUseEmergencyButtonCount`
  (returns (CanUseEmergencyButtonCount :type Integer))
  (return (`self.CanUseEmergencyButtonCount`)))

(fn `GetColors`
  (returns (Colors :type "Array of LinearColor Structure"))
  (return (`self.Colors`)))

(fn `GetCompletedTaskPercentUpdateTiming`
  (returns (Timing :type "/Game/Werewolf_01/Enum/e_CompletedTaskPercentUpdateTiming Enum"))
  (return (`self.CompletedTaskPercentUpdateTiming`)))

(fn `GetEmergencyMeetingCoolTime`
  (returns (EmergencyMeetingCoolTime :type Integer))
  (return (`self.EmergencyMeetingCoolTime`)))

(fn `GetKillCoolDownTime`
  (returns (Time :type Integer))
  (return (`self.KillCoolDownTime`)))

(fn `GetMapUIClass`
  (returns (MapUIClass :type "/Game/Werewolf_01/UI/Gameplay/Map/UI_MiniMap Class Reference"))
  (return (`self.UI_MiniMapClass`)))

(fn `GetMovingSpeed`
  (returns (MovingSpeed :type "Float (double-precision)"))
  (return (`self.MovingSpeed`)))

(fn `GetPlayerStarts`
  (returns (OutActors :type "Array of Actor Object Reference"))
  (bind _playerstarts (message `/Game/Werewolf_01/BP/BP_WerewolfInterface.WW_GetPlayerStarts` (`GameplayStatics.GetGameMode`)))
  (return _playerstarts))

(fn `GetVillagerCount`
  (returns (VillagerCount :type Integer))
  (return (`self.VillagerCount`)))

(fn `GetVoteTime`
  (returns (VoteTime :type Integer))
  (return (`self.VoteTime`)))

(fn `GetWolfCount`
  (returns (WolfCount :type Integer))
  (return (`self.WolfCount`)))

(fn `SpawnPlayers`
  (returns (Wolfs1 :type "Array of /Game/Werewolf_01/BP/Character/BP_Wolf Object Reference") (Villagers1 :type "Array of /Game/Werewolf_01/BP/Character/BP_Villager Object Reference"))
  (locals (NewLocalVar_0 :type "Array of Actor Object Reference") (Wolfs :type "Array of /Game/Werewolf_01/BP/Character/BP_Wolf Object Reference") (Villagers :type "Array of /Game/Werewolf_01/BP/Character/BP_Villager Object Reference"))
  (bind _newlocalvar_0 (`local.NewLocalVar_0`))
  (bind _newlocalvar_0_2 (`local.NewLocalVar_0`))
  (`|ExecutionSequence`
    (:`then_0`
      (bind _output_get (set `local.NewLocalVar_0` (`self.GetPlayerStarts`)))
      (`KismetArrayLibrary.Array_Shuffle` _output_get))
    (:`then_1`
      ;[1 1 1] Spawn Wolf
      (for _index (range (`self.WolfCount`))
        (if (`KismetArrayLibrary.Array_IsValidIndex` _newlocalvar_0_2 _index)
          (bind _returnvalue (`|SpawnActorFromClass` "/Game/Werewolf_01/BP/Character/BP_Wolf.BP_Wolf_C" (`self.GetTransform` (`|GetArrayItem` _newlocalvar_0_2 _index)) "Undefined" "OverrideRootScale" null null))
          (`KismetArrayLibrary.Array_Add` (`local.Wolfs`) _returnvalue)
          (message `/Game/Werewolf_01/BP/BP_WerewolfInterface.WW_ApplyGameSettings` _returnvalue self))))
    (:`then_2`
      ;[1 1 1] Spawn Wolf
      (for _index_2 (range (`self.VillagerCount`))
        (bind _returnvalue_2 (+ (`self.WolfCount`) _index_2))
        (if (`KismetArrayLibrary.Array_IsValidIndex` _newlocalvar_0 _returnvalue_2)
          (bind _returnvalue_3 (`|SpawnActorFromClass` "/Game/Werewolf_01/BP/Character/BP_Villager.BP_Villager_C" (`self.GetTransform` (`|GetArrayItem` _newlocalvar_0 _returnvalue_2)) "Undefined" "OverrideRootScale" null null))
          (`KismetArrayLibrary.Array_Add` (`local.Villagers`) _returnvalue_3)
          (message `/Game/Werewolf_01/BP/BP_WerewolfInterface.WW_ApplyGameSettings` _returnvalue_3 self))))
    (:`then_3`
      (return (`local.Wolfs`) (`local.Villagers`)))))

(fn `UserConstructionScript`)

(fn `WW_GetAllCharacters`
  (returns (Characters :type "Array of Actor Object Reference"))
  (return))

(fn `WW_GetAllPC`
  (returns (PC :type "Array of Actor Object Reference"))
  (return))

(fn `WW_GetAllPlayersCount`
  (returns (Count :type Integer))
  (return (+ (`self.GetWolfCount`) (`self.GetVillagerCount`))))

(fn `WW_GetAllWolfs`
  (returns (Wolfs :type "Array of Actor Object Reference"))
  (return))

(fn `WW_GetCanMovingHatches`
  (returns (Hatches :type "Array of Actor Object Reference"))
  (return))

(fn `WW_GetCanUseEmergencyButton`
  (params (UsedCount :type Integer))
  (returns (Can :type Boolean))
  (return false))

(fn `WW_GetCharacterType`
  (returns (CharacterType :type "/Game/Werewolf_01/Enum/e_CharacterType Enum"))
  (return "NewEnumerator1"))

(fn `WW_GetCompletedTaskCount`
  (returns (Count :type Integer))
  (return 0))

(fn `WW_GetEmergencyButton`
  (returns (EmergencyButton :type "Actor Object Reference"))
  (return null))

(fn `WW_GetEmergencyMeetingCoolTime`
  (returns (Time :type Integer))
  (return (`self.GetEmergencyMeetingCoolTime`)))

(fn `WW_GetEmergencyTasks`
  (returns (Tasks :type "Array of Actor Object Reference"))
  (return))

(fn `WW_GetGameSettings`
  (returns (GameSettings :type "Actor Object Reference"))
  (return null))

(fn `WW_GetIsCharacterCapsule`
  (params (Comp :type "SceneComponent Object Reference"))
  (returns (NewParam :type Boolean))
  (return false))

(fn `WW_GetIsDead`
  (returns (IsDead :type Boolean))
  (return false))

(fn `WW_GetIsEmergencyTaskCoolDown`
  (returns (IsCoolDown :type Boolean))
  (return false))

(fn `WW_GetIsEnableTask`
  (returns (IsEnable :type Boolean))
  (return false))

(fn `WW_GetIsGameFinished`
  (returns (IsGameFinished :type Boolean))
  (return false))

(fn `WW_GetIsInGame`
  (returns (IsInGame :type Boolean))
  (return false))

(fn `WW_GetIsInHatch`
  (returns (IsIn :type Boolean))
  (return false))

(fn `WW_GetIsInMeeting`
  (returns (In :type Boolean))
  (return false))

(fn `WW_GetIsInVotingTime`
  (returns (In :type Boolean))
  (return false))

(fn `WW_GetIsKillCoolDown`
  (returns (CoolDown :type Boolean))
  (return false))

(fn `WW_GetIsKilling`
  (returns (Killing :type Boolean))
  (return false))

(fn `WW_GetIsPlayerStart`
  (returns (NewParam :type Boolean))
  (return false))

(fn `WW_GetIsPutHand`
  (returns (IsPut :type Boolean))
  (return false))

(fn `WW_GetIsSabotageCoolDown`
  (returns (IsCoolDown :type Boolean))
  (return false))

(fn `WW_GetIsTaskManager`
  (returns (NewParam :type Boolean))
  (return false))

(fn `WW_GetIsUseCamera`
  (returns (Use :type Boolean))
  (return false))

(fn `WW_GetIsValidEmergencyTimer`
  (returns (IsValid :type Boolean))
  (return false))

(fn `WW_GetIsVotedToPlayer`
  (returns (NewParam :type Boolean))
  (return false))

(fn `WW_GetKillCoolDownTime`
  (returns (Time :type Integer))
  (return (`self.GetKillCoolDownTime`)))

(fn `WW_GetMovingSpeed`
  (returns (Speed :type "Float (double-precision)"))
  (return (`self.GetMovingSpeed`)))

(fn `WW_GetOverlapHatch`
  (returns (Hatch :type "/Game/Werewolf_01/BP/Hatch/BP_Hatch Object Reference"))
  (return null))

(fn `WW_GetPCByIndex`
  (params (Index :type Integer))
  (returns (PC :type "Actor Object Reference"))
  (return null))

(fn `WW_GetPlayerColorByIndex`
  (params (Index :type Integer))
  (returns (Color :type "LinearColor Structure"))
  (bind _colors (`self.Colors`))
  (if (`KismetArrayLibrary.Array_IsValidIndex` _colors Index)
    (return (`|GetArrayItem` _colors Index))
    (else
      (return))))

(fn `WW_GetPlayerIndex`
  (returns (Index :type Integer))
  (return 0))

(fn `WW_GetPlayerName`
  (returns (Name :type String))
  (return ""))

(fn `WW_GetPlayerStarts`
  (returns (PlayerStarts :type "Array of Actor Object Reference"))
  (return))

(fn `WW_GetReportTarget`
  (returns (ReportTarget :type "Actor Object Reference"))
  (return null))

(fn `WW_GetSabotageCooldownPercent`
  (returns (Percent :type "Float (double-precision)"))
  ;[1 1 1] 妨害クールダウンの残り時間の割合
  (return (/ (`KismetSystemLibrary.K2_GetTimerRemainingTime` null "EndSabotageCooldown") (`KismetMathLibrary.Conv_IntToDouble` 0))))

(fn `WW_GetTask`
  (returns (Task :type "Actor Object Reference"))
  (return null))

(fn `WW_GetTaskManagers`
  (returns (TaskManagers :type "Array of Actor Object Reference"))
  (return))

(fn `WW_GetTaskUIClass`
  (returns (TaskUIClass :type "UserWidget Class Reference"))
  (return null))

(fn `WW_GetVotedFromPlayerCount`
  (returns (Count :type Integer))
  (return 0))

(fn `WW_GetVotedFromPlayerIndex`
  (returns (Index :type "Array of Integer"))
  (return))

(fn `WW_GetVoteTime`
  (returns (Time :type Integer))
  (return (`self.GetVoteTime`)))

(fn `WW_IsCompleted`
  (returns (Completed :type Boolean))
  (return false))

(fn `WW_IsCompletedAllTask`
  (returns (IsCompleted :type Boolean))
  (return false))

(fn `WW_IsControlledCharacter`
  (returns (ReturnValue :type Boolean))
  (return false))

(fn `WW_IsEmergencyButton`
  (returns (NewParam :type Boolean))
  (return false))

(fn `WW_IsEmergencyTask`
  (returns (NewParam :type Boolean))
  (return false))

(fn `WW_IsGameSettings`
  (returns (ReturnValue :type Boolean))
  (return true))

(fn `WW_IsHatch`
  (returns (IsHatch :type Boolean))
  (return false))

(fn `WW_IsReportSphere`
  (params (Comp :type "PrimitiveComponent Object Reference"))
  (returns (NewParam :type Boolean))
  (return false))

(fn `WW_IsTask`
  (returns (NewParam :type Boolean))
  (return false))

(fn `WW_IsValidDeadBody`
  (returns (Valid :type Boolean))
  (return false))

(fn `WW_IsVillager`
  (returns (IsVillager :type Boolean))
  (return false))

(fn `WW_IsWolf`
  (returns (Wolf :type Boolean))
  (return false))

(fn `WW_SpawnPlayers`
  (returns (Vilagers :type "Array of /Game/Werewolf_01/BP/Character/BP_Villager Object Reference") (Wolfs :type "Array of /Game/Werewolf_01/BP/Character/BP_Wolf Object Reference"))
  (bind (_wolfs1 _villagers1) (`self.SpawnPlayers`))
  (return _villagers1 _wolfs1))