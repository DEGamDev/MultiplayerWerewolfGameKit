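; BP_Switch is a touchable lever switch with an indicator lamp that players flip on and off.
; A press, gated by CanTouch, inverts IsOn, requests the toggle sound through the player controller and calls OnToggle with that controller.
; IsOn's RepNotify updates the lamp's dynamic material color and brightness and tilts the lever, with IsOnLow reversing its direction.
; The construction script creates that material and applies the initial state.
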(event `CreateRampMI`
  ;[1 1 1] ランプのマテリアルを作成
  (bind _returnvalue (`PrimitiveComponent.CreateDynamicMaterialInstance` (`self.RampMesh`) 0 null "None"))
  (set `self.M_ramp` _returnvalue))

(event `/Game/Werewolf_01/BP/BP_TouchInterface.TCH_Presse`
  (params (PC :type "/Game/Werewolf_01/BP/Gameplay/BP_GameplayPlayerController Object Reference") (TouchComp :type "SceneComponent Object Reference"))
  ;[1 1 1] スイッチを押したとき、スイッチを切り替える
  (`self.ToggleSwitch` PC))

(event `ToggleSwitch`
  (params (PC :type "/Game/Werewolf_01/BP/Gameplay/BP_GameplayPlayerController Object Reference"))
  ;[1 0.1543 0.1244] スイッチを切り替える
  (if (`self.canTouch`)
    (`|ExecutionSequence`
      (:`then_0`
        (set `self.isOn` (not (`self.isOn`)))
        (`/Game/Werewolf_01/BP/Gameplay/BP_GameplayPlayerController.PlayToggleSwitchSoundToPlayer` PC self))
      (:`then_1`
        (`self.OnToggle` PC)))))

(event `PlayToggleSwitchSound`
  ;[0.2026 0.2461 1] スイッチを切り替えたときの音を再生
  (`GameplayStatics.PlaySound2D` "/Game/Werewolf_01/Interface_And_Item_Sounds/Cues/Flick_Switch_05_Cue.Flick_Switch_05_Cue" 1.0 1.0 0.0 null null))

(event `SetIsOn`
  (params (On :type Boolean))
  ;[1 0.1543 0.1244] ライトが点灯しているかをセット
  (set `self.isOn` On))

(fn `BPI_CanTouch`
  (returns (can :type Boolean))
  (return (`self.canTouch`)))

(fn `OnRep_isOn`
  (`self.updateIsOn`))

(fn `updateIsOn`
  (bind _leverangle (`self.leverAngle`))
  (bind _returnvalue (`KismetMathLibrary.SelectFloat` (* _leverangle -1.0) _leverangle (`self.isOn`)))
  (`|ExecutionSequence`
    (:`then_0`
      (bind _m_ramp (`self.M_ramp`)
        (:`then`
          (`MaterialInstanceDynamic.SetVectorParameterValue` _m_ramp "Color" (`KismetMathLibrary.SelectColor` (struct :`G` 1.0 :`B` 0.013358 :`A` 1.0) (struct :`R` 0.001689 :`G` 0.03125 :`A` 1.0) (`self.isOn`)))
          (`MaterialInstanceDynamic.SetScalarParameterValue` _m_ramp "Brightness" (`KismetMathLibrary.SelectFloat` 1.0 0.0 (`self.isOn`))))
        (:`else`)))
    (:`then_1`
      (`SceneComponent.K2_SetRelativeRotation` (`self.SwitchRoot`) (`KismetMathLibrary.MakeRotator` 0.0 (`KismetMathLibrary.SelectFloat` _returnvalue (* _returnvalue -1.0) (`self.isOnLow`))) false false))))

(fn `UserConstructionScript`
  (`parent.UserConstructionScript`)
  (`self.CreateRampMI`)
  (`self.updateIsOn`))