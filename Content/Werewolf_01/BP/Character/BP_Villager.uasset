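; Villager character for the werewolf game, a child Blueprint that handles being killed by a wolf and leaving a body behind.
; On death it becomes a ghost, spawns a detached DeadBody-tagged capsule at its location and notifies the GM to update the villager count and check for game end.
; After the death montage, a copied skeletal mesh follows the hidden original's pose as the corpse, removable via ClearDeadBody.
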(event `self.InitializeCharacterState`
  ;[1 0.1543 0.1244] ゲームの状態が初期化されたとき
  (`parent.InitializeCharacterState`)
  (`self.UpdateUseButtonEnabled`))

(event `SimulateBody`
  (bind _mesh (`self.Mesh`))
  ;[0.5587 0.217 1] メッシュを物理シミュレーション
  (`PrimitiveComponent.SetCollisionResponseToAllChannels` _mesh "ECR_Ignore")
  (`PrimitiveComponent.SetCollisionResponseToChannel` _mesh "ECC_WorldStatic" "ECR_Block")
  (`PrimitiveComponent.SetCollisionResponseToChannel` _mesh "ECC_WorldDynamic" "ECR_Block")
  (`PrimitiveComponent.SetCollisionEnabled` _mesh "PhysicsOnly")
  (`PrimitiveComponent.SetSimulatePhysics` _mesh true))

(event `/Game/Werewolf_01/BP/BP_WerewolfInterface.WW_KilledFromWolf`
  ;[1 0.2495 0.2395] 狼によって殺害されたとき
  (`self.KilledByWolf`))

(event `KilledByWolf`
  (bind _pc (`self.GetPC`))
  (bind _capsulecomponent (`self.CapsuleComponent`))
  ;[1 0.2495 0.2395] 狼によって殺害されたとき
  (`|ExecutionSequence`
    (:`then_0`
      (`/Engine/EditorBlueprintResources/StandardMacros.IsValid` _pc
        (:`Is Valid`
          (`/Game/Werewolf_01/BP/Gameplay/BP_GameplayPlayerController.EndCurrentAction` _pc))))
    (:`then_1`
      (`self.SetIsValidDeadBody` true) ; 死体が存在する
      (`self.SetIsDead` true) ; 死亡
      (`self.PlayDeadAnim`)
      (`self.UpdateCapsuleOverlap`)
      (`self.BecomeAGhost`)
      (`self.ClearReportTarget`)
      ;;[1 1 1] 死体用のカプセルを生成
      (bind _returnvalue (`AddComponent|NODE_AddCapsuleComponent-0`)) ; DeadBodyタグを所有
      (bind _output_get (set `self.DeadBodyCapsule` _returnvalue))
      (`SceneComponent.K2_DetachFromComponent` _output_get "KeepWorld" "KeepWorld" "KeepWorld" true)
      (`CapsuleComponent.SetCapsuleSize` _output_get (`CapsuleComponent.CapsuleRadius` _capsulecomponent) (`CapsuleComponent.CapsuleHalfHeight` _capsulecomponent) true))
    (:`then_2`
      (bind _gm (`self.GM`)
        (:`then`
          (message `/Game/Werewolf_01/BP/BP_WerewolfInterface.WW_DecrementAliveVillagersCount` _gm) ; 生存している村人の数を減らす
          (message `/Game/Werewolf_01/BP/BP_WerewolfInterface.WW_GameFinishCheck` _gm) ; ゲームが終了するか確認
        )
        (:`else`)))))

(event `UpdateCapsuleOverlap`
  ;[1 0.1039 0.1238] カプセルの重なりを更新
  (`PrimitiveComponent.SetCollisionEnabled` (`self.CapsuleComponent`) "NoCollision")
  (`PrimitiveComponent.SetCollisionEnabled` (`self.CapsuleComponent`) "QueryOnly"))

(event `ClearDeadBody`
  ;[1 0.1543 0.1244] 死体を削除
  (`|ExecutionSequence`
    (:`then_0`
      (bind _deadbodycapsule (`self.DeadBodyCapsule`)
        (:`then`
          (`ActorComponent.K2_DestroyComponent` _deadbodycapsule))
        (:`else`)))
    (:`then_1`
      (`self.DestroyDeadBodyMesh`)
      (`self.SetIsValidDeadBody` false))))

(event `PlayDeadAnim`
  (bind _mesh (`self.Mesh`))
  ;[0.4557 0.2946 1] 死亡アニメーションを再生
  (`|PlayMontage` (`self.Mesh`) "/Game/Werewolf_01/Animation/Mannequin/AM_DeathFromRight.AM_DeathFromRight"
    (:`then`
      ;;[1 1 1] 死体をデタッチする
      (bind _returnvalue (`AddComponent|NODE_AddSkeletalMeshComponent-0` :`bManualAttachment` true :`RelativeTransform` (`SceneComponent.K2_GetComponentToWorld` (`self.Mesh`)))) ; *Meshをそのまま使用すると、\nプレイヤーが移動したときにメッシュが原点へ移動してしまう
      (bind _output_get (set `self.SKM_DeadBody` _returnvalue))
      (`SkinnedMeshComponent.SetSkinnedAssetAndUpdate` _output_get (`SkinnedMeshComponent.SkeletalMesh` _mesh) true) ; メッシュをコピー
      (for (_array_element _array_index) (`self.Get MI Meshes`)
        (`PrimitiveComponent.SetMaterial` _output_get _array_index _array_element) ; マテリアルをコピー
      )
      (`SkinnedMeshComponent.SetLeaderPoseComponent` (`self.SKM_DeadBody`) (`self.Mesh`) false) ; ポーズをコピー
      (`SceneComponent.SetVisibility` _mesh false false) ; 元のメッシュを非表示
    )))

(event `DestroyDeadBodyMesh`
  ;[0.4557 0.2946 1] 死体のメッシュを削除
  (bind _skm_deadbody (`self.SKM_DeadBody`)
    (:`then`
      (`ActorComponent.K2_DestroyComponent` _skm_deadbody))
    (:`else`)))

(event `self.SetOverlapTask`
  (params (Task :type "/Game/Werewolf_01/BP/Task/BP_Task Object Reference"))
  ;[1 0.1543 0.1244] 重なっているタスクがセットされたとき
  (`parent.SetOverlapTask` Task))

(event `self.ClearOverlapTask`
  ;[1 0.1543 0.1244] 重なっているタスクが削除されたとき
  (`parent.ClearOverlapTask`))

(event `self.SetOverlapEmergencyButton`
  (params (EmergencyButton :type "/Game/Werewolf_01/BP/Gameplay/BP_EmergencyButton Object Reference"))
  ;[1 0.1543 0.1244] 重なっている緊急ボタンがセットされたとき
  (`parent.SetOverlapEmergencyButton` EmergencyButton))

(event `self.ClearOverlapEmergencyButton`
  ;[1 0.1543 0.1244] 重なっている緊急ボタンが削除されたとき
  (`parent.ClearOverlapEmergencyButton`))

(event `self.InitializeGameplayUI`
  ;[1 0.1543 0.1244] ゲームプレイ画面が初期化されたとき
  (`parent.InitializeGameplayUI`))

(event `self.SetIsValidDeadBody`
  (params (Valid :type Boolean))
  ;[1 0.1543 0.1244] 死体が存在するかをセット
  (`parent.SetIsValidDeadBody` Valid)
  (set `self.IsValidDeadBody` Valid))

(event `self.ReceiveTick`
  (params (DeltaSeconds :type "Float (single-precision)"))
  (`parent.ReceiveTick` DeltaSeconds))

(fn `GetDeadBodyCapsuleLocation`
  (returns (Location :type "Vector Structure"))
  (return (`SceneComponent.K2_GetComponentLocation` (`self.DeadBodyCapsule`))))

(fn `GetIsValidDeadBody`
  (returns (Valid :type Boolean))
  (return (`self.IsValidDeadBody`)))

(fn `UserConstructionScript`
  (`parent.UserConstructionScript`))

(fn `WW_GetCharacterType`
  (returns (CharacterType :type "/Game/Werewolf_01/Enum/e_CharacterType Enum"))
  (return "NewEnumerator2"))