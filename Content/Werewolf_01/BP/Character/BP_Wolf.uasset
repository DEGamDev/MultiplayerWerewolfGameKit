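; Werewolf player character in a social-deduction game, able to kill villagers and hide or travel through hatches.
; A server-side overlap sphere picks living villagers as targets, with a sphere trace rejecting obstructed kills.
; Kills move the wolf behind the victim and play a knife montage whose notify applies death and starts a timer-based cooldown.
; Hatch entry and exit toggle visibility and input, while player-controller buttons track kill and hatch availability.
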(event `self.InitializeCharacterState`
  ;[1 1 1] ゲームの状態を初期化
  (`parent.InitializeCharacterState`)
  ;;[1 1 1] ハッチに入れるように
  (set `self.IsInHatch` false)
  (set `self.IsOnTheWayInHatch` false)
  (`KismetSystemLibrary.K2_ClearTimer` null "UpdateKillCooldown") ; 殺害クールダウンの更新を止める
  (`self.ClearKillCoolDown`))

(event `self.ReceiveTick`
  (params (DeltaSeconds :type "Float (single-precision)"))
  ;[1 0.7202 0.07785] Tick
  (`parent.ReceiveTick` DeltaSeconds)
  (`/Engine/EditorBlueprintResources/ActorMacros.Switch Has Authority`
    (:`Authority`
      (if (`self.GetIsKillCoolDown`)
        (message `/Game/Werewolf_01/BP/BP_WerewolfInterface.WW_SetRemainingKillCooldown` (`self.GetController`) (`self.GetKillCooldownRemainingPercent`))))))

(event `SetKillSphereRadius`
  (params (InSphereRadius :type "Float (double-precision)"))
  ;[1 0.2493 0.2792] 殺害スフィアの半径をセット
  (`SphereComponent.SetSphereRadius` (`self.GetKillSphere`) InSphereRadius true))

(event `/Game/Werewolf_01/BP/BP_WerewolfInterface.WW_Kill`
  ;[1 0.2916 0.3015] ターゲットを殺害する
  (`self.Kill`))

(event `Kill`
  (bind _savekilltarget (`self.SaveKillTarget`))
  (bind _returnvalue (`self.K2_GetActorRotation` _savekilltarget))
  ;[1 0.2916 0.3015] ターゲットを殺害する
  (if (`self.CanTryKillToTarget`)
    (bind _can (`self.CanKillTarget`))
    (if _can
      (bind _output_get (set `self.SaveKillTarget` (`self.GetKillTarget`)))
      (if (not (`self.GetIsDead` _output_get))
        (set `self.IsKilling` true)
        ;;[1 1 1] お互いを移動不可にする
        (`self.SetCharacterMovementActive` false)
        (`self.SetCharacterMovementActive` (`self.SaveKillTarget`) false)
        (`self.MoveToKillTarget` (+ (`self.K2_GetActorLocation` _savekilltarget) (* (`KismetMathLibrary.GetForwardVector` _returnvalue) -50.0)) _returnvalue)))))

(event `ClearKillTarget`
  ;[1 0.1543 0.1244] 殺害ターゲットを削除
  (set `self.KillTarget` null)
  (`KismetSystemLibrary.K2_ClearTimer` null "UpdateKillButtonEnable") ; 殺害ボタンの有効性の更新を終了
  (`self.UpdateKillButtonEnable`))

(event `SetKillTarget`
  (params (KillTarget :type "/Game/Werewolf_01/BP/Character/BP_WerewolfCharacter Object Reference"))
  ;[1 0.2188 0.2188] 殺害するターゲットをセット
  (set `self.KillTarget` KillTarget)
  (`self.UpdateKillButtonEnable`)
  (`KismetSystemLibrary.K2_SetTimer` null "UpdateKillButtonEnable" 0.1 true) ; 殺害ボタンの有効性を0.1秒毎に更新
)

(event `self.KillSphere.OnComponentBeginOverlap`
  (params (OverlappedComponent :type "PrimitiveComponent Object Reference") (OtherActor :type "Actor Object Reference") (OtherComp :type "PrimitiveComponent Object Reference") (OtherBodyIndex :type Integer) (bFromSweep :type Boolean) (SweepResult :type "HitResult Structure (by ref)"))
  ;[1 1 1] 殺害スフィアに重なった時
  (`/Engine/EditorBlueprintResources/ActorMacros.Switch Has Authority`
    (:`Authority`
      (if (`self.ActorHasTag` OtherActor "WerewolfCharacter")
        (if (`ActorComponent.ComponentHasTag` OtherComp "Capsule")
          ;;[1 1 1] 村人なら、殺害ターゲットにセット
          (bind _charactertype (message `/Game/Werewolf_01/BP/BP_WerewolfInterface.WW_GetCharacterType` OtherActor))
          (bind _isdead (message `/Game/Werewolf_01/BP/BP_WerewolfInterface.WW_GetIsDead` OtherActor))
          (if (and (`|EnumEquality` _charactertype "NewEnumerator2") (not _isdead))
            (bind _asbp_werewolf_character (cast `/Game/Werewolf_01/BP/Character/BP_WerewolfCharacter` OtherActor))
            (`self.SetKillTarget` _asbp_werewolf_character)))))))

(event `PlayKillSound`
  ;[0.2026 0.2461 1] 殺害したときの音を再生
  (`GameplayStatics.PlaySoundAtLocation` "/Game/Werewolf_01/Sound/ReceiveDamage.ReceiveDamage" (`self.K2_GetActorLocation`) (struct) 1.0 1.0 0.0 null null null null))

(event `PlayKillAnim`
  (bind _savekilltarget (`self.SaveKillTarget`))
  ;[1 1 1] 殺害アニメーションを再生する
  (bind _notifyname (`|PlayMontage` (`self.Mesh`) "/Game/Werewolf_01/Animation/Mannequin/AM_Mannequin_Knife_Kill.AM_Mannequin_Knife_Kill" 2.0)
    (:`then`
      (bind _returnvalue (`AddComponent|NODE_AddStaticMeshComponent-0`))
      (bind _output_get (set `self.SMC_Knife` _returnvalue))
      (`SceneComponent.K2_AttachToComponent` _output_get (`self.Mesh`) "Knife" "SnapToTarget" "SnapToTarget" "KeepRelative" true) ; ナイフを手に持たせる
    )
    (:`OnCompleted`
      (`|ExecutionSequence` :!label _label
        (:`then_0`
          (bind _smc_knife (`self.SMC_Knife`)
            (:`then`
              (`ActorComponent.K2_DestroyComponent` _smc_knife))
            (:`else`)))
        (:`then_1`
          (`/Engine/EditorBlueprintResources/ActorMacros.Switch Has Authority`
            (:`Authority`
              (set `self.SaveKillTarget` null)
              (`self.SetCharacterMovementActive` true)
              (set `self.IsKilling` false))))))
    (:`OnInterrupted`
      (goto _label))
    (:`OnNotifyBegin`
      (`/Engine/EditorBlueprintResources/ActorMacros.Switch Has Authority`
        (:`Authority`
          (switch `name` _notifyname
            (:`Stab`
              (if (not (`self.GetIsDead` _savekilltarget))
                (message `/Game/Werewolf_01/BP/BP_WerewolfInterface.WW_KilledFromWolf` _savekilltarget)
                (`self.PlayKillSound`)
                ;;[1 1 1] 殺害のクールダウンを開始
                (bind _gamesettings (message `/Game/Werewolf_01/BP/BP_WerewolfInterface.WW_GetGameSettings` (`GameplayStatics.GetGameMode`)))
                (bind _time (message `/Game/Werewolf_01/BP/BP_WerewolfInterface.WW_GetKillCoolDownTime` _gamesettings))
                (`self.StartKillCoolDown` (`KismetMathLibrary.Conv_IntToDouble` _time))))))))))

(event `MoveToKillTarget`
  (params (TargetLocation :type "Vector Structure") (TargetRotation :type "Rotator Structure"))
  ;[1 1 1] 殺害のターゲットまで移動する
  (`KismetSystemLibrary.MoveComponentTo` (`self.CapsuleComponent`) TargetLocation TargetRotation false false 0.1 true :!label _label_2) ; 殺害ターゲットの位置へ移動
  (`/Engine/EditorBlueprintResources/ActorMacros.Switch Has Authority`
    (:`Authority`
      (bind _gm (`self.GM`)
        (:`then`
          (if (and (`/Game/Werewolf_01/BP/Gameplay/BP_GameplayGameMode.GetIsInGame` _gm) (not (`self.GetIsDead` (`self.SaveKillTarget`))))
            (`self.PlayKillAnim`)
            (else
              (set `self.IsKilling` false))))
        (:`else`)))))

(event `StopKill`
  ;[1 1 1] 殺害のターゲットまで移動する
  (goto _label_2 :!via `Stop`))

(event `self.KillSphere.OnComponentEndOverlap`
  (params (OverlappedComponent :type "PrimitiveComponent Object Reference") (OtherActor :type "Actor Object Reference") (OtherComp :type "PrimitiveComponent Object Reference") (OtherBodyIndex :type Integer))
  ;[1 1 1] 殺害スフィアに重なった時
  (`/Engine/EditorBlueprintResources/ActorMacros.Switch Has Authority`
    (:`Authority`
      (if (`self.ActorHasTag` OtherActor "WerewolfCharacter")
        (if (`ActorComponent.ComponentHasTag` OtherComp "Capsule")
          ;;[1 1 1] 村人かつ殺害ターゲットと同じとき、殺害ターゲットを削除
          (bind _charactertype (message `/Game/Werewolf_01/BP/BP_WerewolfInterface.WW_GetCharacterType` OtherActor))
          (bind _isdead (message `/Game/Werewolf_01/BP/BP_WerewolfInterface.WW_GetIsDead` OtherActor))
          (if (and (not _isdead) (`|EnumEquality` _charactertype "NewEnumerator2"))
            (if (== OtherActor (`self.GetKillTarget`))
              (`self.ClearKillTarget`))))))))

(event `StartKillCoolDown`
  (params (Time :type "Float (double-precision)"))
  (bind _pc (`self.GetPC`))
  ;[1 0.2384 0.2185] 殺害のクールダウンを開始する
  (set `self.KillCooldownTime` Time)
  (`self.SetIsKillCoolDown` true)
  (`KismetSystemLibrary.K2_SetTimer` null "EndKillCoolDown" Time)
  (`self.UpdateKillCooldown`)
  (`KismetSystemLibrary.K2_SetTimer` null "UpdateKillCooldown" 1.0 true) ; 殺害のクールダウンを更新する
  (`/Engine/EditorBlueprintResources/StandardMacros.IsValid` _pc
    (:`Is Valid`
      (`/Game/Werewolf_01/BP/Gameplay/BP_GameplayPlayerController.SetKillCooldownVisible` _pc true))))

(event `EndKillCoolDown`
  (bind _pc (`self.GetPC`))
  ;[1 0.2643 0.1946] 殺害のクールダウンを終了する
  (`self.SetIsKillCoolDown` false)
  (`KismetSystemLibrary.K2_ClearTimer` null "UpdateKillCooldown") ; 殺害クールダウンの更新を止める
  (`self.UpdateKillTarget`)
  (`/Engine/EditorBlueprintResources/StandardMacros.IsValid` _pc
    (:`Is Valid`
      (`/Game/Werewolf_01/BP/Gameplay/BP_GameplayPlayerController.SetKillCooldownVisible` _pc false))))

(event `UpdateKillCooldown`
  (bind _pc (`self.GetPC`))
  ;[1 0.1543 0.1244] 殺害のクールダウンを更新する
  (`/Engine/EditorBlueprintResources/StandardMacros.IsValid` _pc
    (:`Is Valid`
      (`/Game/Werewolf_01/BP/Gameplay/BP_GameplayPlayerController.SetKillButtonCooldown` _pc (`KismetMathLibrary.FCeil` (`KismetSystemLibrary.K2_GetTimerRemainingTime` null "EndKillCoolDown"))))))

(event `/Game/Werewolf_01/BP/BP_WerewolfInterface.WW_ClearKillCoolDown`
  ;[1 0.1768 0.1967] 殺害のクールダウンを削除する
  (`self.ClearKillCoolDown`))

(event `ClearKillCoolDown`
  (bind _pc (`self.GetPC`))
  ;[1 0.1768 0.1967] 殺害のクールダウンを削除する
  (`self.SetIsKillCoolDown` false)
  (`KismetSystemLibrary.K2_ClearTimer` null "EndKillCoolDown")
  (`self.UpdateKillTarget`)
  (`/Engine/EditorBlueprintResources/StandardMacros.IsValid` _pc
    (:`Is Valid`
      (`/Game/Werewolf_01/BP/Gameplay/BP_GameplayPlayerController.SetKillCooldownVisible` _pc false))))

(event `self.CapsuleBeginOverlap`
  (params (OtherActor :type "Actor Object Reference"))
  ;[1 1 1] カプセルが重なり始めたとき
  (`parent.CapsuleBeginOverlap` OtherActor)
  (`/Engine/EditorBlueprintResources/ActorMacros.Switch Has Authority`
    (:`Authority`
      (bind _ishatch (message `/Game/Werewolf_01/BP/BP_WerewolfInterface.WW_IsHatch` OtherActor))
      (if _ishatch
        (bind _asbp_hatch (cast `/Game/Werewolf_01/BP/Hatch/BP_Hatch` OtherActor))
        (`self.SetOverlapHatch` _asbp_hatch)))))

(event `SetIsKillCoolDown`
  (params (IsKillCoolDown :type Boolean))
  ;[1 0.177 0.187] 殺害のクールダウンかをセットする
  (set `self.IsKillCoolDown` IsKillCoolDown))

(event `/Game/Werewolf_01/BP/BP_WerewolfInterface.WW_UpdateKillButtonEnabled`
  ;[1 0.1543 0.1244] 殺害ボタンの有効性を更新
  (`self.UpdateKillButtonEnable`))

(event `UpdateKillButtonEnable`
  (bind _pc (`self.GetPC`))
  (bind _pc_2 (`self.GetPC`))
  ;[1 0.1543 0.1244] 殺害ボタンの有効性を更新
  (if (`self.CanTryKillToTarget`)
    (bind _can (`self.CanKillTarget`))
    (`/Engine/EditorBlueprintResources/StandardMacros.IsValid` _pc
      (:`Is Valid`
        (`/Game/Werewolf_01/BP/Gameplay/BP_GameplayPlayerController.SetKillButtonEnable` _pc _can)))
    (else
      (`/Engine/EditorBlueprintResources/StandardMacros.IsValid` _pc_2
        (:`Is Valid`
          (`/Game/Werewolf_01/BP/Gameplay/BP_GameplayPlayerController.SetKillButtonEnable` _pc_2 false))))))

(event `UpdateKillTarget`
  ;[1 1 1] 殺害ターゲットを更新
  (bind _target (`self.FindNewKillTarget`))
  (`self.SetKillTarget` _target))

(event `self.CapsuleEndOverlap`
  (params (OtherActor :type "Actor Object Reference"))
  ;[1 1 1] カプセルが重なり終えたとき
  (`parent.CapsuleEndOverlap` OtherActor)
  (`/Engine/EditorBlueprintResources/ActorMacros.Switch Has Authority`
    (:`Authority`
      (bind _ishatch (message `/Game/Werewolf_01/BP/BP_WerewolfInterface.WW_IsHatch` OtherActor))
      (if _ishatch
        (if (== OtherActor (`self.GetOverlapHatch`))
          (`self.ClearOverlapHatch`) ; 重なっているハッチを削除
        )))))

(event `SetOverlapHatch`
  (params (OverlapHatch :type "/Game/Werewolf_01/BP/Hatch/BP_Hatch Object Reference"))
  (set `self.OverlapHatch` OverlapHatch)
  (`self.UpdateHatchButtonEnabled`))

(event `ClearOverlapHatch`
  (set `self.OverlapHatch` null)
  (`self.UpdateUseButtonEnabled`))

(event `UpdateHatchButtonEnabled`
  (bind _pc (`self.GetPC`))
  (`/Engine/EditorBlueprintResources/StandardMacros.IsValid` _pc
    (:`Is Valid`
      (`/Game/Werewolf_01/BP/Gameplay/BP_GameplayPlayerController.SetHatchButtonEnabled` _pc (or (`self.CanEnterToHatch`) (`self.CanLeaveFromHatch`))))))

(event `MoveToHatch`
  (params (Hatch :type "Actor Object Reference"))
  (`/Engine/EditorBlueprintResources/StandardMacros.IsValid` Hatch
    (:`Is Valid`
      (`self.K2_SetActorLocation` (`self.GetOnHatchLocation` (`self.K2_GetActorLocation` Hatch)))
      (message `/Game/Werewolf_01/BP/BP_WerewolfInterface.WW_UpdateHatchButtons` (`self.GetController`)))))

(event `EnterToHatch`
  (if (`self.CanEnterToHatch`)
    (`self.SetCharacterMovementActive` false)
    (`self.InterpToHatch` (`self.GetOverlapHatch`))))

(event `LeaveFromHatch`
  (bind _pc (`self.GetPC`))
  (bind _pc_2 (`self.GetPC`))
  (bind _hatch (`self.GetOverlapHatch`))
  (if (`self.CanLeaveFromHatch`)
    (`/Engine/EditorBlueprintResources/StandardMacros.IsValid` (`self.GetPC`)
      (:`Is Valid`
        (`|ExecutionSequence`
          (:`then_0`
            (`|ExecutionSequence`
              (:`then_0`
                (set `self.IsOnTheWayInHatch` true)
                (`self.SetIsInHatch` false)
                (message `/Game/Werewolf_01/BP/BP_WerewolfInterface.WW_OpenHatch` _hatch (`self.GetPC`))
                (message `/Game/Werewolf_01/BP/BP_WerewolfInterface.WW_RemoveInHatchScreen` (`self.GetController`))
                (`self.UpdateHatchButtonEnabled`)
                (`self.PlayLeaveFromHatchAnim`)
                (`self.OnEnterFloor` self)
                (if (not (`/Game/Werewolf_01/BP/Gameplay/BP_GameplayPlayerController.IsOpenSabotageScreen` _pc))
                  (`/Game/Werewolf_01/BP/Gameplay/BP_GameplayPlayerController.DisableUIInput` _pc) ; 妨害画面を開いていないとき、画面入力を無効にする
                ))
              (:`then_1`
                (bind _gm (`self.GM`)
                  (:`then`
                    (`/Game/Werewolf_01/BP/Gameplay/BP_GameplayGameMode.SetCharacterVisibleToAllPlayers` _gm self true) ; キャラクターを表示
                  )
                  (:`else`)))))
          (:`then_1`
            (`KismetSystemLibrary.Delay` 1.5)
            (`/Engine/EditorBlueprintResources/StandardMacros.IsValid` (`self.GetOverlapHatch`)
              (:`Is Valid`
                (`/Engine/EditorBlueprintResources/StandardMacros.IsValid` _pc_2
                  (:`Is Valid`
                    (`|ExecutionSequence`
                      (:`then_0`
                        (set `self.IsOnTheWayInHatch` false)
                        (message `/Game/Werewolf_01/BP/BP_WerewolfInterface.WW_CloseHatch` _hatch _pc_2)
                        (`/Game/Werewolf_01/BP/Gameplay/BP_GameplayPlayerController.EnableGameInput` _pc_2)
                        (`/Game/Werewolf_01/BP/Gameplay/BP_GameplayPlayerController.SetIsEnableCameraInput` _pc_2 true)
                        (`self.SetCharacterMovementActive` true) ; 移動可能にする
                        (`self.UpdateHatchButtonEnabled`) ; ハッチボタンの有効性を更新
                        (`self.UpdateReportButtonEnable`) ; 通報ボタンの有効性を更新
                      ))))))))))))

(event `SetIsInHatch`
  (params (IsIn :type Boolean))
  (set `self.IsInHatch` IsIn))

(event `/Game/Werewolf_01/BP/BP_WerewolfInterface.WW_EnterToHatch`
  (`self.EnterToHatch`))

(event `/Game/Werewolf_01/BP/BP_WerewolfInterface.WW_LeaveFromHatch`
  (`self.LeaveFromHatch`))

(event `/Game/Werewolf_01/BP/BP_WerewolfInterface.WW_MoveToHatch`
  (params (Hatch :type "Actor Object Reference"))
  (`self.MoveToHatch` Hatch))

(event `/Game/Werewolf_01/BP/BP_WerewolfInterface.WW_UpdateHatchButtonEnabled`
  (`self.UpdateHatchButtonEnabled`))

(event `PlayEnterToHatchAnim`
  (`self.PlayAnimMontage` "/Game/Werewolf_01/Animation/Mannequin/AM_EnterToHatch.AM_EnterToHatch" 2.0))

(event `PlayLeaveFromHatchAnim`
  (`self.PlayAnimMontage` "/Game/Werewolf_01/Animation/Mannequin/AM_LeaveFromHatch.AM_LeaveFromHatch" 2.0))

(event `InterpToHatch`
  (params (Hatch :type "/Game/Werewolf_01/BP/Hatch/BP_Hatch Object Reference"))
  (bind _hatch (`self.GetOverlapHatch`))
  (bind _pc (`self.GetPC`))
  (bind _returnvalue (`self.GetController`))
  (bind _pc_2 (`self.GetPC`))
  (`/Engine/EditorBlueprintResources/StandardMacros.IsValid` Hatch
    (:`Is Valid`
      (`KismetSystemLibrary.MoveComponentTo` (`self.CapsuleComponent`) (`self.GetOnHatchLocation` (`self.K2_GetActorLocation` Hatch)) (`KismetMathLibrary.ComposeRotators` (`self.K2_GetActorRotation` Hatch) (struct :`Yaw` -90.0)) true true 0.2 true :!label _label_3) ; ハッチの位置へ移動
      (`/Engine/EditorBlueprintResources/ActorMacros.Switch Has Authority`
        (:`Authority`
          (bind _gm (`self.GM`)
            (:`then`
              (if (`/Game/Werewolf_01/BP/Gameplay/BP_GameplayGameMode.GetIsInGame` _gm)
                (`/Engine/EditorBlueprintResources/StandardMacros.IsValid` (`self.GetPC`)
                  (:`Is Valid`
                    (`|ExecutionSequence`
                      (:`then_0`
                        (set `self.IsOnTheWayInHatch` true)
                        (message `/Game/Werewolf_01/BP/BP_WerewolfInterface.WW_OpenHatch` _hatch _pc)
                        (`self.SetIsInHatch` true)
                        (`/Game/Werewolf_01/BP/Gameplay/BP_GameplayPlayerController.DisableGameInput` _pc)
                        (`self.UpdateHatchButtonEnabled`) ; ハッチボタンの有効性を更新
                        (`self.UpdateReportButtonEnable`) ; 通報ボタンの有効性を更新
                        (`self.PlayEnterToHatchAnim`)
                        (`self.OnLeaveFloor` self (`/Game/Werewolf_01/BP/Gameplay/BP_GameplayPlayerController.GetInFloor` _pc)))
                      (:`then_1`
                        (`KismetSystemLibrary.Delay` 1.5)
                        (set `self.IsOnTheWayInHatch` false)
                        (`/Engine/EditorBlueprintResources/StandardMacros.IsValid` (`self.GetOverlapHatch`)
                          (:`Is Valid`
                            (`/Engine/EditorBlueprintResources/StandardMacros.IsValid` _pc_2
                              (:`Is Valid`
                                (message `/Game/Werewolf_01/BP/BP_WerewolfInterface.WW_CloseHatch` _hatch _pc_2)
                                (`self.UpdateHatchButtonEnabled`)
                                (message `/Game/Werewolf_01/BP/BP_WerewolfInterface.WW_UpdateHatchButtons` _returnvalue)
                                (message `/Game/Werewolf_01/BP/BP_WerewolfInterface.WW_SetIsEnableCameraInput` _returnvalue false)
                                (message `/Game/Werewolf_01/BP/BP_WerewolfInterface.WW_EnableUIInput` _returnvalue)
                                (bind _gm_2 (`self.GM`)
                                  (:`then`
                                    (`/Game/Werewolf_01/BP/Gameplay/BP_GameplayGameMode.SetCharacterVisibleToAllPlayers` _gm_2 self false) ; キャラクターを非表示
                                  )
                                  (:`else`))))))))))))
            (:`else`)))))))

(event `StopInterpToHatch`
  (`/Engine/EditorBlueprintResources/StandardMacros.IsValid` (stale `InterpToHatch` Hatch)
    (:`Is Valid`
      (goto _label_3 :!via `Stop`))))

(event `self.ReceiveBeginPlay`
  (`parent.ReceiveBeginPlay`))

(event `self.BecomeAGhost`
  ;[1 1 1] 幽霊になったとき
  (`parent.BecomeAGhost`)
  (`self.UpdateKillButtonEnable`) ; 追放後に殺害ボタンが光ったままになるのを防ぐ
)

(event `/Game/Werewolf_01/BP/BP_WerewolfInterface.WW_EndCurrentAction`
  ;[1 1 1] 現在のアクションを終了する
  (`self.StopAnim`)
  (`self.StopKill`)
  (`self.StopInterpToHatch`))

(event `StopAnim`
  ;[0.4557 0.2946 1] アニメーションを停止
  (`self.StopAnimMontage` (`self.GetCurrentMontage`)))

(fn `CanEnterToHatch`
  (returns (Can :type Boolean))
  (bind _pc (`self.GetPC`))
  (`/Engine/EditorBlueprintResources/StandardMacros.IsValid` _pc
    (:`Is Valid`
      (return (and (not (`self.GetIsInHatch`)) (not (`self.IsOnTheWayInHatch`)) (`KismetSystemLibrary.IsValid` (`self.GetOverlapHatch`)) (`/Game/Werewolf_01/BP/Gameplay/BP_GameplayPlayerController.IsAlive` _pc) (not (`self.GetIsKilling`)))))
    (:`Is Not Valid`
      (return false))))

(fn `CanKillTarget`
  (returns (Can :type Boolean))
  (bind _killtarget (`self.GetKillTarget`))
  (`/Engine/EditorBlueprintResources/StandardMacros.IsValid` _killtarget
    (:`Is Valid`
      (bind (_outhits _returnvalue) (`KismetSystemLibrary.SphereTraceMulti` (`self.K2_GetActorLocation`) (`self.K2_GetActorLocation` _killtarget) (/ (`CapsuleComponent.CapsuleRadius` (`self.CapsuleComponent`)) 2.0) "TraceTypeQuery1"))
      (if _returnvalue
        (for _array_element _outhits
          (bind (_bblockinghit _binitialoverlap _time _distance _location _impactpoint _normal _impactnormal _physmat _hitactor) (`GameplayStatics.BreakHitResult` _array_element))
          (`/Engine/EditorBlueprintResources/StandardMacros.IsValid` _hitactor
            (:`Is Valid`
              (if (not (`self.ActorHasTag` _hitactor "WerewolfCharacter"))
                (`|ExecutionSequence` :!label _label
                  (:`then_0`
                    (break))
                  (:`then_1`
                    (return false) ; キャラクター以外の障害物にヒットしたとき、殺害不可
                  ))))
            (:`Is Not Valid`
              (goto _label))))
        (return true) ; キャラクター以外の障害物にヒットしなかったとき、殺害可
      ))
    (:`Is Not Valid`
      (return false))))

(fn `CanLeaveFromHatch`
  (returns (Can :type Boolean))
  (return (and (`self.GetIsInHatch`) (not (`self.IsOnTheWayInHatch`)) (`KismetSystemLibrary.IsValid` (`self.GetOverlapHatch`)))))

(fn `CanTryKillToTarget`
  (returns (Can :type Boolean))
  (bind _pc (`self.GetPC`))
  (`/Engine/EditorBlueprintResources/StandardMacros.IsValid` _pc
    (:`Is Valid`
      (return (and (not (`self.GetIsKillCoolDown`)) (not (`self.GetIsInHatch`)) (`KismetSystemLibrary.IsValid` (`self.GetKillTarget`)) (`/Game/Werewolf_01/BP/Gameplay/BP_GameplayPlayerController.IsAlive` _pc) (not (`/Game/Werewolf_01/BP/Gameplay/BP_GameplayPlayerController.GetIsOpenTask` _pc)) (not (`/Game/Werewolf_01/BP/Gameplay/BP_GameplayPlayerController.IsOpenSabotageScreen` _pc)) (not (`self.GetIsKilling`)) (not (`/Game/Werewolf_01/BP/Gameplay/BP_GameplayPlayerController.Get Is Open Mini Map` _pc)))))
    (:`Is Not Valid`
      (return false))))

(fn `CanTryReportTarget`
  (returns (Can :type Boolean))
  (return (and (`parent.CanTryReportTarget`) (not (`self.IsInHatch`)))))

(fn `EnableRandomEmergencyTask`
  (locals (Tasks_l :type "Array of Actor Object Reference"))
  (bind _returnvalue (`GameplayStatics.GetGameMode`))
  ;[0 0 0] ランダムな緊急タスクを有効にする
  (bind _gamesettings (message `/Game/Werewolf_01/BP/BP_WerewolfInterface.WW_GetGameSettings` _returnvalue))
  (bind _tasks (message `/Game/Werewolf_01/BP/BP_WerewolfInterface.WW_GetEmergencyTasks` _returnvalue))
  (bind _output_get (set `local.Tasks_l` _tasks))
  (`KismetArrayLibrary.Array_Shuffle` _output_get)
  (for _array_element (`local.Tasks_l`)
    (bind _isenable (message `/Game/Werewolf_01/BP/BP_WerewolfInterface.WW_GetIsEnableTask` _array_element))
    (if (not _isenable)
      (message `/Game/Werewolf_01/BP/BP_WerewolfInterface.WW_TaskEnable` _array_element)
      (message `/Game/Werewolf_01/BP/BP_WerewolfInterface.WW_StartSabotageCooldown` _gamesettings))))

(fn `FindNewKillTarget`
  (returns (Target :type "/Game/Werewolf_01/BP/Character/BP_Villager Object Reference"))
  (for _array_element (`PrimitiveComponent.GetOverlappingActors` (`self.KillSphere`) "/Game/Werewolf_01/BP/Character/BP_Villager.BP_Villager_C")
    (bind _asbp_villager (cast `/Game/Werewolf_01/BP/Character/BP_Villager` _array_element))
    (bind _returnvalue (`self.GetComponentsByTag` _asbp_villager "/Script/Engine.CapsuleComponent" "Capsule"))
    (if (`KismetArrayLibrary.Array_IsValidIndex` _returnvalue)
      (if (`PrimitiveComponent.IsOverlappingComponent` (`self.KillSphere`) (`|GetArrayItem` _returnvalue))
        (bind _pc (`self.GetPC` _asbp_villager))
        (`/Engine/EditorBlueprintResources/StandardMacros.IsValid` _pc
          (:`Is Valid`
            (if (`/Game/Werewolf_01/BP/Gameplay/BP_GameplayPlayerController.IsAlive` _pc)
              (return _asbp_villager)))))))
  (return null))

(fn `GetIsEmergencyTaskCoolDown`
  (returns (IsCoolDown :type Boolean))
  (bind _iscooldown (message `/Game/Werewolf_01/BP/BP_WerewolfInterface.WW_GetIsEmergencyTaskCoolDown` (`GameplayStatics.GetGameMode`)))
  (return _iscooldown))

(fn `GetIsInHatch`
  (returns (IsIn :type Boolean))
  (return (`self.IsInHatch`)))

(fn `GetIsKillCoolDown`
  (returns (CoolDown :type Boolean))
  (return (`self.IsKillCoolDown`)))

(fn `GetIsKilling`
  (returns (Killing :type Boolean))
  (return (`self.IsKilling`)))

(fn `GetKillCooldownRemainingPercent`
  (returns (Time :type "Float (double-precision)"))
  (return (/ (`KismetSystemLibrary.K2_GetTimerRemainingTime` null "EndKillCoolDown") (`self.KillCooldownTime`))))

(fn `GetKillRange`
  (returns (KillRange :type "Float (double-precision)"))
  (return (`self.KillRange`)))

(fn `GetKillSphere`
  (returns (KillSphere :type "SphereComponent Object Reference"))
  (return (`self.KillSphere`)))

(fn `GetKillTarget`
  (returns (KillTarget :type "/Game/Werewolf_01/BP/Character/BP_WerewolfCharacter Object Reference"))
  (return (`self.KillTarget`)))

(fn `GetOnHatchLocation`
  (params (Location :type "Vector Structure"))
  (returns (ReturnValue :type "Vector Structure"))
  (return (+ Location (`KismetMathLibrary.MakeVector` 0.0 0.0 (`CapsuleComponent.CapsuleHalfHeight` (`self.CapsuleComponent`))))))

(fn `GetOverlapHatch`
  (returns (Hatch :type "/Game/Werewolf_01/BP/Hatch/BP_Hatch Object Reference"))
  (return (`self.OverlapHatch`)))

(fn `UserConstructionScript`
  (`parent.UserConstructionScript`)
  (`self.SetKillSphereRadius` (`self.GetKillRange`)))

(fn `WW_GetCharacterType`
  (returns (CharacterType :type "/Game/Werewolf_01/Enum/e_CharacterType Enum"))
  (return "NewEnumerator1"))

(fn `WW_GetIsInHatch`
  (returns (IsIn :type Boolean))
  (return (`self.GetIsInHatch`)))

(fn `WW_GetIsKilling`
  (returns (Killing :type Boolean))
  (return (`self.GetIsKilling`)))

(fn `WW_GetOverlapHatch`
  (returns (Hatch :type "/Game/Werewolf_01/BP/Hatch/BP_Hatch Object Reference"))
  (return (`self.GetOverlapHatch`)))