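; Player controller for the werewolf game's result screen, handling result display and game restart.
; On the server it waits briefly after BeginPlay, then asks BP_ResultGamemode to show the result for itself.
; Its events forward winner info and camera to BP_ResultGameState, restarts to the game mode and screen removal to the HUD, and create the loading widget.
; It stores a character type, while the WW_ getter functions are stubs returning defaults.
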(event `self.ReceiveBeginPlay`
  (`/Engine/EditorBlueprintResources/ActorMacros.Switch Has Authority`
    (:`Authority`
      (`KismetSystemLibrary.Delay` 0.5)
      (bind _asbp_result_gamemode (cast `/Game/Werewolf_01/BP/Result/BP_ResultGamemode` (`GameplayStatics.GetGameMode`)))
      (bind _output_get (set `self.GM` _asbp_result_gamemode))
      (`/Game/Werewolf_01/BP/Result/BP_ResultGamemode.ShowResult` _output_get self))))

(event `ShowResultToPlayer`
  (params (WinnerrInfo :type "Array of /Game/Werewolf_01/BP/Result/s_WinnerInfo Structure (by ref)") (Win :type Boolean) (Camera :type "Actor Object Reference"))
  ;[1 1 1] プレイヤーへゲームの結果を表示
  (bind _asbp_result_game_state (cast `/Game/Werewolf_01/BP/Result/BP_ResultGameState` (`GameplayStatics.GetGameState`))
    (:`then`
      (`/Game/Werewolf_01/BP/Result/BP_ResultGameState.ShowResult` _asbp_result_game_state WinnerrInfo Win Camera))
    (:`CastFailed`
      (`KismetSystemLibrary.PrintString` "ShowResultToPlayer Failed" true true (struct :`R` 1.0 :`A` 1.0)))))

(event `/Game/Werewolf_01/BP/BP_WerewolfInterface.WW_SetCharacterType`
  (params (CharacterType :type "/Game/Werewolf_01/Enum/e_CharacterType Enum" :default "NewEnumerator1"))
  ;[1 1 1] キャラクタータイプをセット
  (set `self.Character Type` CharacterType))

(event `RestartGame`
  ;[1 1 1] 新しくゲームを再開する
  (bind _gm (`self.GM`)
    (:`then`
      (`/Game/Werewolf_01/BP/Result/BP_ResultGamemode.RestartGame` _gm))
    (:`else`)))

(event `RemoveResult`
  ;[1 1 1] 結果画面を削除
  (bind _asbp_result_hud (cast `/Game/Werewolf_01/BP/Result/BP_ResultHUD` (`self.GetHUD`)))
  (`/Game/Werewolf_01/BP/Result/BP_ResultHUD.RemoveResultScreen` _asbp_result_hud))

(event `DisplayRoadingScreen`
  ;[1 1 1] 読み込み画面を表示
  (`self.UI_LoadingScreen`
    (:`then`)
    (:`else`
      (bind _returnvalue (`|CreateWidget` "/Game/Werewolf_01/UI/Character/UI_LoadingScreen.UI_LoadingScreen_C"))
      (bind _output_get (set `self.UI_LoadingScreen` _returnvalue))
      (`UserWidget.AddToViewport` _output_get 0))))

(fn `UserConstructionScript`)

(fn `WW_GetAllCharacters`
  (returns (Characters :type "Array of Actor Object Reference"))
  (return))

(fn `WW_GetAllPC`
  (returns (PC :type "Array of Actor Object Reference"))
  (return))

(fn `WW_GetAllPlayersCount`
  (returns (Count :type Integer))
  (return 0))

(fn `WW_GetAllWolfs`
  (returns (Wolfs :type "Array of Actor Object Reference"))
  (return))

(fn `WW_GetCanMovingHatches`
  (returns (Hatches :type "Array of Actor Object Reference"))
  (return))

(fn `WW_GetCanUseEmergencyButton`
  (params (UsedCount :type Integer))
  (returns (Can :type Boolean))
  (return false))

(fn `WW_GetCharacterType`
  (returns (CharacterType :type "/Game/Werewolf_01/Enum/e_CharacterType Enum"))
  (return "NewEnumerator1"))

(fn `WW_GetCompletedTaskCount`
  (returns (Count :type Integer))
  (return 0))

(fn `WW_GetEmergencyButton`
  (returns (EmergencyButton :type "Actor Object Reference"))
  (return null))

(fn `WW_GetEmergencyMeetingCoolTime`
  (returns (Time :type Integer))
  (return 0))

(fn `WW_GetEmergencyTasks`
  (returns (Tasks :type "Array of Actor Object Reference"))
  (return))

(fn `WW_GetGameSettings`
  (returns (GameSettings :type "Actor Object Reference"))
  (return null))

(fn `WW_GetIsCharacterCapsule`
  (params (Comp :type "SceneComponent Object Reference"))
  (returns (NewParam :type Boolean))
  (return false))

(fn `WW_GetIsDead`
  (returns (IsDead :type Boolean))
  (return false))

(fn `WW_GetIsEmergencyTaskCoolDown`
  (returns (IsCoolDown :type Boolean))
  (return false))

(fn `WW_GetIsEnableTask`
  (returns (IsEnable :type Boolean))
  (return false))

(fn `WW_GetIsGameFinished`
  (returns (IsGameFinished :type Boolean))
  (return false))

(fn `WW_GetIsInGame`
  (returns (IsInGame :type Boolean))
  (return false))

(fn `WW_GetIsInHatch`
  (returns (IsIn :type Boolean))
  (return false))

(fn `WW_GetIsInMeeting`
  (returns (In :type Boolean))
  (return false))

(fn `WW_GetIsInVotingTime`
  (returns (In :type Boolean))
  (return false))

(fn `WW_GetIsKillCoolDown`
  (returns (CoolDown :type Boolean))
  (return false))

(fn `WW_GetIsKilling`
  (returns (Killing :type Boolean))
  (return false))

(fn `WW_GetIsPlayerStart`
  (returns (NewParam :type Boolean))
  (return false))

(fn `WW_GetIsPutHand`
  (returns (IsPut :type Boolean))
  (return false))

(fn `WW_GetIsSabotageCoolDown`
  (returns (IsCoolDown :type Boolean))
  (return false))

(fn `WW_GetIsTaskManager`
  (returns (NewParam :type Boolean))
  (return false))

(fn `WW_GetIsUseCamera`
  (returns (Use :type Boolean))
  (return false))

(fn `WW_GetIsValidEmergencyTimer`
  (returns (IsValid :type Boolean))
  (return false))

(fn `WW_GetIsVotedToPlayer`
  (returns (NewParam :type Boolean))
  (return false))

(fn `WW_GetKillCoolDownTime`
  (returns (Time :type Integer))
  (return 0))

(fn `WW_GetMovingSpeed`
  (returns (Speed :type "Float (double-precision)"))
  (return 0.0))

(fn `WW_GetOverlapHatch`
  (returns (Hatch :type "/Game/Werewolf_01/BP/Hatch/BP_Hatch Object Reference"))
  (return null))

(fn `WW_GetPCByIndex`
  (params (Index :type Integer))
  (returns (PC :type "Actor Object Reference"))
  (return null))

(fn `WW_GetPlayerColorByIndex`
  (params (Index :type Integer))
  (returns (Color :type "LinearColor Structure"))
  (return))

(fn `WW_GetPlayerIndex`
  (returns (Index :type Integer))
  (return 0))

(fn `WW_GetPlayerName`
  (returns (Name :type String))
  (return ""))

(fn `WW_GetPlayerStarts`
  (returns (PlayerStarts :type "Array of Actor Object Reference"))
  (return))

(fn `WW_GetReportTarget`
  (returns (ReportTarget :type "Actor Object Reference"))
  (return null))

(fn `WW_GetSabotageCooldownPercent`
  (returns (Percent :type "Float (double-precision)"))
  (return 0.0))

(fn `WW_GetTask`
  (returns (Task :type "Actor Object Reference"))
  (return null))

(fn `WW_GetTaskManagers`
  (returns (TaskManagers :type "Array of Actor Object Reference"))
  (return))

(fn `WW_GetTaskUIClass`
  (returns (TaskUIClass :type "UserWidget Class Reference"))
  (return null))

(fn `WW_GetVotedFromPlayerCount`
  (returns (Count :type Integer))
  (return 0))

(fn `WW_GetVotedFromPlayerIndex`
  (returns (Index :type "Array of Integer"))
  (return))

(fn `WW_GetVoteTime`
  (returns (Time :type Integer))
  (return 0))

(fn `WW_IsCompleted`
  (returns (Completed :type Boolean))
  (return false))

(fn `WW_IsCompletedAllTask`
  (returns (IsCompleted :type Boolean))
  (return false))

(fn `WW_IsControlledCharacter`
  (returns (ReturnValue :type Boolean))
  (return false))

(fn `WW_IsEmergencyButton`
  (returns (NewParam :type Boolean))
  (return false))

(fn `WW_IsEmergencyTask`
  (returns (NewParam :type Boolean))
  (return false))

(fn `WW_IsGameSettings`
  (returns (ReturnValue :type Boolean))
  (return false))

(fn `WW_IsHatch`
  (returns (IsHatch :type Boolean))
  (return false))

(fn `WW_IsReportSphere`
  (params (Comp :type "PrimitiveComponent Object Reference"))
  (returns (NewParam :type Boolean))
  (return false))

(fn `WW_IsTask`
  (returns (NewParam :type Boolean))
  (return false))

(fn `WW_IsValidDeadBody`
  (returns (Valid :type Boolean))
  (return false))

(fn `WW_IsVillager`
  (returns (IsVillager :type Boolean))
  (return false))

(fn `WW_IsWolf`
  (returns (Wolf :type Boolean))
  (return false))

(fn `WW_SpawnPlayers`
  (returns (Vilagers :type "Array of /Game/Werewolf_01/BP/Character/BP_Villager Object Reference") (Wolfs :type "Array of /Game/Werewolf_01/BP/Character/BP_Wolf Object Reference"))
  (return))