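; BP_ResultHUD is a HUD Blueprint that shows and removes the end-of-game result screen.
; DisplayResultScreen creates a UI_EndGame widget with the win/lose flag, stores it, adds it to the viewport, shows the mouse cursor and switches input to Game and UI with focus on the widget.
; RemoveResultScreen takes the stored widget off screen, or prints a failure message if it is invalid, without restoring cursor or input mode.
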(event `DisplayResultScreen`
  (params (isWin :type Boolean))
  (bind _returnvalue (`self.GetOwningPlayerController`))
  ;[1 1 1] ゲームの結果を表示
  (bind _returnvalue_2 (`|CreateWidget` "/Game/Werewolf_01/UI/Result/UI_EndGame.UI_EndGame_C" (`self.PlayerOwner`) isWin))
  (set `self.UI_Result` _returnvalue_2)
  (`UserWidget.AddToViewport` _returnvalue_2 0)
  (set `PlayerController.bShowMouseCursor` true _returnvalue)
  (`WidgetBlueprintLibrary.SetInputMode_GameAndUIEx` _returnvalue _returnvalue_2 "LockOnCapture" false))

(event `RemoveResultScreen`
  ;[1 1 1] 結果画面を削除
  (bind _ui_result (`self.UI_Result`)
    (:`then`
      (`Widget.RemoveFromParent` _ui_result))
    (:`else`
      (`KismetSystemLibrary.PrintString` "RemoveResultScreen Failed" true true (struct :`R` 1.0 :`A` 1.0)))))

(fn `UserConstructionScript`)