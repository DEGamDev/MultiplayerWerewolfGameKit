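; Base task actor for the werewolf game, covering normal, emergency, blackout and sabotage tasks, either shared or per-player.
; Opening and closing toggle the player's task UI, input, movement and optional spring-arm camera with characters hidden.
; Enable and completion events drive GameMode timers, lights, comms, task assignment and counts, deferring some steps when a manager is used.
; WW interface functions expose task state; empty initialization and per-player events serve as hooks.
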(event `self.ReceiveBeginPlay`
  (`parent.ReceiveBeginPlay`)
  (`|ExecutionSequence`
    (:`then_0`
      (`/Engine/EditorBlueprintResources/ActorMacros.Switch Has Authority`
        (:`Authority`
          (`self.UpdateReplicates`))))
    (:`then_1`
      (`self.InitializePerPlayerTask`))))

(event `UpdateReplicates`
  ;[1 0.1543 0.1244] レプリケートの更新
)

(event `/Game/Werewolf_01/BP/BP_WerewolfInterface.WW_OnOpen`
  (params (PC :type "/Game/Werewolf_01/BP/Gameplay/BP_GameplayPlayerController Object Reference"))
  ;[1 0.1875 0.1875] タスクを開いたとき
  (`self.OnOpen` PC))

(event `OnOpen`
  (params (PC :type "/Game/Werewolf_01/BP/Gameplay/BP_GameplayPlayerController Object Reference"))
  (bind _character (`/Game/Werewolf_01/BP/Gameplay/BP_GameplayPlayerController.GetCharacter` PC))
  ;[1 0.1875 0.1875] タスクを開いたとき
  (`/Engine/EditorBlueprintResources/StandardMacros.IsValid` PC
    (:`Is Valid`
      (`|ExecutionSequence`
        (:`then_0`
          (`/Game/Werewolf_01/BP/Gameplay/BP_GameplayPlayerController.SetIsOpenTask` PC true) ; タスクを開いている状態を保存
          (`/Game/Werewolf_01/BP/Gameplay/BP_GameplayPlayerController.ShowTaskUI` PC (`self.TaskUIClass`) self) ; タスク画面を表示する
          (`/Game/Werewolf_01/BP/Gameplay/BP_GameplayPlayerController.EnableUIInput` PC) ; 画面入力を有効にする
          (`/Game/Werewolf_01/BP/Gameplay/BP_GameplayPlayerController.DisableGameInput` PC) ; ゲーム入力を無効にする
          (`/Engine/EditorBlueprintResources/StandardMacros.IsValid` _character
            (:`Is Valid`
              (`/Game/Werewolf_01/BP/Character/BP_WerewolfCharacter.SetCharacterMovementActive` _character false) ; キャラクターを移動不可にする
              (`/Game/Werewolf_01/BP/Character/BP_WerewolfCharacter.UpdateUseButtonEnabled` _character) ; USEボタンの有効性を更新
              (`/Game/Werewolf_01/BP/Character/BP_WerewolfCharacter.UpdateReportButtonEnable` _character) ; 通報ボタンの有効性を更新
            )))
        (:`then_1`
          ;;[1 1 1] カメラを使用する場合、タスクのカメラへ切り替える
          (if (`self.IsUseCamera`)
            (`/Game/Werewolf_01/BP/Gameplay/BP_GameplayPlayerController.MoveToTaskCamera` PC self) ; タスクのカメラへ移動
            (bind _gm (`/Game/Werewolf_01/BP/Gameplay/BP_GameplayPlayerController.GM` PC)
              (:`then`
                (`/Game/Werewolf_01/BP/Gameplay/BP_GameplayGameMode.SetAllCharacterVisibleToPlayer` _gm PC false) ; 全てのキャラクターを非表示にする
              )
              (:`else`))))
        (:`then_2`
          ;;[1 1 1] 非共有タスクを開く
          (`/Game/Werewolf_01/BP/Gameplay/BP_GameplayPlayerController.OnOpenPerPlayerTask` PC))))))

(event `InitializePerPlayerTask`
  ;[0.2026 0.2461 1] 非共有タスクを初期化
)

(event `/Game/Werewolf_01/BP/BP_WerewolfInterface.WW_Initialize`
  ;[1 0.2182 0.2083] 初期化
  (`self.Initialize`))

(event `Initialize`
  ;[1 0.2182 0.2083] 初期化
)

(event `OnOpenPerPlayerTask`
  (params (PC :type "/Game/Werewolf_01/BP/Gameplay/BP_GameplayPlayerController Object Reference"))
  ;[0.2026 0.2461 1] 非共有タスクを開いたとき
)

(event `OnClosePerPlayerTask`
  (params (PC :type "/Game/Werewolf_01/BP/Gameplay/BP_GameplayPlayerController Object Reference"))
  ;[0.2026 0.2461 1] 非共有タスクを閉じたとき
)

(event `PerPlayerTaskComplete`
  (params (PC :type "/Game/Werewolf_01/BP/Gameplay/BP_GameplayPlayerController Object Reference"))
  ;[0.2026 0.2461 1] 非共有タスクを完了する
  (`|ExecutionSequence`
    (:`then_0`
      (`/Engine/EditorBlueprintResources/StandardMacros.IsValid` PC
        (:`Is Valid`
          (`|ExecutionSequence`
            (:`then_0`
              (`/Game/Werewolf_01/BP/Gameplay/BP_GameplayPlayerController.AddCompletedTaskCount` PC 1))
            (:`then_1`
              ;;[1 1 1] ゲームが終了するか確認
              (if (`self.IsNormalTask`)
                (`/Game/Werewolf_01/BP/Gameplay/BP_GameplayPlayerController.GameFinishCheck` PC)))))))
    (:`then_1`
      (`self.OnCompleted` self PC))))

(event `/Game/Werewolf_01/BP/BP_WerewolfInterface.WW_OnClose`
  ;[1 0.1543 0.1244] タスクを閉じたとき
  (`self.OnClose` null))

(event `TaskComplete`
  (params (PC :type "/Game/Werewolf_01/BP/Gameplay/BP_GameplayPlayerController Object Reference"))
  (`|ExecutionSequence`
    (:`then_0`
      (set `self.IsEnable` false))
    (:`then_2`
      (if (`self.IsLightDown`)
        (bind _asbp_gameplay_game_mode (cast `/Game/Werewolf_01/BP/Gameplay/BP_GameplayGameMode` (`GameplayStatics.GetGameMode`)))
        (`/Game/Werewolf_01/BP/Gameplay/BP_GameplayGameMode.StartLightUp` _asbp_gameplay_game_mode)))
    (:`then_4`
      (if (not (`self.IsTasksPerPlayer`))
        (bind _asbp_gameplay_game_mode_2 (cast `/Game/Werewolf_01/BP/Gameplay/BP_GameplayGameMode` (`GameplayStatics.GetGameMode`)))
        (for _array_element (`/Game/Werewolf_01/BP/Gameplay/BP_GameplayGameMode.GetAllPC` _asbp_gameplay_game_mode_2)
          (`/Game/Werewolf_01/BP/Gameplay/BP_GameplayPlayerController.RemoveRemainingTaskToPlayer` _array_element self))))
    (:`then_5`
      (if (`self.IsSabotageTask`)
        (`self.SetIsCompleted` true)
        (if (not (`self.IsUseManager`))
          (`|ExecutionSequence`
            (:`then_0`
              (bind _asbp_gameplay_game_mode_3 (cast `/Game/Werewolf_01/BP/Gameplay/BP_GameplayGameMode` (`GameplayStatics.GetGameMode`)))
              (set `/Game/Werewolf_01/BP/Gameplay/BP_GameplayGameMode.IsSabotaging` false _asbp_gameplay_game_mode_3)
              (`/Game/Werewolf_01/BP/Gameplay/BP_GameplayGameMode.StartSabotageCoolDown` _asbp_gameplay_game_mode_3 (`self.CoolDownTime`))
              (if (`self.IsCommsSabotage`)
                (`/Game/Werewolf_01/BP/Gameplay/BP_GameplayGameMode.CommsEnable` _asbp_gameplay_game_mode_3 self) ; 通信を有効に戻す
              ))
            (:`then_1`
              (if (`self.GetIsEmergency`)
                (message `/Game/Werewolf_01/BP/BP_WerewolfInterface.WW_ClearEmergencyTimer` (`GameplayStatics.GetGameMode`))))))
        (else
          (`/Engine/EditorBlueprintResources/StandardMacros.IsValid` PC
            (:`Is Valid`
              (`/Game/Werewolf_01/BP/Gameplay/BP_GameplayPlayerController.AddCompletedTaskCount` PC 1)
              (`/Game/Werewolf_01/BP/Gameplay/BP_GameplayPlayerController.GameFinishCheck` PC))))))
    (:`then_6`
      (`self.OnCompleted` self PC))))

(event `/Game/Werewolf_01/BP/BP_WerewolfInterface.WW_TaskComplete`
  (params (PC_ :type "/Game/Werewolf_01/BP/Gameplay/BP_GameplayPlayerController Object Reference"))
  (`self.TaskComplete` PC_))

(event `OnClose`
  (params (PC :type "/Game/Werewolf_01/BP/Gameplay/BP_GameplayPlayerController Object Reference"))
  (bind _character (`/Game/Werewolf_01/BP/Gameplay/BP_GameplayPlayerController.GetCharacter` PC))
  ;[1 0.1543 0.1244] タスクを閉じたとき
  (`/Engine/EditorBlueprintResources/StandardMacros.IsValid` PC
    (:`Is Valid`
      (`|ExecutionSequence`
        (:`then_0`
          (`/Game/Werewolf_01/BP/Gameplay/BP_GameplayPlayerController.SetIsOpenTask` PC false) ; タスクを閉じている状態を保存
          (`/Game/Werewolf_01/BP/Gameplay/BP_GameplayPlayerController.RemoveTaskUI` PC) ; タスク画面を非表示
          (`/Game/Werewolf_01/BP/Gameplay/BP_GameplayPlayerController.DisableUIInput` PC) ; 画面入力を無効化
          (`/Game/Werewolf_01/BP/Gameplay/BP_GameplayPlayerController.EnableGameInput` PC) ; ゲーム入力を有効化
          (`/Engine/EditorBlueprintResources/StandardMacros.IsValid` _character
            (:`Is Valid`
              (`/Game/Werewolf_01/BP/Character/BP_WerewolfCharacter.SetCharacterMovementActive` _character true) ; キャラクターの移動を有効化
              (`/Game/Werewolf_01/BP/Character/BP_WerewolfCharacter.UpdateUseButtonEnabled` _character) ; USEボタンの有効性を更新
              (`/Game/Werewolf_01/BP/Character/BP_WerewolfCharacter.UpdateReportButtonEnable` _character) ; 通報ボタンの有効性を更新
            )))
        (:`then_1`
          ;;[1 1 1] カメラを使用する場合、キャラクターのカメラへ戻る
          (if (`self.GetIsUseCamera`)
            (`/Game/Werewolf_01/BP/Gameplay/BP_GameplayPlayerController.ReturnToCharacterCamera` PC)
            (bind _gm (`/Game/Werewolf_01/BP/Gameplay/BP_GameplayPlayerController.GM` PC)
              (:`then`
                (`/Game/Werewolf_01/BP/Gameplay/BP_GameplayGameMode.SetAllCharacterVisibleToPlayer` _gm PC true))
              (:`else`))))
        (:`then_2`
          (`/Game/Werewolf_01/BP/Gameplay/BP_GameplayPlayerController.CloseTaskPerPlayer` PC))))))

(event `/Game/Werewolf_01/BP/BP_WerewolfInterface.WW_SetIsCompleted`
  (params (NewParam :type Boolean))
  ;[1 0.2896 0.2598] タスクを完了したかをセット
  (`self.SetIsCompleted` NewParam))

(event `SetIsCompleted`
  (params (IsCompleted :type Boolean))
  ;[1 0.2896 0.2598] タスクを完了したかをセット
  (set `self.IsCompleted` IsCompleted))

(event `/Game/Werewolf_01/BP/BP_WerewolfInterface.WW_TaskEnable`
  ;[1 0.3 0.2702] タスクを有効にする
  (`self.TaskEnable` null))

(event `TaskEnable`
  (params (TargetPC :type "/Game/Werewolf_01/BP/Gameplay/BP_GameplayPlayerController Object Reference"))
  ;[1 0.3 0.2702] タスクを有効にする
  (`|ExecutionSequence`
    (:`then_0`
      ;;[1 1 1] 緊急のタスクなら緊急タイマーをセットする
      (if (`self.GetIsEmergency`)
        (if (not (`self.IsUseManager`))
          (bind _asbp_gameplay_game_mode (cast `/Game/Werewolf_01/BP/Gameplay/BP_GameplayGameMode` (`GameplayStatics.GetGameMode`)))
          (`/Game/Werewolf_01/BP/Gameplay/BP_GameplayGameMode.StartEmergencyTimer` _asbp_gameplay_game_mode self (`self.EmergencyTime`) (`self.CoolDownTime`) null))))
    (:`then_1`
      (if (`self.IsTasksPerPlayer`)
        ;[1 1 1] 非共有タスクをプレイヤーに割り当てる
        (`/Engine/EditorBlueprintResources/StandardMacros.IsValid` TargetPC
          (:`Is Valid`
            (`/Game/Werewolf_01/BP/Gameplay/BP_GameplayPlayerController.AssignTaskToPlayer` TargetPC self)))
        (else
          ;[1 1 1] 共有タスクのとき、タスクを未完了にする
          (`self.SetIsCompleted` false)
          ;[1 1 1] 全てのプレイヤーがタスクをこなせるようにする
          (bind _asbp_gameplay_game_mode_2 (cast `/Game/Werewolf_01/BP/Gameplay/BP_GameplayGameMode` (`GameplayStatics.GetGameMode`)))
          (for _array_element (`/Game/Werewolf_01/BP/Gameplay/BP_GameplayGameMode.GetAllPC` _asbp_gameplay_game_mode_2)
            (`/Game/Werewolf_01/BP/Gameplay/BP_GameplayPlayerController.AssignTaskToPlayer` _array_element self)
            (bind _character (`/Game/Werewolf_01/BP/Gameplay/BP_GameplayPlayerController.GetCharacter` _array_element))
            (`/Engine/EditorBlueprintResources/StandardMacros.IsValid` _character
              (:`Is Valid`
                (`/Game/Werewolf_01/BP/Character/BP_WerewolfCharacter.UpdateFieldOfVisionOverlap` _character)))))))
    (:`then_2`
      ;[1 1 1] 停電させるタスクのとき、停電を開始する
      (if (`self.IsLightDown`)
        (bind _asbp_gameplay_game_mode_3 (cast `/Game/Werewolf_01/BP/Gameplay/BP_GameplayGameMode` (`GameplayStatics.GetGameMode`)))
        (`/Game/Werewolf_01/BP/Gameplay/BP_GameplayGameMode.StartLightDown` _asbp_gameplay_game_mode_3 self)))
    (:`then_3`
      ;[1 1 1] 妨害のタスクのとき、妨害中にセット
      (if (`self.IsSabotageTask`)
        (bind _asbp_gameplay_game_mode_4 (cast `/Game/Werewolf_01/BP/Gameplay/BP_GameplayGameMode` (`GameplayStatics.GetGameMode`)))
        (set `/Game/Werewolf_01/BP/Gameplay/BP_GameplayGameMode.IsSabotaging` true _asbp_gameplay_game_mode_4)
        (`/Game/Werewolf_01/BP/Gameplay/BP_GameplayGameMode.UpdateSabotageButtonEnableToAllPlayers` _asbp_gameplay_game_mode_4)
        (if (`self.IsCommsSabotage`)
          (`/Game/Werewolf_01/BP/Gameplay/BP_GameplayGameMode.CommsDisable` _asbp_gameplay_game_mode_4 self))
        (else
          ;[1 1 1] 妨害タスクではないとき、有効なタスクの数を追加
          (bind _asbp_gameplay_game_mode_5 (cast `/Game/Werewolf_01/BP/Gameplay/BP_GameplayGameMode` (`GameplayStatics.GetGameMode`)))
          (`/Game/Werewolf_01/BP/Gameplay/BP_GameplayGameMode.AddEnableTaskCount` _asbp_gameplay_game_mode_5 1))))))

(event `SetIsUseManager`
  (params (IsUseManager :type Boolean))
  ;[1 1 1] マネージャーを使用するかをセット
  (set `self.IsUseManager` IsUseManager))

(event `TaskFail`
  ;[1 1 1] タスクを失敗する
  (`self.OnFail`))

(event `TaskFailPerPlayer`
  ;[1 1 1] 非共有タスクを失敗する
  (`GameplayStatics.PlaySound2D` "/Engine/EditorSounds/Notifications/CompileFailed.CompileFailed" 1.0 1.0 0.0 null null)
  (`self.OnFail`))

(event `HighlightOn`
  ;[1 1 1] ハイライトをオンにする
  (`|ExecutionSequence`
    (:`then_0`
      (`SceneComponent.SetVisibility` (`self.EnableWidget`) true false))
    (:`then_1`
      (`ArrowComponent.SetArrowColor` (`self.Arrow`) (struct :`R` 1.0 :`G` 0.896179 :`A` 1.0)))))

(event `HighlightOff`
  ;[1 1 1] ハイライトをオフにする
  (`|ExecutionSequence`
    (:`then_0`
      (`SceneComponent.SetVisibility` (`self.EnableWidget`) false false))
    (:`then_1`
      (`ArrowComponent.SetArrowColor` (`self.Arrow`) (struct :`G` 0.084233 :`B` 1.0 :`A` 1.0)))))

(fn `GetEmergencyTaskCoolDownTime`
  (returns (Time :type Integer))
  (return (`self.CoolDownTime`)))

(fn `GetEmergencyTime`
  (returns (EmergencyTime :type Integer))
  (return (`self.EmergencyTime`)))

(fn `GetIsCompleted`
  (returns (IsCompleted :type Boolean))
  (return (`self.IsCompleted`)))

(fn `GetIsEmergency`
  (returns (IsEmergency :type Boolean))
  (return (`self.IsEmergency`)))

(fn `GetIsEnable`
  (returns (IsEnable :type Boolean))
  (return (`self.IsEnable`)))

(fn `GetIsUseCamera`
  (returns (IsUseCamera :type Boolean))
  (return (`self.IsUseCamera`)))

(fn `IsNormalTask`
  (returns (ReturnValue :type Boolean))
  (return (and (not (`self.IsLightDown`)) (not (`self.IsEmergency`)))))

(fn `UserConstructionScript`
  (`parent.UserConstructionScript`)
  (`StaticMeshComponent.SetStaticMesh` (`self.StaticMesh`) (`self.Mesh`))
  (`SceneComponent.K2_SetRelativeLocation` (`self.SpringArm`) (`self.CameraOrigin`) false false)
  (set `SpringArmComponent.TargetArmLength` (`self.CameraDistance`) (`self.SpringArm`)))

(fn `WW_GetAllCharacters`
  (returns (Characters :type "Array of Actor Object Reference"))
  (return))

(fn `WW_GetAllPC`
  (returns (PC :type "Array of Actor Object Reference"))
  (return))

(fn `WW_GetAllPlayersCount`
  (returns (Count :type Integer))
  (return 0))

(fn `WW_GetAllWolfs`
  (returns (Wolfs :type "Array of Actor Object Reference"))
  (return))

(fn `WW_GetCanMovingHatches`
  (returns (Hatches :type "Array of Actor Object Reference"))
  (return))

(fn `WW_GetCanUseEmergencyButton`
  (params (UsedCount :type Integer))
  (returns (Can :type Boolean))
  (return false))

(fn `WW_GetCharacterType`
  (returns (CharacterType :type "/Game/Werewolf_01/Enum/e_CharacterType Enum"))
  (return "NewEnumerator1"))

(fn `WW_GetCompletedTaskCount`
  (returns (Count :type Integer))
  (return 0))

(fn `WW_GetEmergencyButton`
  (returns (EmergencyButton :type "Actor Object Reference"))
  (return null))

(fn `WW_GetEmergencyMeetingCoolTime`
  (returns (Time :type Integer))
  (return 0))

(fn `WW_GetEmergencyTasks`
  (returns (Tasks :type "Array of Actor Object Reference"))
  (return))

(fn `WW_GetGameSettings`
  (returns (GameSettings :type "Actor Object Reference"))
  (return null))

(fn `WW_GetIsCharacterCapsule`
  (params (Comp :type "SceneComponent Object Reference"))
  (returns (NewParam :type Boolean))
  (return false))

(fn `WW_GetIsDead`
  (returns (IsDead :type Boolean))
  (return false))

(fn `WW_GetIsEmergencyTaskCoolDown`
  (returns (IsCoolDown :type Boolean))
  (return false))

(fn `WW_GetIsEnableTask`
  (returns (IsEnable :type Boolean))
  (return (`self.GetIsEnable`)))

(fn `WW_GetIsGameFinished`
  (returns (IsGameFinished :type Boolean))
  (return false))

(fn `WW_GetIsInGame`
  (returns (IsInGame :type Boolean))
  (return false))

(fn `WW_GetIsInHatch`
  (returns (IsIn :type Boolean))
  (return false))

(fn `WW_GetIsInMeeting`
  (returns (In :type Boolean))
  (return false))

(fn `WW_GetIsInVotingTime`
  (returns (In :type Boolean))
  (return false))

(fn `WW_GetIsKillCoolDown`
  (returns (CoolDown :type Boolean))
  (return false))

(fn `WW_GetIsKilling`
  (returns (Killing :type Boolean))
  (return false))

(fn `WW_GetIsPlayerStart`
  (returns (NewParam :type Boolean))
  (return false))

(fn `WW_GetIsPutHand`
  (returns (IsPut :type Boolean))
  (return false))

(fn `WW_GetIsSabotageCoolDown`
  (returns (IsCoolDown :type Boolean))
  (return false))

(fn `WW_GetIsTaskManager`
  (returns (NewParam :type Boolean))
  (return false))

(fn `WW_GetIsUseCamera`
  (returns (Use :type Boolean))
  (return (`self.GetIsUseCamera`)))

(fn `WW_GetIsValidEmergencyTimer`
  (returns (IsValid :type Boolean))
  (return false))

(fn `WW_GetIsVotedToPlayer`
  (returns (NewParam :type Boolean))
  (return false))

(fn `WW_GetKillCoolDownTime`
  (returns (Time :type Integer))
  (return 0))

(fn `WW_GetMovingSpeed`
  (returns (Speed :type "Float (double-precision)"))
  (return 0.0))

(fn `WW_GetOverlapHatch`
  (returns (Hatch :type "/Game/Werewolf_01/BP/Hatch/BP_Hatch Object Reference"))
  (return null))

(fn `WW_GetPCByIndex`
  (params (Index :type Integer))
  (returns (PC :type "Actor Object Reference"))
  (return null))

(fn `WW_GetPlayerColorByIndex`
  (params (Index :type Integer))
  (returns (Color :type "LinearColor Structure"))
  (return))

(fn `WW_GetPlayerIndex`
  (returns (Index :type Integer))
  (return 0))

(fn `WW_GetPlayerName`
  (returns (Name :type String))
  (return ""))

(fn `WW_GetPlayerStarts`
  (returns (PlayerStarts :type "Array of Actor Object Reference"))
  (return))

(fn `WW_GetReportTarget`
  (returns (ReportTarget :type "Actor Object Reference"))
  (return null))

(fn `WW_GetSabotageCooldownPercent`
  (returns (Percent :type "Float (double-precision)"))
  (return 0.0))

(fn `WW_GetTask`
  (returns (Task :type "Actor Object Reference"))
  (return null))

(fn `WW_GetTaskManagers`
  (returns (TaskManagers :type "Array of Actor Object Reference"))
  (return))

(fn `WW_GetTaskUIClass`
  (returns (TaskUIClass :type "UserWidget Class Reference"))
  (return (`self.TaskUIClass`)))

(fn `WW_GetVotedFromPlayerCount`
  (returns (Count :type Integer))
  (return 0))

(fn `WW_GetVotedFromPlayerIndex`
  (returns (Index :type "Array of Integer"))
  (return))

(fn `WW_GetVoteTime`
  (returns (Time :type Integer))
  (return 0))

(fn `WW_IsCompleted`
  (returns (Completed :type Boolean))
  (return (`self.IsCompleted`)))

(fn `WW_IsCompletedAllTask`
  (returns (IsCompleted :type Boolean))
  (return false))

(fn `WW_IsControlledCharacter`
  (returns (ReturnValue :type Boolean))
  (return false))

(fn `WW_IsEmergencyButton`
  (returns (NewParam :type Boolean))
  (return false))

(fn `WW_IsEmergencyTask`
  (returns (NewParam :type Boolean))
  (return (`self.GetIsEmergency`)))

(fn `WW_IsGameSettings`
  (returns (ReturnValue :type Boolean))
  (return false))

(fn `WW_IsHatch`
  (returns (IsHatch :type Boolean))
  (return false))

(fn `WW_IsReportSphere`
  (params (Comp :type "PrimitiveComponent Object Reference"))
  (returns (NewParam :type Boolean))
  (return false))

(fn `WW_IsTask`
  (returns (NewParam :type Boolean))
  (return true))

(fn `WW_IsValidDeadBody`
  (returns (Valid :type Boolean))
  (return false))

(fn `WW_IsVillager`
  (returns (IsVillager :type Boolean))
  (return false))

(fn `WW_IsWolf`
  (returns (Wolf :type Boolean))
  (return false))

(fn `WW_SetCompletedTaskCount`
  (params (Count :type Integer))
  (return))

(fn `WW_SpawnPlayers`
  (returns (Vilagers :type "Array of /Game/Werewolf_01/BP/Character/BP_Villager Object Reference") (Wolfs :type "Array of /Game/Werewolf_01/BP/Character/BP_Wolf Object Reference"))
  (return))