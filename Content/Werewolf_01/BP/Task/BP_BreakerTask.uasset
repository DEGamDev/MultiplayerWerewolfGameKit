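; Breaker task actor in which a player flips switches until every one is on to complete the task.
; On authority, after a short delay, it respawns its child-actor BP_Switches (a standalone visibility workaround), caches them and binds their toggle events.
; TaskEnable randomizes each switch's IsOnLow flag, shuffles them to set OffCount off, and makes them touchable.
; When all are on, it calls TaskComplete on the toggling controller and locks the switches.
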(event `self.ReceiveBeginPlay`
  (`parent.ReceiveBeginPlay`)
  (`/Engine/EditorBlueprintResources/ActorMacros.Switch Has Authority`
    (:`Authority`
      (`KismetSystemLibrary.Delay` 1.0) ; Delayが無いと停電させたときに、スイッチが切り替わらない
      ;[1 1 1] スイッチをリフレッシュ　*この処理が無ければスタンドアローンでスイッチが表示されない
      (for _array_element (`self.K2_GetComponentsByClass` "/Script/Engine.ChildActorComponent")
        (`ChildActorComponent.SetChildActorClass` _array_element null)
        (`ChildActorComponent.SetChildActorClass` _array_element "/Game/Werewolf_01/BP/Gameplay/BP_Switch.BP_Switch_C"))
      (for _array_element_2 (`self.K2_GetComponentsByClass` "/Script/Engine.ChildActorComponent")
        ;[1 1 1] 全てのスイッチの参照を保存
        (bind _asbp_switch (cast `/Game/Werewolf_01/BP/Gameplay/BP_Switch` (`ChildActorComponent.ChildActor` _array_element_2)))
        (`KismetArrayLibrary.Array_Add` (`self.switches`) _asbp_switch))
      ;[1 1 1] スイッチを切り替えたときのイベントをバインド
      (for _array_element_3 (`self.switches`)
        (add `/Game/Werewolf_01/BP/Gameplay/BP_Switch.OnToggle` _array_element_3 (delegate `OnToggleSwitch`))))))

(event `self.TaskEnable`
  (params (TargetPC :type "/Game/Werewolf_01/BP/Gameplay/BP_GameplayPlayerController Object Reference"))
  (`parent.TaskEnable` TargetPC)
  (`self.SetUpSwitches`))

(event `OnToggleSwitch`
  (params (PC :type "/Game/Werewolf_01/BP/Gameplay/BP_GameplayPlayerController Object Reference"))
  (if (`self.isSuccess`)
    (`|ExecutionSequence`
      (:`then_0`
        (`/Game/Werewolf_01/BP/Gameplay/BP_GameplayPlayerController.TaskComplete` PC))
      (:`then_1`
        (for _array_element (`self.switches`)
          (set `/Game/Werewolf_01/BP/Gameplay/BP_Switch.canTouch` false _array_element))))))

(event `SetUpSwitches`
  ;[1 0.1543 0.1244] スイッチをセットアップ
  (`|ExecutionSequence`
    (:`then_0`
      (`self.UpdateIsOnLow`)
      (`self.UpdateSwitchTilt`))
    (:`then_1`
      (for _array_element (`self.switches`)
        (set `/Game/Werewolf_01/BP/Gameplay/BP_Switch.canTouch` true _array_element)))))

(fn `isSuccess`
  (returns (ReturnValue :type Boolean))
  (locals (isOn_l :type "Array of Boolean"))
  (for _array_element (`self.switches`)
    (`KismetArrayLibrary.Array_Add` (`local.isOn_l`) (`/Game/Werewolf_01/BP/Gameplay/BP_Switch.isOn` _array_element)))
  (return (not (`KismetArrayLibrary.Array_Contains` (`local.isOn_l`)))))

(fn `UpdateIsOnLow`
  (for _array_element (`self.switches`)
    (set `/Game/Werewolf_01/BP/Gameplay/BP_Switch.isOnLow` (`KismetMathLibrary.RandomBool`) _array_element)))

(fn `UpdateSwitchTilt`
  (locals (Switches_l :type "Array of /Game/Werewolf_01/BP/Gameplay/BP_Switch Object Reference"))
  (bind _switches_l (`local.Switches_l`))
  (set `local.Switches_l` (`self.switches`))
  (`|ExecutionSequence`
    (:`then_0`
      (`KismetArrayLibrary.Array_Shuffle` (`local.Switches_l`)))
    (:`then_1`
      (for _index (range (`self.switchCount`))
        (if (`KismetArrayLibrary.Array_IsValidIndex` _switches_l _index)
          (if (<= _index (- (`self.offCount`) 1))
            (bind _output (`|GetArrayItem` _switches_l _index))
            (`/Game/Werewolf_01/BP/Gameplay/BP_Switch.SetIsOn` _output false)
            (else
              (`/Game/Werewolf_01/BP/Gameplay/BP_Switch.SetIsOn` _output true))))))))

(fn `UserConstructionScript`
  (`parent.UserConstructionScript`))