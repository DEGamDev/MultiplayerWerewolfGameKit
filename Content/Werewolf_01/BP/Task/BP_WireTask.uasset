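; Per-player wire-connection task for the Werewolf game, where the player must correctly attach every colored wire.
; The construction script collects four BP_Wire child actors and assigns each a color and connection distance.
; Initialization shuffles the wires' end locations and binds their attach events, which complete the player's task once all wires report success.
; Opening the task resets and shows the wires, and closing it hides them.
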(event `self.TaskEnable`
  (params (TargetPC :type "/Game/Werewolf_01/BP/Gameplay/BP_GameplayPlayerController Object Reference"))
  (`parent.TaskEnable` TargetPC))

(event `self.InitializePerPlayerTask`
  ;[1 1 1] 初期化
  (`parent.InitializePerPlayerTask`)
  (`|ExecutionSequence`
    (:`then_0`
      ;;[1 1 1] ワイヤーが接続されたときのイベントをバインド
      (for _array_element (`self.Wires`)
        (`/Engine/EditorBlueprintResources/StandardMacros.IsValid` _array_element
          (:`Is Valid`
            (add `/Game/Werewolf_01/BP/Gameplay/BP_Wire.OnAttached` _array_element (delegate `OnAttached`))))))
    (:`then_1`
      (`self.ShuffleEndLocation`) ; ワイヤーをシャッフル
    )))

(event `OnAttached`
  (params (PC :type "/Game/Werewolf_01/BP/Gameplay/BP_GameplayPlayerController Object Reference"))
  ;[1 1 1] ワイヤーを接続したとき、全てのワイヤーが正しく接続されていたらタスクを完了する
  (bind _issuccess (`self.GetIsSuccess`))
  (if _issuccess
    (`/Engine/EditorBlueprintResources/StandardMacros.IsValid` PC
      (:`Is Valid`
        (`/Game/Werewolf_01/BP/Gameplay/BP_GameplayPlayerController.TaskComplete` PC)))))

(event `self.OnOpenPerPlayerTask`
  (params (PC :type "/Game/Werewolf_01/BP/Gameplay/BP_GameplayPlayerController Object Reference"))
  ;[1 1 1] タスクを開いたとき、ワイヤーの位置をリセットし、ワイヤーを表示する
  (`parent.OnOpenPerPlayerTask` PC)
  (`self.ResetWiresLocation`)
  (`self.SetWiresVisible` true))

(event `ResetWiresLocation`
  ;[1 1 1] ワイヤーの位置をリセット
  (for _array_element (`self.Wires`)
    (`/Engine/EditorBlueprintResources/StandardMacros.IsValid` _array_element
      (:`Is Valid`
        (`/Game/Werewolf_01/BP/Gameplay/BP_Wire.ResetWireLocation` _array_element)))))

(event `SetWiresVisible`
  (params (Visibility :type Boolean))
  ;[1 1 1] 全てのワイヤーの可視性をセット
  (for _array_element (`self.Wires`)
    (`/Engine/EditorBlueprintResources/StandardMacros.IsValid` _array_element
      (:`Is Valid`
        (`/Game/Werewolf_01/BP/Gameplay/BP_Wire.SetWireVisible` _array_element Visibility)))))

(event `self.OnClosePerPlayerTask`
  (params (PC :type "/Game/Werewolf_01/BP/Gameplay/BP_GameplayPlayerController Object Reference"))
  ;[1 1 1] タスクを閉じたとき、全てのワイヤーを非表示にする
  (`parent.OnClosePerPlayerTask` PC)
  (`self.SetWiresVisible` false))

(fn `GetIsSuccess`
  (returns (isSuccess :type Boolean))
  (locals (isSuccess_l :type "Array of Boolean"))
  (`|ExecutionSequence`
    (:`then_0`
      (for _array_element (`self.Wires`)
        (`KismetArrayLibrary.Array_Add` (`local.isSuccess_l`) (`/Game/Werewolf_01/BP/Gameplay/BP_Wire.isSuccess` _array_element))))
    (:`then_1`
      (return (not (`KismetArrayLibrary.Array_Contains` (`local.isSuccess_l`)))))))

(fn `ShuffleEndLocation`
  (locals (NewLocalVar_0 :type "Array of Vector Structure") (NewLocalVar_1 :type Integer :default 0))
  (`|ExecutionSequence`
    (:`then_0`
      (for _array_element (`self.Wires`)
        (`KismetArrayLibrary.Array_Add` (`local.NewLocalVar_0`) (`/Game/Werewolf_01/BP/Gameplay/BP_Wire.GetEndLocation` _array_element))))
    (:`then_1`
      (`KismetArrayLibrary.Array_Shuffle` (`local.NewLocalVar_0`)))
    (:`then_2`
      (for (_array_element_2 _array_index) (`self.Wires`)
        (`/Game/Werewolf_01/BP/Gameplay/BP_Wire.SetEndLocation` _array_element_2 (`|GetArrayItem` (`local.NewLocalVar_0`) _array_index))))))

(fn `UserConstructionScript`
  (bind _colors (`self.colors`))
  (`parent.UserConstructionScript`)
  (for _array_element (`|MakeArray` (`self.CA_Wire_01`) (`self.CA_Wire_02`) (`self.CA_Wire_04`) (`self.CA_Wire_03`))
    (`ChildActorComponent.SetChildActorClass` _array_element (select `bool` (`self.isPreview`) :`true` "/Game/Werewolf_01/BP/Gameplay/BP_Wire.BP_Wire_C" :!type "Actor Class Reference"))
    (bind _asbp_wire (cast `/Game/Werewolf_01/BP/Gameplay/BP_Wire` (`ChildActorComponent.ChildActor` _array_element)))
    (`KismetArrayLibrary.Array_Add` (`self.Wires`) _asbp_wire))
  (for (_array_element_2 _array_index) (`self.Wires`)
    (if (`KismetArrayLibrary.Array_IsValidIndex` _colors _array_index)
      (`/Game/Werewolf_01/BP/Gameplay/BP_Wire.SetColor` _array_element_2 (`|GetArrayItem` _colors _array_index))
      (`/Game/Werewolf_01/BP/Gameplay/BP_Wire.SetConnectionDistance` _array_element_2 (`self.ConnectionDistance`)))))