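; Per-player comms task in which the player drags a dial to tune to a random target value.
; Mouse deprojection onto the dial's plane sets the angle, whose wrapped distance from the target drives noise volume and left waveform width.
; Within tolerance, the red lamp turns off and releasing calls TaskComplete on the player controller.
; Construction builds the lamp and waveform dynamic materials; opening and closing the task start and stop the noise.
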(event `PlayNoiseSound`
  (`|ExecutionSequence`
    (:`then_0`
      (`self.NoiseSound`
        (:`then`
          (`KismetSystemLibrary.PrintString` "PlayNoiseSound Failed" true true (struct :`R` 1.0 :`A` 1.0)))
        (:`else`
          (bind _returnvalue (`GameplayStatics.SpawnSound2D` "/Game/Werewolf_01/Sound/Cue_Noise.Cue_Noise" 0.5 0.5 0.0 null))
          (set `self.NoiseSound` _returnvalue))))
    (:`then_1`
      (`self.UpdateAngle` (`self.angle`) true))))

(event `self.OnOpenPerPlayerTask`
  (params (PC :type "/Game/Werewolf_01/BP/Gameplay/BP_GameplayPlayerController Object Reference"))
  (`parent.OnOpenPerPlayerTask` PC)
  (`self.PlayNoiseSound`))

(event `self.TaskEnable`
  (params (TargetPC :type "/Game/Werewolf_01/BP/Gameplay/BP_GameplayPlayerController Object Reference"))
  (`parent.TaskEnable` TargetPC))

(event `self.InitializePerPlayerTask`
  ;[0.2026 0.2461 1] 初期化
  (`parent.InitializePerPlayerTask`)
  (set `self.successValue` (`KismetMathLibrary.RandomFloat`)))

(event `/Game/Werewolf_01/BP/BP_TouchInterface.TCH_Move`
  (params (PC :type "/Game/Werewolf_01/BP/Gameplay/BP_GameplayPlayerController Object Reference") (Location :type "Vector Structure"))
  (bind (_worldlocation _worlddirection) (`PlayerController.DeprojectMousePositionToWorld` PC))
  (bind (_t _intersection _returnvalue) (`KismetMathLibrary.LinePlaneIntersection_OriginNormal` _worldlocation (+ _worldlocation (* _worlddirection 1000.0)) (`self.K2_GetActorLocation`) (`self.GetActorForwardVector`)))
  ;[0.2026 0.2461 1] ダイヤルの角度をセット
  (`/Engine/EditorBlueprintResources/StandardMacros.IsValid` PC
    (:`Is Valid`
      (if _returnvalue
        (`self.SetAngle` _intersection)))))

(event `/Game/Werewolf_01/BP/BP_TouchInterface.TCH_Release`
  (params (PC :type "/Game/Werewolf_01/BP/Gameplay/BP_GameplayPlayerController Object Reference") (Actor :type "Actor Object Reference") (Comp :type "SceneComponent Object Reference"))
  ;[0.2026 0.2461 1] 成功しているとき、プレイヤーコントローラーにタスク完了イベントを呼ぶ
  (if (`self.isSuccess`)
    (`/Game/Werewolf_01/BP/Gameplay/BP_GameplayPlayerController.TaskComplete` PC)))

(event `UpdateNoiseSoundScale`
  (params (Difference :type "Float (double-precision)"))
  ;[1 1 1] ノイズの音量を更新
  (bind _noisesound (`self.NoiseSound`)
    (:`then`
      (`AudioComponent.SetVolumeMultiplier` _noisesound (`KismetMathLibrary.Lerp` 0.0 0.1 Difference)))
    (:`else`
      (`KismetSystemLibrary.PrintString` "UpdateNoiseSoundScale Failed" true true (struct :`R` 1.0 :`A` 1.0)))))

(event `self.OnClosePerPlayerTask`
  (params (PC :type "/Game/Werewolf_01/BP/Gameplay/BP_GameplayPlayerController Object Reference"))
  ;[1 1 1] タスクを閉じたとき、ノイズの音を削除
  (`parent.OnClosePerPlayerTask` PC)
  (bind _noisesound (`self.NoiseSound`)
    (:`then`
      (`AudioComponent.Stop` _noisesound)
      (`ActorComponent.K2_DestroyComponent` _noisesound))
    (:`else`
      (`KismetSystemLibrary.PrintString` "Stop NoiseSound Failed" true true (struct :`R` 1.0 :`A` 1.0)))))

(fn `GetValue`
  (returns (ReturnValue :type "Float (double-precision)"))
  (return (- 1.0 (`KismetMathLibrary.Abs` (mod (+ (/ (+ (.roll (`SceneComponent.RelativeRotation` (`self.DialMeshRoot`))) 180.0) 360.0) 0.5) 1.0)))))

(fn `SetAngle`
  (params (location :type "Vector Structure"))
  (locals (value_l :type "Float (double-precision)" :default 0.0))
  (`|ExecutionSequence`
    (:`then_0`
      (bind _output_get (set `local.value_l` (- 1.0 (`KismetMathLibrary.Abs` (mod (+ (/ (+ (.roll (`KismetMathLibrary.MakeRotFromXY` (`self.GetActorForwardVector`) (`KismetMathLibrary.GetForwardVector` (`KismetMathLibrary.FindLookAtRotation` (`SceneComponent.K2_GetComponentLocation` (`self.DialMeshRoot`)) location)))) 180.0) 360.0) 0.5) 1.0)))))
      (set `self.angle` _output_get)
      (bind _output_get_2 (set `self.isSuccess` (`KismetMathLibrary.NearlyEqual_FloatFloat` (`local.value_l`) (`self.successValue`) (`self.successTolerance`))))
      (if _output_get_2
        (`self.SetRampBrightness` (`self.M_RedRamp`))
        (else
          (`self.SetRampBrightness` (`self.M_RedRamp`) 2.0))))
    (:`then_1`
      (`self.UpdateAngle` (`self.angle`) true))))

(fn `SetRampBrightness`
  (params (M_Ramp :type "MaterialInstanceDynamic Object Reference") (Value :type "Float (double-precision)"))
  (`MaterialInstanceDynamic.SetScalarParameterValue` M_Ramp "Brightness" Value))

(fn `SetRampColor`
  (params (M_Ramp :type "MaterialInstanceDynamic Object Reference") (Color :type "LinearColor Structure"))
  (`MaterialInstanceDynamic.SetVectorParameterValue` M_Ramp "Color" Color))

(fn `UpdateAngle`
  (params (Value :type "Float (double-precision)") (UpdateSound :type Boolean))
  (bind _returnvalue (- Value (`self.successValue`)))
  (bind _returnvalue_2 (`KismetMathLibrary.Abs` (mod _returnvalue 0.5)))
  (bind _returnvalue_3 (/ (`KismetMathLibrary.SelectFloat` (- 0.5 _returnvalue_2) _returnvalue_2 (> (`KismetMathLibrary.Abs` _returnvalue) 0.5)) 0.5))
  (`|ExecutionSequence`
    (:`then_0`
      (`SceneComponent.K2_SetRelativeRotation` (`self.DialMeshRoot`) (`KismetMathLibrary.MakeRotator` (`KismetMathLibrary.Lerp` 0.0 -360.0 Value)) false false)
      (if UpdateSound
        (`self.UpdateNoiseSoundScale` _returnvalue_3)))
    (:`then_1`
      (bind _m_wave_l (`self.M_Wave_L`)
        (:`then`
          (`MaterialInstanceDynamic.SetScalarParameterValue` _m_wave_l "Width" (`KismetMathLibrary.Lerp` 1.0 (`self.WaveWidth`) _returnvalue_3)))
        (:`else`)))))

(fn `UserConstructionScript`
  (bind _m_wave_r (`self.M_Wave_R`))
  (bind _m_wave_l (`self.M_Wave_L`))
  (`parent.UserConstructionScript`)
  (`|ExecutionSequence`
    (:`then_0`
      ;[1 1 1] ランプ
      (`|ExecutionSequence`
        (:`then_0`
          ;[1 1 1] 緑色のランプのマテリアルをセット
          (bind _returnvalue (`PrimitiveComponent.CreateDynamicMaterialInstance` (`self.GreenRampMesh`) 0 null "None"))
          (bind _output_get (set `self.M_GreenRamp` _returnvalue))
          (`self.SetRampColor` _output_get (struct :`G` 0.057292 :`B` 0.002391 :`A` 1.0))
          (`self.SetRampBrightness` _output_get 1.0))
        (:`then_1`
          ;[1 1 1] 赤色のランプのマテリアルをセット
          (bind _returnvalue_2 (`PrimitiveComponent.CreateDynamicMaterialInstance` (`self.RedRampMesh`) 0 null "None"))
          (bind _output_get_2 (set `self.M_RedRamp` _returnvalue_2))
          (`self.SetRampColor` _output_get_2 (struct :`R` 0.145833 :`G` 0.001255 :`A` 1.0))
          (`self.SetRampBrightness` _output_get_2 2.0))))
    (:`then_1`
      ;[1 1 1] 音声波形
      (`|ExecutionSequence`
        (:`then_0`
          ;[1 1 1] 右側の音声波形のマテリアルをセット
          (bind _returnvalue_3 (`KismetMaterialLibrary.CreateDynamicMaterialInstance` "/Game/Werewolf_01/Materials/M_Wave.M_Wave"))
          (set `self.M_Wave_R` _returnvalue_3)
          (`PrimitiveComponent.SetMaterial` (`self.WaveMesh_R`) 0 _m_wave_r)
          (`MaterialInstanceDynamic.SetVectorParameterValue` _m_wave_r "BackColor" (`self.backColor`))
          (`MaterialInstanceDynamic.SetVectorParameterValue` _m_wave_r "WaveColor" (`self.waveColor`))
          (`MaterialInstanceDynamic.SetScalarParameterValue` _m_wave_r "Noise" 0.0))
        (:`then_1`
          ;[1 1 1] 左側の音声波形のマテリアルをセット
          (bind _returnvalue_4 (`KismetMaterialLibrary.CreateDynamicMaterialInstance` "/Game/Werewolf_01/Materials/M_Wave.M_Wave"))
          (set `self.M_Wave_L` _returnvalue_4)
          (`PrimitiveComponent.SetMaterial` (`self.WaveMesh_L`) 0 _m_wave_l)
          (`MaterialInstanceDynamic.SetVectorParameterValue` _m_wave_l "BackColor" (`self.backColor`))
          (`MaterialInstanceDynamic.SetVectorParameterValue` _m_wave_l "WaveColor" (`self.waveColor`)))))
    (:`then_2`
      (`self.UpdateAngle` (`self.angle`)))))