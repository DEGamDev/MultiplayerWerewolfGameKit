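; Task manager actor that groups several tasks into one set, optionally an emergency, for the Werewolf game.
; On the server, it flags its tasks as manager-controlled and binds their completion events; EnableSetTask enables them and starts the GameMode's emergency timer if needed.
; Once all report complete, it clears that timer, removes the tasks from every player and closes open ones.
; It identifies itself via the WW interface, leaving other getters as stubs.
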(event `BindEvent`
  ;[1 1 1] タスクを完了したときにイベントをバインド
  (for _array_element (`self.GetTasks`)
    (`/Engine/EditorBlueprintResources/StandardMacros.IsValid` _array_element
      (:`Is Valid`
        (add `/Game/Werewolf_01/BP/Task/BP_Task.OnCompleted` _array_element (delegate `OnTaskCompleted`))))))

(event `self.ReceiveBeginPlay`
  (`/Engine/EditorBlueprintResources/ActorMacros.Switch Has Authority`
    (:`Authority`
      (`self.BindEvent`)
      (`self.UpdateTaskUseManager`))))

(event `UpdateTaskUseManager`
  ;[1 1 1] マネージャーを使用するようにセット
  (for _array_element (`self.Tasks`)
    (`/Engine/EditorBlueprintResources/StandardMacros.IsValid` _array_element
      (:`Is Valid`
        (`/Game/Werewolf_01/BP/Task/BP_Task.SetIsUseManager` _array_element true)))))

(event `OnTaskCompleted`
  (params (Task :type "Actor Object Reference") (PC :type "/Game/Werewolf_01/BP/Gameplay/BP_GameplayPlayerController Object Reference"))
  ;[1 1 1] タスクを完了したとき
  (bind _completed (`self.Get Is Tasks Complete`))
  (if _completed
    (`self.SetTaskComplete`)))

(event `EnableSetTask`
  ;[1 1 1] セットタスクを有効にする
  (`|ExecutionSequence`
    (:`then_0`
      ;;[1 1 1] 緊急タイマーを開始する
      (if (`self.IsEmergency`)
        (bind _asbp_gameplay_game_mode (cast `/Game/Werewolf_01/BP/Gameplay/BP_GameplayGameMode` (`GameplayStatics.GetGameMode`)))
        (`/Game/Werewolf_01/BP/Gameplay/BP_GameplayGameMode.StartEmergencyTimer` _asbp_gameplay_game_mode null (`self.Emergency Time`) (`self.EmergencyCooldown`) self)))
    (:`then_1`
      (for _array_element (`self.Tasks`)
        (`/Engine/EditorBlueprintResources/StandardMacros.IsValid` _array_element
          (:`Is Valid`
            (message `/Game/Werewolf_01/BP/BP_WerewolfInterface.WW_TaskEnable` _array_element)))))))

(event `SetTaskComplete`
  ;[1 0.1869 0.2167] セットタスクを完了する
  (`|ExecutionSequence`
    (:`then_0`
      (if (`self.IsEmergency`)
        (message `/Game/Werewolf_01/BP/BP_WerewolfInterface.WW_ClearEmergencyTimer` (`GameplayStatics.GetGameMode`))))
    (:`then_1`
      (bind _asbp_gameplay_game_mode (cast `/Game/Werewolf_01/BP/Gameplay/BP_GameplayGameMode` (`GameplayStatics.GetGameMode`)))
      (for _array_element (`self.Tasks`)
        (`/Engine/EditorBlueprintResources/StandardMacros.IsValid` _array_element
          (:`Is Valid`
            ;;[1 1 1] 全てのプレイヤーからタスクを開けなくする
            (for _array_element_2 (`/Game/Werewolf_01/BP/Gameplay/BP_GameplayGameMode.GetAllPC` _asbp_gameplay_game_mode)
              (`/Engine/EditorBlueprintResources/StandardMacros.IsValid` _array_element_2
                (:`Is Valid`
                  (`/Game/Werewolf_01/BP/Gameplay/BP_GameplayPlayerController.RemoveRemainingTaskToPlayer` _array_element_2 _array_element)
                  (if (== (`/Game/Werewolf_01/BP/Gameplay/BP_GameplayPlayerController.GetTask` _array_element_2) _array_element)
                    (`/Game/Werewolf_01/BP/Gameplay/BP_GameplayPlayerController.CloseTask` _array_element_2) ; タスクマネージャーのタスクを開いていたら閉じる
                  )))))))
      (`KismetSystemLibrary.PrintString` "SetTaskCompleted" true true (struct :`R` 1.0 :`G` 0.351839 :`A` 1.0)))))

(fn `Get Is Tasks Complete`
  (returns (Completed :type Boolean))
  (for _array_element (`self.Tasks`)
    (bind _completed (message `/Game/Werewolf_01/BP/BP_WerewolfInterface.WW_IsCompleted` _array_element))
    (if (not _completed)
      (return false)))
  (return true))

(fn `GetTasks`
  (returns (Tasks :type "Array of /Game/Werewolf_01/BP/Task/BP_Task Object Reference"))
  (return (`self.Tasks`)))

(fn `UserConstructionScript`)

(fn `WW_GetAllCharacters`
  (returns (Characters :type "Array of Actor Object Reference"))
  (return))

(fn `WW_GetAllPC`
  (returns (PC :type "Array of Actor Object Reference"))
  (return))

(fn `WW_GetAllPlayersCount`
  (returns (Count :type Integer))
  (return 0))

(fn `WW_GetAllWolfs`
  (returns (Wolfs :type "Array of Actor Object Reference"))
  (return))

(fn `WW_GetCanMovingHatches`
  (returns (Hatches :type "Array of Actor Object Reference"))
  (return))

(fn `WW_GetCanUseEmergencyButton`
  (params (UsedCount :type Integer))
  (returns (Can :type Boolean))
  (return false))

(fn `WW_GetCharacterType`
  (returns (CharacterType :type "/Game/Werewolf_01/Enum/e_CharacterType Enum"))
  (return "NewEnumerator1"))

(fn `WW_GetCompletedTaskCount`
  (returns (Count :type Integer))
  (return 0))

(fn `WW_GetEmergencyButton`
  (returns (EmergencyButton :type "Actor Object Reference"))
  (return null))

(fn `WW_GetEmergencyMeetingCoolTime`
  (returns (Time :type Integer))
  (return 0))

(fn `WW_GetEmergencyTasks`
  (returns (Tasks :type "Array of Actor Object Reference"))
  (return))

(fn `WW_GetGameSettings`
  (returns (GameSettings :type "Actor Object Reference"))
  (return null))

(fn `WW_GetIsCharacterCapsule`
  (params (Comp :type "SceneComponent Object Reference"))
  (returns (NewParam :type Boolean))
  (return false))

(fn `WW_GetIsDead`
  (returns (IsDead :type Boolean))
  (return false))

(fn `WW_GetIsEmergencyTaskCoolDown`
  (returns (IsCoolDown :type Boolean))
  (return false))

(fn `WW_GetIsEnableTask`
  (returns (IsEnable :type Boolean))
  (return false))

(fn `WW_GetIsGameFinished`
  (returns (IsGameFinished :type Boolean))
  (return false))

(fn `WW_GetIsInGame`
  (returns (IsInGame :type Boolean))
  (return false))

(fn `WW_GetIsInHatch`
  (returns (IsIn :type Boolean))
  (return false))

(fn `WW_GetIsInMeeting`
  (returns (In :type Boolean))
  (return false))

(fn `WW_GetIsInVotingTime`
  (returns (In :type Boolean))
  (return false))

(fn `WW_GetIsKillCoolDown`
  (returns (CoolDown :type Boolean))
  (return false))

(fn `WW_GetIsKilling`
  (returns (Killing :type Boolean))
  (return false))

(fn `WW_GetIsPlayerStart`
  (returns (NewParam :type Boolean))
  (return false))

(fn `WW_GetIsPutHand`
  (returns (IsPut :type Boolean))
  (return false))

(fn `WW_GetIsSabotageCoolDown`
  (returns (IsCoolDown :type Boolean))
  (return false))

(fn `WW_GetIsTaskManager`
  (returns (NewParam :type Boolean))
  (return true) ; 自分はタスクマネージャー
)

(fn `WW_GetIsUseCamera`
  (returns (Use :type Boolean))
  (return false))

(fn `WW_GetIsValidEmergencyTimer`
  (returns (IsValid :type Boolean))
  (return false))

(fn `WW_GetIsVotedToPlayer`
  (returns (NewParam :type Boolean))
  (return false))

(fn `WW_GetKillCoolDownTime`
  (returns (Time :type Integer))
  (return 0))

(fn `WW_GetMovingSpeed`
  (returns (Speed :type "Float (double-precision)"))
  (return 0.0))

(fn `WW_GetOverlapHatch`
  (returns (Hatch :type "/Game/Werewolf_01/BP/Hatch/BP_Hatch Object Reference"))
  (return null))

(fn `WW_GetPCByIndex`
  (params (Index :type Integer))
  (returns (PC :type "Actor Object Reference"))
  (return null))

(fn `WW_GetPlayerColorByIndex`
  (params (Index :type Integer))
  (returns (Color :type "LinearColor Structure"))
  (return))

(fn `WW_GetPlayerIndex`
  (returns (Index :type Integer))
  (return 0))

(fn `WW_GetPlayerName`
  (returns (Name :type String))
  (return ""))

(fn `WW_GetPlayerStarts`
  (returns (PlayerStarts :type "Array of Actor Object Reference"))
  (return))

(fn `WW_GetReportTarget`
  (returns (ReportTarget :type "Actor Object Reference"))
  (return null))

(fn `WW_GetSabotageCooldownPercent`
  (returns (Percent :type "Float (double-precision)"))
  (return 0.0))

(fn `WW_GetTask`
  (returns (Task :type "Actor Object Reference"))
  (return null))

(fn `WW_GetTaskManagers`
  (returns (TaskManagers :type "Array of Actor Object Reference"))
  (return))

(fn `WW_GetTaskUIClass`
  (returns (TaskUIClass :type "UserWidget Class Reference"))
  (return null))

(fn `WW_GetVotedFromPlayerCount`
  (returns (Count :type Integer))
  (return 0))

(fn `WW_GetVotedFromPlayerIndex`
  (returns (Index :type "Array of Integer"))
  (return))

(fn `WW_GetVoteTime`
  (returns (Time :type Integer))
  (return 0))

(fn `WW_IsCompleted`
  (returns (Completed :type Boolean))
  (return false))

(fn `WW_IsCompletedAllTask`
  (returns (IsCompleted :type Boolean))
  (return false))

(fn `WW_IsControlledCharacter`
  (returns (ReturnValue :type Boolean))
  (return false))

(fn `WW_IsEmergencyButton`
  (returns (NewParam :type Boolean))
  (return false))

(fn `WW_IsEmergencyTask`
  (returns (NewParam :type Boolean))
  (return false))

(fn `WW_IsGameSettings`
  (returns (ReturnValue :type Boolean))
  (return false))

(fn `WW_IsHatch`
  (returns (IsHatch :type Boolean))
  (return false))

(fn `WW_IsReportSphere`
  (params (Comp :type "PrimitiveComponent Object Reference"))
  (returns (NewParam :type Boolean))
  (return false))

(fn `WW_IsTask`
  (returns (NewParam :type Boolean))
  (return false))

(fn `WW_IsValidDeadBody`
  (returns (Valid :type Boolean))
  (return false))

(fn `WW_IsVillager`
  (returns (IsVillager :type Boolean))
  (return false))

(fn `WW_IsWolf`
  (returns (Wolf :type Boolean))
  (return false))

(fn `WW_SpawnPlayers`
  (returns (Vilagers :type "Array of /Game/Werewolf_01/BP/Character/BP_Villager Object Reference") (Wolfs :type "Array of /Game/Werewolf_01/BP/Character/BP_Wolf Object Reference"))
  (return))