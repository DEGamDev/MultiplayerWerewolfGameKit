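; Password-entry task for the werewolf game: the player types digits to match a randomly generated code and complete the task.
; Initialize rolls the code; on open, the task asks the player controller to clear the input and refresh the O2 task widget.
; Digit, delete and confirm events play sounds and update input, capped at code length.
; A match completes the task and later shows OK; a mismatch clears input and signals failure.
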(event `self.Initialize`
  ;[1 1 1] 初期化されたとき、パスワードをセットする
  (`parent.Initialize`)
  (`self.SetNumber`))

(event `self.OnOpen`
  (params (PC :type "/Game/Werewolf_01/BP/Gameplay/BP_GameplayPlayerController Object Reference"))
  ;[1 0.1543 0.1244] タスクを開いたとき、パスワードを表示する
  (`parent.OnOpen` PC)
  (`/Engine/EditorBlueprintResources/StandardMacros.IsValid` PC
    (:`Is Valid`
      (`/Game/Werewolf_01/BP/Gameplay/BP_GameplayPlayerController.ClearO2Number` PC self)
      (`/Game/Werewolf_01/BP/Gameplay/BP_GameplayPlayerController.UpdateO2InputNumber` PC self)
      (`/Game/Werewolf_01/BP/Gameplay/BP_GameplayPlayerController.UpdateO2Number` PC self))))

(event `EnterNumber`
  (params (number :type Integer) (PC :type "/Game/Werewolf_01/BP/Gameplay/BP_GameplayPlayerController Object Reference"))
  ;[1 1 1] 番号を入力する
  (`/Engine/EditorBlueprintResources/StandardMacros.IsValid` PC
    (:`Is Valid`
      (`|ExecutionSequence`
        (:`then_0`
          (set `self.InputNumber` (`KismetStringLibrary.GetSubstring` (`KismetStringLibrary.Concat_StrStr` (`self.InputNumber`) (`KismetStringLibrary.Conv_IntToString` number)) 0 (`self.numberLength`)))
          (`self.UpdateInputNumber` PC))
        (:`then_1`
          (`GameplayStatics.PlaySound2D` "/Game/Werewolf_01/Interface_And_Item_Sounds/Cues/Coins_05_Cue.Coins_05_Cue" 1.0 1.0 0.0 null null))))))

(event `SetNumber`
  ;[0.2026 0.2461 1] 正解の番号をセット
  (set `self.number` "")
  (for _ (range (`self.numberLength`))
    (set `self.number` (`KismetStringLibrary.Concat_StrStr` (`self.number`) (`KismetStringLibrary.Conv_IntToString` (`KismetMathLibrary.RandomInteger` 10))))))

(event `Confirm`
  (params (PC :type "/Game/Werewolf_01/BP/Gameplay/BP_GameplayPlayerController Object Reference"))
  ;[1 1 1] 入力を確定する
  (`/Engine/EditorBlueprintResources/StandardMacros.IsValid` PC
    (:`Is Valid`
      (if (`KismetStringLibrary.EqualEqual_StrStr` (`self.number`) (`self.InputNumber`))
        (`/Game/Werewolf_01/BP/Gameplay/BP_GameplayPlayerController.TaskComplete` PC)
        (`GameplayStatics.PlaySound2D` "/Game/Werewolf_01/Interface_And_Item_Sounds/Cues/Special_Musical_05_Cue.Special_Musical_05_Cue" 1.0 1.0 0.0 null null)
        (else
          (`|ExecutionSequence`
            (:`then_0`
              (`self.ClearNumber` PC))
            (:`then_1`
              (`GameplayStatics.PlaySound2D` "/Game/Werewolf_01/Interface_And_Item_Sounds/Cues/Error_Buzz_04_Cue.Error_Buzz_04_Cue" 1.0 1.0 0.0 null null))
            (:`then_2`
              (bind _asui_task_o2 (cast `/Game/Werewolf_01/UI/Task/UI_Task_O2` (`/Game/Werewolf_01/BP/Gameplay/BP_GameplayPlayerController.GetUI_Task` PC)))
              (`/Game/Werewolf_01/UI/Task/UI_Task_O2.Fail` _asui_task_o2))))))))

(event `UpdateNumber`
  (params (PC :type "/Game/Werewolf_01/BP/Gameplay/BP_GameplayPlayerController Object Reference"))
  ;[0.2825 0.3984 1] 正解の番号を更新
  (`/Engine/EditorBlueprintResources/StandardMacros.IsValid` PC
    (:`Is Valid`
      (bind _asui_task_o2 (cast `/Game/Werewolf_01/UI/Task/UI_Task_O2` (`/Game/Werewolf_01/BP/Gameplay/BP_GameplayPlayerController.GetUI_Task` PC)))
      (`/Game/Werewolf_01/UI/Task/UI_Task_O2.SetNumber` _asui_task_o2 (`self.number`)))))

(event `UpdateInputNumber`
  (params (PC :type "/Game/Werewolf_01/BP/Gameplay/BP_GameplayPlayerController Object Reference"))
  ;[0.2026 0.2461 1] 入力番号の表示を更新
  (`/Engine/EditorBlueprintResources/StandardMacros.IsValid` PC
    (:`Is Valid`
      (bind _asui_task_o2 (cast `/Game/Werewolf_01/UI/Task/UI_Task_O2` (`/Game/Werewolf_01/BP/Gameplay/BP_GameplayPlayerController.GetUI_Task` PC)))
      (`/Game/Werewolf_01/UI/Task/UI_Task_O2.SetInputNumber` _asui_task_o2 (`self.InputNumber`)))))

(event `ClearNumber`
  (params (PC :type "/Game/Werewolf_01/BP/Gameplay/BP_GameplayPlayerController Object Reference"))
  ;[1 1 1] 入力した番号を削除する
  (set `self.InputNumber` "")
  (`self.UpdateInputNumber` PC))

(event `self.TaskComplete`
  (params (PC :type "/Game/Werewolf_01/BP/Gameplay/BP_GameplayPlayerController Object Reference"))
  ;[1 0.1543 0.1244] タスクを完了したとき
  (`parent.TaskComplete` PC)
  (`/Engine/EditorBlueprintResources/StandardMacros.IsValid` PC
    (:`Is Valid`
      (`/Game/Werewolf_01/BP/Gameplay/BP_GameplayPlayerController.DisplayOK` PC self))))

(event `Delete`
  (params (PC :type "/Game/Werewolf_01/BP/Gameplay/BP_GameplayPlayerController Object Reference"))
  (bind _inputnumber (`self.InputNumber`))
  ;[1 1 1] 最後に入力した番号を削除する
  (`|ExecutionSequence`
    (:`then_0`
      (set `self.InputNumber` (`KismetStringLibrary.GetSubstring` _inputnumber 0 (- (`KismetStringLibrary.Len` _inputnumber) 1)))
      (`self.UpdateInputNumber` PC))
    (:`then_1`
      (`GameplayStatics.PlaySound2D` "/Game/Werewolf_01/Interface_And_Item_Sounds/Cues/Futuristic_Click_05_Cue.Futuristic_Click_05_Cue" 1.0 1.0 0.0 null null))))

(event `DisplayOK`
  (params (PC :type "/Game/Werewolf_01/BP/Gameplay/BP_GameplayPlayerController Object Reference"))
  ;[0.2026 0.2461 1] OKを表示
  (bind _asui_task_o2 (cast `/Game/Werewolf_01/UI/Task/UI_Task_O2` (`/Game/Werewolf_01/BP/Gameplay/BP_GameplayPlayerController.GetUI_Task` PC)))
  (`/Game/Werewolf_01/UI/Task/UI_Task_O2.SetInputNumber` _asui_task_o2 "OK"))

(fn `UserConstructionScript`
  (`parent.UserConstructionScript`))