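; BP_PutHandTaskManager is a task manager in the Werewolf game that completes once a hand is placed on every one of its put-hand tasks.
; When events are bound, it subscribes to each BP_PutHandTask's OnPutHand dispatcher.
; Each notification rechecks all tasks through an interface message and calls SetTaskComplete only if every task reports a hand placed.
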(event `self.BindEvent`
  ;[1 1 1] イベントをバインド
  (`parent.BindEvent`)
  ;[1 1 1] タスクに手を置いたときのイベントをバインド
  (for _array_element (`self.GetTasks`)
    (bind _asbp_put_hand_task (cast `/Game/Werewolf_01/BP/Task/BP_PutHandTask` _array_element))
    (add `/Game/Werewolf_01/BP/Task/BP_PutHandTask.OnPutHand` _asbp_put_hand_task (delegate `OnPutHand`))))

(event `OnPutHand`
  (params (IsPut :type Boolean))
  ;[1 1 1] タスクに手を置いたとき
  (bind _completed (`self.Get Is Tasks Complete`))
  (if _completed
    (`self.SetTaskComplete`)))

(fn `Get Is Tasks Complete`
  (returns (Completed :type Boolean))
  (for _array_element (`self.GetTasks`)
    (bind _isput (message `/Game/Werewolf_01/BP/BP_WerewolfInterface.WW_GetIsPutHand` _array_element))
    (if (not _isput)
      (return false) ; 手を置いてないタスクがあれば未完了
    ))
  (return true) ; 全てのタスクに手を置いていれば完了
)

(fn `UserConstructionScript`
  (`parent.UserConstructionScript`))