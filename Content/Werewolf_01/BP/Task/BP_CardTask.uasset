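; Card-swipe task where the player inserts a card into a reader and drags it across at the right speed.
; Touch drags project the cursor onto the reader's plane, clamped to the slide line.
; Tick times the swipe until it passes halfway; releasing near the end completes the task if that time is within tolerance, otherwise fails as too fast or slow.
; Timelines animate insertion and resets, with text and red/green lamps showing status.
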(event `self.ReceiveBeginPlay`
  (bind _cardbox (`self.CardBox`))
  (`parent.ReceiveBeginPlay`)
  ;[1 1 1] カードの初期の位置と回転を保存
  (set `self.InitialCardLocation` (`SceneComponent.K2_GetComponentLocation` _cardbox))
  (set `self.InitialCardRotation` (`SceneComponent.K2_GetComponentRotation` _cardbox)))

(event `self.ReceiveTick`
  (params (DeltaSeconds :type "Float (single-precision)"))
  ;[1 0 0] Tick
  (`parent.ReceiveTick` DeltaSeconds)
  (if (`self.isGrab`)
    (if (not (`self.isReadSuccess`))
      (set `self.slidedTime` (+ (`self.slidedTime`) DeltaSeconds)) ; カードをスライドしている間の時間を保存
    )))

(event `checkSlide`
  ;[1 1 1] カードの読み込みに成功したかを確認
  (if (not (`self.isReadSuccess`))
    (if (> (`self.SlidePercent`) 0.5)
      (set `self.isReadSuccess` true)
      (`GameplayStatics.PlaySound2D` "/Game/Werewolf_01/Sound/CardSwipe.CardSwipe" 1.0 1.0 0.0 null null))))

(event `EndSlide`
  (params (PC :type "/Game/Werewolf_01/BP/Gameplay/BP_GameplayPlayerController Object Reference"))
  (bind _slidedtime (`self.slidedTime`))
  (bind _slidespeed (`self.slideSpeed`))
  ;[1 1 1] カードのスライドを終了する
  (set `self.isGrab` false)
  (if (`KismetMathLibrary.NearlyEqual_FloatFloat` (`self.SlidePercent`) 1.0 0.1)
    (if (`KismetMathLibrary.NearlyEqual_FloatFloat` _slidedtime _slidespeed (`self.speedTolerance`))
      (`self.SetText` "ACCEPTED. THANK YOU.")
      (`self.SetGreenRampOn` true)
      (`self.ReturnToStartPoint`)
      (`/Engine/EditorBlueprintResources/StandardMacros.IsValid` PC
        (:`Is Valid`
          (`/Game/Werewolf_01/BP/Gameplay/BP_GameplayPlayerController.TaskComplete` PC)))
      (else
        (`|ExecutionSequence`
          (:`then_0`
            (`self.TaskFailPerPlayer`))
          (:`then_1`
            (if (> _slidedtime _slidespeed)
              (`self.SetText` "TOO SLOW. TRY AGAIN.")
              (else
                (`self.SetText` "TOO FAST. TRY AGAIN.")))))))
    (else
      (`self.Return`))))

(event `SetCardLocation`
  (params (Location :type "Vector Structure"))
  (bind _location (`self.Get Insert Card Location`))
  ;[1 1 1] カードの位置をセット
  (`SceneComponent.K2_SetWorldLocation` (`self.CardBox`) (+ _location (`KismetMathLibrary.Vector_ClampSizeMax` (- (`KismetMathLibrary.FindClosestPointOnLine` Location _location (`self.GetSlideDirection`)) _location) (/ (`self.slideLength`) 2.0))) false false)
  (`self.checkSlide`))

(event `Return`
  ;[1 1 1] カードを現在の地点から開始地点まで補完させる
  (set `self.startPercent` (`self.SlidePercent`))
  (bind (_direction _alpha) (`Timeline|TL_Return` :!via `PlayFromStart`)
    (:`Update`
      (`self.SetSlidePercent` (`KismetMathLibrary.Lerp` (`self.startPercent`) 0.0 _alpha)))
    (:`Finished`
      (`KismetSystemLibrary.Delay` 1.0)
      (`self.SetText` "PLEASE SWIPE CARD")
      (`self.SetGreenRampOn` true)
      (`self.SetRedRampOn` false))))

(event `ReturnToStartPoint`
  (bind _cardbox (`self.CardBox`))
  ;[1 1 1] カードをスライドの開始地点へ戻す
  (`TimelineComponent.Stop` (`self.TL_Return`))
  (set `self.cardRotation` (`SceneComponent.K2_GetComponentRotation` (`self.CardBox`)))
  (set `self.cardLocation` (`SceneComponent.K2_GetComponentLocation` (`self.CardBox`)))
  (bind (_direction _alpha) (`Timeline|TL_ReturnStartPoint` :!via `PlayFromStart`)
    (:`Update`
      (`SceneComponent.K2_SetWorldLocation` _cardbox (`KismetMathLibrary.VLerp` (`self.cardLocation`) (`self.InitialCardLocation`) _alpha) false false)
      (`SceneComponent.K2_SetWorldRotation` _cardbox (`KismetMathLibrary.RLerp` (`self.cardRotation`) (`self.InitialCardRotation`) _alpha true) false false))
    (:`Finished`
      (`self.SetGreenRampOn` false)
      (`self.SetRedRampOn` false)
      (set `self.isInsert` false))))

(event `/Game/Werewolf_01/BP/BP_TouchInterface.TCH_Move`
  (params (PC :type "/Game/Werewolf_01/BP/Gameplay/BP_GameplayPlayerController Object Reference") (Location :type "Vector Structure"))
  (bind (_worldlocation _worlddirection _returnvalue) (`PlayerController.DeprojectMousePositionToWorld` PC))
  (bind (_t _intersection _returnvalue_2) (`KismetMathLibrary.LinePlaneIntersection_OriginNormal` _worldlocation (+ _worldlocation (* _worlddirection 1000.0)) (`self.Get Insert Card Location`) (`self.GetActorForwardVector`)))
  ;[1 1 1] カードをスライドする
  (`/Engine/EditorBlueprintResources/StandardMacros.IsValid` PC
    (:`Is Valid`
      (if _returnvalue
        (if _returnvalue_2
          (if (and (not (`self.isCompleted`)) (`self.isInsert`) (not (`TimelineComponent.IsPlaying` (`self.TL_Return`))) (`self.isGrab`))
            (`self.SetCardLocation` _intersection)
            (else
              (`KismetSystemLibrary.PrintString` "Slide Card Failed" true true (struct :`R` 1.0 :`A` 1.0) :!label _label)))
          (else
            (goto _label)))
        (else
          (goto _label))))
    (:`Is Not Valid`
      (goto _label))))

(event `self.OnOpenPerPlayerTask`
  (params (PC :type "/Game/Werewolf_01/BP/Gameplay/BP_GameplayPlayerController Object Reference"))
  ;[1 1 1] タスクを開いたとき
  (`parent.OnOpenPerPlayerTask` PC)
  (set `self.isReadSuccess` false)
  (set `self.slidedTime` 0.0)
  (`self.SetText` "PLEASE INSERT CARD")
  (`TimelineComponent.SetPlayRate` (`self.TL_ReturnStartPoint`) (/ 1.0 (`self.animSpeed`)))
  (`TimelineComponent.SetPlayRate` (`self.TL_Insert`) (/ 1.0 (`self.animSpeed`)))
  (`TimelineComponent.SetPlayRate` (`self.TL_Return`) (/ 1.0 (`self.animSpeed`))))

(event `StartSlide`
  ;[1 1 1] カードのスライドを開始する
  (set `self.isGrab` true)
  (set `self.isReadSuccess` false)
  (set `self.slidedTime` 0.0)
  (`self.SetGreenRampOn` false))

(event `InsertCard`
  (bind _cardbox (`self.CardBox`))
  ;[1 1 1] カードを挿入する
  (if (not (`TimelineComponent.IsPlaying` (`self.TL_Insert`)))
    (`|ExecutionSequence`
      (:`then_0`
        (bind _location (`self.PercentToLocation` 0.0))
        (bind (_direction _alpha) (`Timeline|TL_Insert` :!via `PlayFromStart`)
          (:`Update`
            (`SceneComponent.K2_SetWorldLocation` _cardbox (`KismetMathLibrary.VLerp` (`self.InitialCardLocation`) _location _alpha) false false)
            (`SceneComponent.K2_SetWorldRotation` _cardbox (`KismetMathLibrary.RLerp` (`self.InitialCardRotation`) (`self.GetInsertCardRotation`) _alpha true) false false))
          (:`Finished`
            (`self.SetText` "PLEASE SWIPE CARD")
            (`self.SetGreenRampOn` true)
            (set `self.isInsert` true))))
      (:`then_1`
        (`GameplayStatics.PlaySound2D` "/Game/Werewolf_01/Sound/CardSwipe.CardSwipe" 1.0 1.0 0.0 null null)))))

(event `/Game/Werewolf_01/BP/BP_TouchInterface.TCH_Presse`
  (params (PC :type "/Game/Werewolf_01/BP/Gameplay/BP_GameplayPlayerController Object Reference") (TouchComp :type "SceneComponent Object Reference"))
  ;[1 1 1] カードを掴み始める
  (if (and (not (`TimelineComponent.IsPlaying` (`self.TL_Return`))) (== TouchComp (`self.CardBox`)))
    (if (`self.isInsert`)
      (`self.StartSlide`)
      (else
        (`self.InsertCard`)))
    (else
      (set `self.isGrab` false))))

(event `self.OnClose`
  (params (PC :type "/Game/Werewolf_01/BP/Gameplay/BP_GameplayPlayerController Object Reference"))
  (`|ExecutionSequence`
    (:`then_0`
      (if (`/Game/Werewolf_01/BP/Task/PlayerTaskManagerComponent.IsContainsRemainingTask` (`/Game/Werewolf_01/BP/Gameplay/BP_GameplayPlayerController.PlayerTaskManagerComponent` PC) self)
        (`self.OnClosePerPlayerTask` PC)))
    (:`then_1`
      (`parent.OnClose` PC))))

(event `/Game/Werewolf_01/BP/BP_TouchInterface.TCH_Release`
  (params (PC :type "/Game/Werewolf_01/BP/Gameplay/BP_GameplayPlayerController Object Reference") (Actor :type "Actor Object Reference") (Comp :type "SceneComponent Object Reference"))
  ;[1 1 1] カードのスライドを終了する
  (if (and (not (`self.isCompleted`)) (`self.isInsert`))
    (`self.EndSlide` PC)))

(event `self.OnClosePerPlayerTask`
  (params (PC :type "/Game/Werewolf_01/BP/Gameplay/BP_GameplayPlayerController Object Reference"))
  ;[1 1 1] タスクを閉じたとき
  (`parent.OnClosePerPlayerTask` PC)
  (if (`self.isInsert`)
    (`self.ReturnToStartPoint`)))

(event `self.TaskFailPerPlayer`
  ;[1 1 1] カードの読み取りに失敗したとき、ランプを赤に点灯させ、カードをスライドの開始地点へ戻す
  (`parent.TaskFailPerPlayer`)
  (`self.Return`)
  (`self.SetRedRampOn` true))

(fn `Get Insert Card Location`
  (returns (Location :type "Vector Structure"))
  (return (`KismetMathLibrary.TransformLocation` (`self.GetTransform`) (.location (`self.InsertCardTransform`)))))

(fn `GetInsertCardRotation`
  (returns (Rotation :type "Rotator Structure"))
  (return (.rotation (`self.InsertCardTransform`))))

(fn `GetSlideDirection`
  (returns (ReturnValue :type "Vector Structure"))
  (return (`self.GetActorRightVector`)))

(fn `PercentToLocation`
  (params (percent :type "Float (double-precision)"))
  (returns (location :type "Vector Structure"))
  (bind _slidelength (`self.slideLength`))
  (return (+ (* (`self.GetSlideDirection`) (+ (/ _slidelength 2.0) (* (* percent _slidelength) -1.0))) (`self.Get Insert Card Location`))))

(fn `SetGreenRampOn`
  (params (isOn :type Boolean))
  (bind _m_greenramp (`self.M_GreenRamp`)
    (:`then`
      (`MaterialInstanceDynamic.SetVectorParameterValue` _m_greenramp "Color" (`KismetMathLibrary.SelectColor` (struct :`R` 0.003319 :`G` 1.0 :`A` 1.0) (struct :`G` 0.026042 :`B` 4.9e-05 :`A` 1.0) isOn)))
    (:`else`)))

(fn `SetRedRampOn`
  (params (isOn :type Boolean))
  (bind _m_redramp (`self.M_RedRamp`)
    (:`then`
      (`MaterialInstanceDynamic.SetVectorParameterValue` _m_redramp "Color" (`KismetMathLibrary.SelectColor` (struct :`R` 1.0 :`G` 0.007764 :`A` 1.0) (struct :`R` 0.03125 :`G` 0.000259 :`A` 1.0) isOn)))
    (:`else`)))

(fn `SetSlidePercent`
  (params (percent :type "Float (double-precision)"))
  (bind _location (`self.PercentToLocation` percent))
  (`SceneComponent.K2_SetWorldLocation` (`self.CardBox`) _location false false))

(fn `SetText`
  (params (Value :type Text))
  (`TextRenderComponent.K2_SetText` (`self.TextRender`) Value))

(fn `SlidePercent`
  (returns (ReturnValue :type "Float (double-precision)"))
  (bind _returnvalue (/ (`self.slideLength`) 2.0))
  (return (`KismetMathLibrary.FClamp` (- 1.0 (`KismetMathLibrary.NormalizeToRange` (.y (`SceneComponent.RelativeLocation` (`self.CardBox`))) (* _returnvalue -1.0) _returnvalue)))))

(fn `UserConstructionScript`
  (`parent.UserConstructionScript`)
  (`|ExecutionSequence`
    (:`then_1`
      (`|ExecutionSequence`
        (:`then_0`
          (bind _returnvalue (`KismetMaterialLibrary.CreateDynamicMaterialInstance` "/Game/Werewolf_01/Materials/M_Ramp.M_Ramp"))
          (bind _output_get (set `self.M_GreenRamp` _returnvalue))
          (`PrimitiveComponent.SetMaterial` (`self.GreenRamp`) 0 _output_get))
        (:`then_1`
          (`self.SetGreenRampOn` false))))
    (:`then_2`
      (`|ExecutionSequence`
        (:`then_0`
          (bind _returnvalue_2 (`KismetMaterialLibrary.CreateDynamicMaterialInstance` "/Game/Werewolf_01/Materials/M_Ramp.M_Ramp"))
          (bind _output_get_2 (set `self.M_RedRamp` _returnvalue_2))
          (`PrimitiveComponent.SetMaterial` (`self.RedRamp`) 0 _output_get_2))
        (:`then_1`
          (`self.SetRedRampOn` false))))
    (:`then_3`
      (if (`self.PreviewInsertCard`)
        (`self.SetSlidePercent` (`self.PreviewSlidePercent`))
        (`SceneComponent.K2_SetWorldRotation` (`self.CardBox`) (`self.GetInsertCardRotation`) false false)
        (else
          (`SceneComponent.K2_SetRelativeTransform` (`self.CardBox`) (`self.InitialCardTransform`) false false))))))