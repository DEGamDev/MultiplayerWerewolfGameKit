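; Per-player memory task in which the player repeats a random button sequence that grows by one step each round.
; SetPattern builds the sequence, and chained timers light it step by step on UI_PatternButtonTask with input locked during playback.
; EnterNumber checks each press: a mistake fails and regenerates the pattern, while completing the full length calls TaskComplete.
; An inactivity timer restarts between presses, and button tones rise in pitch with button number.
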(event `self.OnOpenPerPlayerTask`
  (params (PC :type "/Game/Werewolf_01/BP/Gameplay/BP_GameplayPlayerController Object Reference"))
  ;[1 0.2083 0.2083] タスクを開いたとき
  (`parent.OnOpenPerPlayerTask` PC)
  (`self.SetPattern` PC))

(event `/Game/Werewolf_01/BP/BP_WerewolfInterface.WW Enter Number_A`
  (params (Number :type Integer) (PC :type "/Game/Werewolf_01/BP/Gameplay/BP_GameplayPlayerController Object Reference"))
  ;[0.2026 0.2461 1] 番号を入力する
  (`self.EnterNumber` Number PC))

(event `SetPattern`
  (params (PC :type "/Game/Werewolf_01/BP/Gameplay/BP_GameplayPlayerController Object Reference"))
  ;[0.2026 0.2461 1] パターンをセット
  (set `self.PC` PC)
  (`|ExecutionSequence`
    (:`then_0`
      (`|ExecutionSequence`
        (:`then_0`
          (`self.InitializePerPlayerTask`)
          (`self.UpdateInputCount` PC)
          (`self.UpdatePatternCount` PC)
          (`self.SetCanInput` false))
        (:`then_1`
          (for _ (range (`self.PatternLength`))
            (`KismetArrayLibrary.Array_Add` (`self.pattern`) (`KismetMathLibrary.RandomInteger` (`self.BUTTON_COUNT`)))))))
    (:`then_1`
      (`self.PlayNextPattern`))))

(event `EnterNumber`
  (params (Number :type Integer) (PC :type "/Game/Werewolf_01/BP/Gameplay/BP_GameplayPlayerController Object Reference"))
  ;[0.2026 0.2461 1] 番号を入力する
  (if (`self.canInput`)
    (`|ExecutionSequence`
      (:`then_0`
        (`self.ClearResetTimer`)
        (`KismetArrayLibrary.Array_Add` (`self.CureentEnterNumber`) Number)
        (`self.UpdateInputCount` PC))
      (:`then_1`
        (bind _asui_pattern_button_task (cast `/Game/Werewolf_01/UI/Task/UI_PatternButtonTask` (`/Game/Werewolf_01/BP/Gameplay/BP_GameplayPlayerController.GetUI_Task` PC)))
        (`/Game/Werewolf_01/UI/Task/UI_PatternButtonTask.LightInputButton` _asui_pattern_button_task Number))
      (:`then_2`
        (if (== (`|GetArrayItem` (`self.pattern`) (`KismetArrayLibrary.Array_LastIndex` (`self.CureentEnterNumber`))) (`|GetArrayItem` (`self.CureentEnterNumber`) (`KismetArrayLibrary.Array_LastIndex` (`self.CureentEnterNumber`))))
          (if (== (`KismetArrayLibrary.Array_Length` (`self.CureentEnterNumber`)) (`self.currentPatternCount`))
            (`self.ConfirmInput`)
            (else
              (`self.SetResetTimer`)))
          (else
            (`self.TaskFailPerPlayer`))))
      (:`then_3`
        (`self.PlayEnteredSound` Number)))))

(event `ClearResetTimer`
  ;[0.2026 0.2461 1] リセットタイマーを削除する
  (`KismetSystemLibrary.K2_ClearAndInvalidateTimerHandle` (`self.resetPatternTimer`)))

(event `SetResetTimer`
  ;[0.2026 0.2461 1] リセットタイマーをセットする
  (`|ExecutionSequence`
    (:`then_0`
      (`self.ClearResetTimer`))
    (:`then_1`
      (bind _returnvalue (`KismetSystemLibrary.K2_SetTimerDelegate` (`|CreateDelegate` :!event `ResetPattern`) (`self.continueDuration`)))
      (set `self.resetPatternTimer` _returnvalue)
      (`self.SetCanInput` true))))

(event `SetCanInput`
  (params (canInput :type Boolean))
  ;[0.2026 0.2461 1] 入力可能かをセット
  (bind _output_get (set `self.canInput` canInput))
  (bind _pc (`self.PC`)
    (:`then`
      (bind _asui_pattern_button_task (cast `/Game/Werewolf_01/UI/Task/UI_PatternButtonTask` (`/Game/Werewolf_01/BP/Gameplay/BP_GameplayPlayerController.GetUI_Task` _pc)))
      (`/Game/Werewolf_01/UI/Task/UI_PatternButtonTask.SetInputEnable` _asui_pattern_button_task _output_get))
    (:`else`)))

(event `PlayNextPattern`
  ;[0.2026 0.2461 1] 次のパターンを再生
  (`|ExecutionSequence`
    (:`then_0`
      (set `self.currentPatternCount` (+ (`self.currentPatternCount`) 1)))
    (:`then_1`
      (`self.StartStreamPattern` (`self.PC`)))))

(event `UpdateInputCount`
  (params (PC :type "/Game/Werewolf_01/BP/Gameplay/BP_GameplayPlayerController Object Reference"))
  ;[0.2728 0.37 1] 入力数を更新
  (`/Engine/EditorBlueprintResources/StandardMacros.IsValid` PC
    (:`Is Valid`
      (bind _asui_pattern_button_task (cast `/Game/Werewolf_01/UI/Task/UI_PatternButtonTask` (`/Game/Werewolf_01/BP/Gameplay/BP_GameplayPlayerController.GetUI_Task` PC)))
      (`/Game/Werewolf_01/UI/Task/UI_PatternButtonTask.SetInputEnterCount` _asui_pattern_button_task (`self.GetEnterdNumber`)))))

(event `self.TaskFailPerPlayer`
  ;[0.2026 0.2461 1] タスクを失敗したとき、パターンをリセットする
  (`parent.TaskFailPerPlayer`)
  (`self.ResetPattern`))

(event `UpdatePatternCount`
  (params (PC :type "/Game/Werewolf_01/BP/Gameplay/BP_GameplayPlayerController Object Reference"))
  ;[0.2026 0.2461 1] パターンのカウントを更新
  (`/Engine/EditorBlueprintResources/StandardMacros.IsValid` PC
    (:`Is Valid`
      (bind _asui_pattern_button_task (cast `/Game/Werewolf_01/UI/Task/UI_PatternButtonTask` (`/Game/Werewolf_01/BP/Gameplay/BP_GameplayPlayerController.GetUI_Task` PC)))
      (`/Game/Werewolf_01/UI/Task/UI_PatternButtonTask.SetPatternCount` _asui_pattern_button_task (`self.currentPatternCount`)))))

(event `ResetPattern`
  (bind _pc (`self.PC`))
  ;[0.2026 0.2461 1] パターンをリセットする
  (`self.InitializePerPlayerTask`)
  (`self.SetPattern` _pc)
  (`self.UpdateInputCount` _pc))

(event `StartStreamPattern`
  (params (PC :type "/Game/Werewolf_01/BP/Gameplay/BP_GameplayPlayerController Object Reference"))
  (bind _pc (`self.PC`))
  ;[0.2026 0.2461 1] パターンの再生を開始する
  (`|ExecutionSequence`
    (:`then_0`
      (`self.SetCanInput` false)
      (set `self.currentStreamCount` 0)
      (`KismetSystemLibrary.Delay` 0.3)
      (`KismetArrayLibrary.Array_Clear` (`self.CureentEnterNumber`))
      (`self.UpdateInputCount` _pc))
    (:`then_1`
      (`KismetSystemLibrary.Delay` (`self.StreamWaitTime`))
      (bind _returnvalue (`KismetSystemLibrary.K2_SetTimerDelegate` (`|CreateDelegate` :!event `LightButton`) (`self.StreamInterval`)))
      (set `self.LightButtonTimer` _returnvalue)
      (`self.UpdatePatternCount` _pc))))

(event `LightButton`
  ;[0.2026 0.2461 1] ボタンを点灯させる
  (`self.PC`
    (:`then`
      (`|ExecutionSequence`
        (:`then_0`
          (set `self.currentStreamCount` (+ (`self.currentStreamCount`) 1)))
        (:`then_1`
          (if (!= (`self.currentPatternCount`) (`self.currentStreamCount`))
            (bind _returnvalue (`KismetSystemLibrary.K2_SetTimerDelegate` (`|CreateDelegate` :!event `LightButton`) (`self.StreamInterval`)))
            (set `self.LightButtonTimer` _returnvalue)
            (else
              (`self.SetResetTimer`))))
        (:`then_2`
          (bind _pc (`self.PC`)
            (:`then`
              (bind _asui_pattern_button_task (cast `/Game/Werewolf_01/UI/Task/UI_PatternButtonTask` (`/Game/Werewolf_01/BP/Gameplay/BP_GameplayPlayerController.GetUI_Task` _pc)))
              (`/Game/Werewolf_01/UI/Task/UI_PatternButtonTask.LightButton` _asui_pattern_button_task (`|GetArrayItem` (`self.pattern`) (- (`self.currentStreamCount`) 1))))
            (:`else`)))
        (:`then_3`
          (`self.UpdateInputCount` (`self.PC`))
          (`self.PlayEnteredSound` (`|GetArrayItem` (`self.pattern`) (- (`self.currentStreamCount`) 1))))))
    (:`else`)))

(event `ConfirmInput`
  ;[0.2026 0.2461 1] 入力を決定する
  (if (`self.IsSuccessCurrentPattern`)
    (if (== (`self.currentPatternCount`) (`self.PatternLength`))
      (bind _pc (`self.PC`)
        (:`then`
          (`/Game/Werewolf_01/BP/Gameplay/BP_GameplayPlayerController.TaskComplete` _pc))
        (:`else`))
      (else
        (`self.PlayNextPattern`)))
    (else
      (`self.ResetPattern`))))

(event `self.InitializePerPlayerTask`
  ;[0.2026 0.2461 1] 非共有タスクを初期化
  (`parent.InitializePerPlayerTask`)
  (`KismetArrayLibrary.Array_Clear` (`self.pattern`))
  (`KismetArrayLibrary.Array_Clear` (`self.CureentEnterNumber`))
  (set `self.currentPatternCount` 0)
  (`KismetArrayLibrary.Array_Clear` (`self.CureentEnterNumber`))
  (set `self.currentStreamCount` 0)
  (`self.ClearResetTimer`)
  (`KismetSystemLibrary.K2_ClearAndInvalidateTimerHandle` (`self.LightButtonTimer`)))

(event `PlayEnteredSound`
  (params (Number :type Integer))
  ;[1 1 1] 入力したときの音を再生
  (`GameplayStatics.PlaySound2D` "/Game/Werewolf_01/Sound/Button.Button" 3.0 (`KismetMathLibrary.Lerp` 1.0 2.0 (/ (`KismetMathLibrary.Conv_IntToDouble` Number) (`KismetMathLibrary.Conv_IntToDouble` (`self.BUTTON_COUNT`)))) 0.0 null null))

(event `self.OnClosePerPlayerTask`
  (params (PC :type "/Game/Werewolf_01/BP/Gameplay/BP_GameplayPlayerController Object Reference"))
  ;[1 1 1] タスクを閉じたとき、プレイヤーの参照を削除
  (`parent.OnClosePerPlayerTask` PC)
  (set `self.PC` null))

(fn `BUTTON_COUNT`
  (returns (Count :type Integer))
  (return (`self.ButtonCount`)))

(fn `GetEnterdNumber`
  (returns (ReturnValue :type Integer))
  (return (`KismetArrayLibrary.Array_Length` (`self.CureentEnterNumber`))))

(fn `IsSuccessCurrentPattern`
  (returns (ReturnValue :type Boolean))
  (locals (Enter_l :type "Array of Integer") (pattern_l :type "Array of Integer"))
  (`|ExecutionSequence`
    (:`then_0`
      (for _index (range (`self.currentPatternCount`))
        (`|ExecutionSequence`
          (:`then_0`
            (`KismetArrayLibrary.Array_Add` (`local.Enter_l`) (`|GetArrayItem` (`self.CureentEnterNumber`) _index)))
          (:`then_1`
            (`KismetArrayLibrary.Array_Add` (`local.pattern_l`) (`|GetArrayItem` (`self.pattern`) _index))))))
    (:`then_2`
      (return (`KismetArrayLibrary.Array_Identical` (`local.Enter_l`) (`local.pattern_l`))))))

(fn `UserConstructionScript`
  (`parent.UserConstructionScript`))