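; Task Blueprint for a Werewolf game minigame where the player enters numbers 1 to 10 in ascending order.
; Each entered number is checked against CurrentNumber plus one, and a match advances the count and lights that button through a player controller message.
; Reaching ten sends the task-complete message to the controller.
; A wrong number resets progress, plays a fail sound, and clears the task UI buttons with a fail animation.
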(event `/Game/Werewolf_01/BP/BP_WerewolfInterface.WW Enter Number_A`
  (params (Number :type Integer) (PC :type "/Game/Werewolf_01/BP/Gameplay/BP_GameplayPlayerController Object Reference"))
  ;[1 1 1] 数字を入力する
  (`self.EnterNumber` Number PC))

(event `EnterNumber`
  (params (number :type Integer) (PC :type "/Game/Werewolf_01/BP/Gameplay/BP_GameplayPlayerController Object Reference"))
  ;[1 1 1] 数字を入力する
  (`KismetSystemLibrary.PrintString` (`KismetStringLibrary.Conv_IntToString` number))
  (if (== number (+ (`self.currentNumber`) 1))
    (`|ExecutionSequence`
      (:`then_0`
        (bind _output_get (set `self.currentNumber` number))
        (message `/Game/Werewolf_01/BP/BP_WerewolfInterface.WW_SetIsOnOfNumberButton` PC _output_get true))
      (:`then_1`
        (if (== (`self.currentNumber`) 10)
          (message `/Game/Werewolf_01/BP/BP_WerewolfInterface.WW_TaskComplete` PC PC))))
    (else
      (`|ExecutionSequence`
        (:`then_0`
          (set `self.currentNumber` 0)
          (`self.PlayFailSound`))
        (:`then_1`
          (bind _asui_numerical_orderr_input_task (cast `/Game/Werewolf_01/UI/Task/UI_NumericalOrderrInputTask` (`/Game/Werewolf_01/BP/Gameplay/BP_GameplayPlayerController.GetUI_Task` PC)))
          (`/Game/Werewolf_01/UI/Task/UI_NumericalOrderrInputTask.SetAllIsOn` _asui_numerical_orderr_input_task false)
          (`/Game/Werewolf_01/UI/Task/UI_NumericalOrderrInputTask.PlayFailAnim` _asui_numerical_orderr_input_task))))))

(event `PlayFailSound`
  (`GameplayStatics.PlaySound2D` "/Engine/EditorSounds/Notifications/CompileFailed.CompileFailed" 1.0 1.0 0.0 null null)
  (`KismetSystemLibrary.PrintString` "Fail"))

(fn `UserConstructionScript`
  (`parent.UserConstructionScript`))