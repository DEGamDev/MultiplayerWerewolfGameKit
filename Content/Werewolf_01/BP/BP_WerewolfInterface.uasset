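; BP_WerewolfInterface is the shared Blueprint Interface for a werewolf-versus-villager social deduction game, holding only message signatures with empty or default returns.
; It covers player spawning, roles, input, tasks and emergency sabotage, kills and body reports, meetings with voting and ejection, hatch travel, cameras and cooldowns.
; One contract spans characters, controllers, task actors, game settings and UI, with identity queries such as IsWolf, IsTask and IsHatch available on any implementer.
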(fn `WW Enter Number_A`
  (params (Number :type Integer) (PC :type "/Game/Werewolf_01/BP/Gameplay/BP_GameplayPlayerController Object Reference")))

(fn `WW_AddAliveVillagerCount`
  (params (Value :type Integer)))

(fn `WW_AddAliveWolfCount`
  (params (Count :type Integer)))

(fn `WW_AddHatchButton`
  (params (Hatch :type "Actor Object Reference") (Angle :type "Float (double-precision)")))

(fn `WW_AddToVotedByPlayerIndex`
  (params (Index :type Integer)))

(fn `WW_AddVoteButton`
  (params (Name :type String) (Index :type Integer) (Color :type "LinearColor Structure") (IsDead :type Boolean) (IsReportedToPlayer :type Boolean)))

(fn `WW_AddVotedFromPlayerIcon`
  (params (Color :type "LinearColor Structure") (Index :type Integer)))

(fn `WW_ApplyGameSettings`
  (params (GameSettings :type "Actor Object Reference")))

(fn `WW_ClearCooldown`)

(fn `WW_ClearEmergencyTask`)

(fn `WW_ClearEmergencyTimer`)

(fn `WW_ClearInputNumbers`)

(fn `WW_ClearKillCoolDown`)

(fn `WW_ClearSabotageCooldown`)

(fn `WW_ClearVotedToPlayerIndexes`)

(fn `WW_CloseHatch`
  (params (PC :type "/Game/Werewolf_01/BP/Gameplay/BP_GameplayPlayerController Object Reference")))

(fn `WW_CloseTaskUI`)

(fn `WW_Dead`)

(fn `WW_DecrementAliveVillagersCount`)

(fn `WW_DisableGameInput`)

(fn `WW_DisableInput`)

(fn `WW_DisableUIInput`)

(fn `WW_EjectPlayer`)

(fn `WW_EnableGameInput`)

(fn `WW_EnableSetTask`)

(fn `WW_EnableUIInput`)

(fn `WW_EndCurrentAction`)

(fn `WW_EnterToHatch`)

(fn `WW_GameFinishCheck`)

(fn `WW_GetAllCharacters`
  (returns (Characters :type "Array of Actor Object Reference"))
  (return))

(fn `WW_GetAllPC`
  (returns (PC :type "Array of Actor Object Reference"))
  (return))

(fn `WW_GetAllPlayersCount`
  (returns (Count :type Integer))
  (return 0))

(fn `WW_GetAllWolfs`
  (returns (Wolfs :type "Array of Actor Object Reference"))
  (return))

(fn `WW_GetCanMovingHatches`
  (returns (Hatches :type "Array of Actor Object Reference"))
  (return))

(fn `WW_GetCanUseEmergencyButton`
  (params (UsedCount :type Integer))
  (returns (Can :type Boolean))
  (return false))

(fn `WW_GetCharacterType`
  (returns (CharacterType :type "/Game/Werewolf_01/Enum/e_CharacterType Enum"))
  (return "NewEnumerator1"))

(fn `WW_GetCompletedTaskCount`
  (returns (Count :type Integer))
  (return 0))

(fn `WW_GetEmergencyButton`
  (returns (EmergencyButton :type "Actor Object Reference"))
  (return null))

(fn `WW_GetEmergencyMeetingCoolTime`
  (returns (Time :type Integer))
  (return 0))

(fn `WW_GetEmergencyTasks`
  (returns (Tasks :type "Array of Actor Object Reference"))
  (return))

(fn `WW_GetGameSettings`
  (returns (GameSettings :type "Actor Object Reference"))
  (return null))

(fn `WW_GetIsCharacterCapsule`
  (params (Comp :type "SceneComponent Object Reference"))
  (returns (NewParam :type Boolean))
  (return false))

(fn `WW_GetIsDead`
  (returns (IsDead :type Boolean))
  (return false))

(fn `WW_GetIsEmergencyTaskCoolDown`
  (returns (IsCoolDown :type Boolean))
  (return false))

(fn `WW_GetIsEnableTask`
  (returns (IsEnable :type Boolean))
  (return false))

(fn `WW_GetIsGameFinished`
  (returns (IsGameFinished :type Boolean))
  (return false))

(fn `WW_GetIsInGame`
  (returns (IsInGame :type Boolean))
  (return false))

(fn `WW_GetIsInHatch`
  (returns (IsIn :type Boolean))
  (return false))

(fn `WW_GetIsInMeeting`
  (returns (In :type Boolean))
  (return false))

(fn `WW_GetIsInVotingTime`
  (returns (In :type Boolean))
  (return false))

(fn `WW_GetIsKillCoolDown`
  (returns (CoolDown :type Boolean))
  (return false))

(fn `WW_GetIsKilling`
  (returns (Killing :type Boolean))
  (return false))

(fn `WW_GetIsPlayerStart`
  (returns (NewParam :type Boolean))
  (return false))

(fn `WW_GetIsPutHand`
  (returns (IsPut :type Boolean))
  (return false))

(fn `WW_GetIsSabotageCoolDown`
  (returns (IsCoolDown :type Boolean))
  (return false))

(fn `WW_GetIsTaskManager`
  (returns (NewParam :type Boolean))
  (return false))

(fn `WW_GetIsUseCamera`
  (returns (Use :type Boolean))
  (return false))

(fn `WW_GetIsValidEmergencyTimer`
  (returns (IsValid :type Boolean))
  (return false))

(fn `WW_GetIsVotedToPlayer`
  (returns (NewParam :type Boolean))
  (return false))

(fn `WW_GetKillCoolDownTime`
  (returns (Time :type Integer))
  (return 0))

(fn `WW_GetMovingSpeed`
  (returns (Speed :type "Float (double-precision)"))
  (return 0.0))

(fn `WW_GetOverlapHatch`
  (returns (Hatch :type "/Game/Werewolf_01/BP/Hatch/BP_Hatch Object Reference"))
  (return null))

(fn `WW_GetPCByIndex`
  (params (Index :type Integer))
  (returns (PC :type "Actor Object Reference"))
  (return null))

(fn `WW_GetPlayerColorByIndex`
  (params (Index :type Integer))
  (returns (Color :type "LinearColor Structure"))
  (return))

(fn `WW_GetPlayerIndex`
  (returns (Index :type Integer))
  (return 0))

(fn `WW_GetPlayerName`
  (returns (Name :type String))
  (return ""))

(fn `WW_GetPlayerStarts`
  (returns (PlayerStarts :type "Array of Actor Object Reference"))
  (return))

(fn `WW_GetReportTarget`
  (returns (ReportTarget :type "Actor Object Reference"))
  (return null))

(fn `WW_GetSabotageCooldownPercent`
  (returns (Percent :type "Float (double-precision)"))
  (return 0.0))

(fn `WW_GetTargetHatchAngle`)

(fn `WW_GetTask`
  (returns (Task :type "Actor Object Reference"))
  (return null))

(fn `WW_GetTaskManagers`
  (returns (TaskManagers :type "Array of Actor Object Reference"))
  (return))

(fn `WW_GetTaskUIClass`
  (returns (TaskUIClass :type "UserWidget Class Reference"))
  (return null))

(fn `WW_GetVotedFromPlayerCount`
  (returns (Count :type Integer))
  (return 0))

(fn `WW_GetVotedFromPlayerIndex`
  (returns (Index :type "Array of Integer"))
  (return))

(fn `WW_GetVoteTime`
  (returns (Time :type Integer))
  (return 0))

(fn `WW_Initialize`)

(fn `WW_InitializeCharacterColor`)

(fn `WW_InitializeGameplayUI`)

(fn `WW_IsCompleted`
  (returns (Completed :type Boolean))
  (return false))

(fn `WW_IsCompletedAllTask`
  (returns (IsCompleted :type Boolean))
  (return false))

(fn `WW_IsControlledCharacter`
  (returns (ReturnValue :type Boolean))
  (return false))

(fn `WW_IsEmergencyButton`
  (returns (NewParam :type Boolean))
  (return false))

(fn `WW_IsEmergencyTask`
  (returns (NewParam :type Boolean))
  (return false))

(fn `WW_IsGameSettings`
  (returns (ReturnValue :type Boolean))
  (return false))

(fn `WW_IsHatch`
  (returns (IsHatch :type Boolean))
  (return false))

(fn `WW_IsReportSphere`
  (params (Comp :type "PrimitiveComponent Object Reference"))
  (returns (NewParam :type Boolean))
  (return false))

(fn `WW_IsTask`
  (returns (NewParam :type Boolean))
  (return false))

(fn `WW_IsValidDeadBody`
  (returns (Valid :type Boolean))
  (return false))

(fn `WW_IsVillager`
  (returns (IsVillager :type Boolean))
  (return false))

(fn `WW_IsWolf`
  (returns (Wolf :type Boolean))
  (return false))

(fn `WW_Kill`)

(fn `WW_KilledFromWolf`)

(fn `WW_LeaveFromHatch`)

(fn `WW_LookUp`
  (params (Value :type "Float (double-precision)")))

(fn `WW_LosePlayer`)

(fn `WW_MoveForward`
  (params (Value :type "Float (double-precision)")))

(fn `WW_MoveRight`
  (params (Value :type "Float (double-precision)")))

(fn `WW_MoveToHatch`
  (params (Hatch :type "Actor Object Reference")))

(fn `WW_OnClose`)

(fn `WW_OnOpen`
  (params (PC :type "/Game/Werewolf_01/BP/Gameplay/BP_GameplayPlayerController Object Reference")))

(fn `WW_OpenHatch`
  (params (PC :type "/Game/Werewolf_01/BP/Gameplay/BP_GameplayPlayerController Object Reference")))

(fn `WW_OpenTask`)

(fn `WW_OpenTaskUI`
  (params (TaskUIClass :type "UserWidget Class Reference")))

(fn `WW_PlayEmergencyAnim`)

(fn `WW_PutHand`
  (params (PC :type "/Game/Werewolf_01/BP/Gameplay/BP_GameplayPlayerController Object Reference")))

(fn `WW_ReleaseHand`
  (params (PC :type "/Game/Werewolf_01/BP/Gameplay/BP_GameplayPlayerController Object Reference")))

(fn `WW_RemoveDeadBodyReportScreen`)

(fn `WW_RemoveDeadUI`)

(fn `WW_RemoveEjectResult`)

(fn `WW_RemoveEmergencyMeetingScreen`)

(fn `WW_RemoveEmergencyScreen`)

(fn `WW_RemoveInHatchScreen`)

(fn `WW_RemoveKillCooldown`)

(fn `WW_RemoveSabotageCooldown`)

(fn `WW_RemoveTaskUI`)

(fn `WW_RemoveVoteScreen`)

(fn `WW_ReturnToInitialLocation`)

(fn `WW_Sabotage`)

(fn `WW_SetActiveCharacterMovement`
  (params (IsActive :type Boolean)))

(fn `WW_SetAliveVillagersCount`
  (params (Count :type Integer)))

(fn `WW_SetAliveWolfCount`
  (params (Count :type Integer)))

(fn `WW_SetAllCharacterVisible`
  (params (Visible :type Boolean)))

(fn `WW_SetCharacterColor`
  (params (Color :type "LinearColor Structure")))

(fn `WW_SetCharacterIconColor`
  (params (Color :type "LinearColor Structure")))

(fn `WW_SetCharacterType`
  (params (CharacterType :type "/Game/Werewolf_01/Enum/e_CharacterType Enum" :default "NewEnumerator0")))

(fn `WW_SetCharacterVisible`
  (params (Visible :type Boolean)))

(fn `WW_SetCompletedTaskCount`
  (params (Count :type Integer))
  (return))

(fn `WW_SetCompletedTaskPercent`
  (params (Percent :type "Float (double-precision)")))

(fn `WW_SetConfirmButtonVisible`
  (params (Visible :type Boolean)))

(fn `WW_SetEmergencyTimer`
  (params (Time :type "Float (double-precision)")))

(fn `WW_SetHatchButtonAngle`
  (params (Angle :type "Float (double-precision)"))
  (return))

(fn `WW_SetIsCompleted`
  (params (NewParam :type Boolean)))

(fn `WW_SetIsDead`
  (params (IsDead :type Boolean) (Index :type Integer)))

(fn `WW_SetIsEnableCameraInput`
  (params (Enable :type Boolean)))

(fn `WW_SetIsEnableGameInput`
  (params (Enable :type Boolean)))

(fn `WW_SetIsInGame`
  (params (IsInGame :type Boolean))
  (return))

(fn `WW_SetIsInMeeting`
  (params (In :type Boolean)))

(fn `WW_SetIsInVotingTime`
  (params (In :type Boolean)))

(fn `WW_SetIsOnInputButtonLight`
  (params (Index :type Integer) (IsOn :type Boolean)))

(fn `WW_SetIsOnInputLight`
  (params (Index :type Integer) (IsOn :type Boolean)))

(fn `WW_SetIsOnOfNumberButton`
  (params (Number :type Integer) (IsOn :type Boolean)))

(fn `WW_SetIsOpenTask`
  (params (Open :type Boolean)))

(fn `WW_SetIsPutHand`
  (params (IsPut :type Boolean)))

(fn `WW_SetIsVotedToPlayer`
  (params (IsVotedToPlayer :type Boolean)))

(fn `WW_SetPlayerIndex`
  (params (Index :type Integer)))

(fn `WW_SetPlayerName`
  (params (Name :type String)))

(fn `WW_SetRemainingKillCooldown`
  (params (Percent :type "Float (double-precision)")))

(fn `WW_SetSabotageCooldownPercent`
  (params (Percent :type "Float (double-precision)")))

(fn `WW_SetVoteButton`
  (params (Name :type String)))

(fn `WW_SetWalkingSpeed`
  (params (Speed :type "Float (double-precision)")))

(fn `WW_ShowDeadBodyReportScreen`)

(fn `WW_ShowDeadScreen`)

(fn `WW_ShowEjectResult`
  (params (Name :type String) (IsSkip :type Boolean) (Remaining :type Integer) (CharacterType :type "/Game/Werewolf_01/Enum/e_CharacterType Enum" :default "NewEnumerator0") (VotingResult :type "/Game/Werewolf_01/BP/Gameplay/s_VotingResults Structure")))

(fn `WW_ShowEmergencyMeetingScreen`)

(fn `WW_ShowEmergencyScreen`)

(fn `WW_ShowInHatchScreen`)

(fn `WW_ShowKillCooldown`)

(fn `WW_ShowSabotageCooldown`)

(fn `WW_ShowStartScreen`)

(fn `WW_ShowTaskCompletedUI`)

(fn `WW_ShowVotedFromPlayerResult`)

(fn `WW_ShowVoteResult`)

(fn `WW_ShowVoteScreen`
  (params (VotedByPlayerIndex :type Integer)))

(fn `WW_SpawnPlayers`
  (returns (Vilagers :type "Array of /Game/Werewolf_01/BP/Character/BP_Villager Object Reference") (Wolfs :type "Array of /Game/Werewolf_01/BP/Character/BP_Wolf Object Reference"))
  (return))

(fn `WW_StartEmergencyTaskCoolDown`
  (params (Time :type "Float (double-precision)")))

(fn `WW_StartEndVoteTimer`)

(fn `WW_StartSabotageCooldown`)

(fn `WW_TaskComplete`
  (params (PC_ :type "/Game/Werewolf_01/BP/Gameplay/BP_GameplayPlayerController Object Reference")))

(fn `WW_TaskEnable`)

(fn `WW_Turn`
  (params (Value :type "Float (double-precision)")))

(fn `WW_UpdateCompletedTaskPercent`)

(fn `WW_UpdateHatchButtonEnabled`)

(fn `WW_UpdateHatchButtons`)

(fn `WW_UpdateKillButtonEnabled`)

(fn `WW_UpdateVoteButton`)

(fn `WW_VoteToPlayer`
  (params (Index :type Integer)))

(fn `WW_VoteToPlayerFinished`
  (params (Index :type Integer)))

(fn `WW_WinPlayer`)